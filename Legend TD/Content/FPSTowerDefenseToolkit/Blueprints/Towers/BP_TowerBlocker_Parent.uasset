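; Parent Blueprint for tower blockers, grid-cell-sized volumes meant to prevent tower placement where environment art sits.
; The construction script sizes the box from the grid manager's half cell size, then traces downward for a planar grid generator.
; On a hit, it snaps to that cell and matches the grid's yaw.
; Otherwise it flags itself decommissioned and destroys itself at BeginPlay.
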(event EventBeginPlay
  ;[1 0 0 0.5] Destroy decommissioned towers
  (if (Variables|AutomaticallySet|GetDecommisioned?)
    (Actor|DestroyActor self)))

(fn ConstructionScript
  (bind _returnvalue (Transformation|GetActorLocation))
  ;[0 1 1 0.5] Set Box Size to match a singular grid; Blocks Tower Spawn in this volume - Environment Art assets can be placed within the voulme
  (bind _outactors (Actor|GetAllActorsOfClass "/Game/FPSTowerDefenseToolkit/Blueprints/GameplayActors/BP_GridManager.BP_GridManager_C"))
  (Components|Box|SetBoxExtent (Math|Conversions|ToVector(Float) (Default|RetrieveHalfGridCellSize (Utilities|Array|Get(acopy) _outactors))) true)
  ;[0 1 1 0.5] Determines if tower blocker should be decommissioned or not; Anchor the tower blocker to the Grid Floor
  (bind (_outhit _returnvalue_2) (Collision|LineTraceByChannel _returnvalue (+ _returnvalue (* (Transformation|GetActorUpVector) -1e+03)) "TraceTypeQuery3" false 0 "None"))
  (if _returnvalue_2
    (bind _asbp_planar_grid_generator (Utilities|Casting|CastToBP_PlanarGridGenerator (.HitActor (Collision|BreakHitResult _outhit)))
      (:then
        (LocalVariables|SetLocal_GridGenerator _asbp_planar_grid_generator)
        (Variables|AutomaticallySet|SetDecommisioned? false)
        (bind _gridvector (Default|RetrieveTraceHitGridData (LocalVariables|GetLocal_GridGenerator) (.Location (Collision|BreakHitResult _outhit))))
        (Transformation|SetActorTransform (Math|Transform|MakeTransform _gridvector (Math|Rotator|MakeRotator 0.0 0.0 (.Yaw (Math|Rotator|BreakRotator (Transformation|GetActorRotation (LocalVariables|GetLocal_GridGenerator)))))) false true))
      (:CastFailed
        (Variables|AutomaticallySet|SetDecommisioned? true :!label _label)))
    (else
      (goto _label))))