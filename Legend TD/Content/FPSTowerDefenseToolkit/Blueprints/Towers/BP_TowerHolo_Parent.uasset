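; Parent Blueprint for holographic tower previews that show where a tower can be placed on the grid.
; Creates a dynamic hologram material for the tower and range meshes, tinted cyan or red by placement validity, and starts hidden.
; Stores grid cell data passed from the Tower Spawn Handler and exposes it with placement status, resetting both when deactivated.
; Child classes supply transform creation and resource checks, and extend display updates.
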(fn `ActivateHoloTower`
  ;[0 1 1 0.5] Display Holographic Tower
  (`self.SetActorHiddenInGame` false)
  (return))

(fn `CreateNewActorTransform`
  (params (GridVector :type "Vector Structure") (GridGeneratorRotation :type "Rotator Structure"))
  (returns (ActorTransform :type "Transform Structure"))
  ;[0 1 1 0.5] Creates new transform based on the tower type. Logic implemented in child classes
  (return))

(fn `DeactivateHoloTower`
  ;[1 0.5 0.2 0.5] Hide Holographic Tower
  (`self.SetActorHiddenInGame` true)
  (`self.UpdateTowerPlacementStatus` false)
  (`self.ResetGridData`) ; Resets the associated local grid data everytime the holographic display is deactivated
  (return))

(fn `EvaluateTowerResourceRequirements`
  (returns (`Success?` :type Boolean))
  ;[0 1 1 0.5] Implemented through child classes
  (return false))

(fn `ResetGridData`
  ;[0 1 1 0.5] Resets the associated local grid data
  (set `self.GridCellIndex` -2)
  (set `self.GridGeneratorIndex` -2)
  (return))

(fn `RetrieveTowerPlacementData`
  (returns (`CanPlaceTowerHere?` :type Boolean) (GridCellIndex :type Integer) (GridGeneratorIndex :type Integer))
  ;[0 1 1 0.5] Getter function used to retrieve the tower placement & grid data at the current position of the holo tower
  (return (`self.CanPlaceTowerHere?`) (`self.GridCellIndex`) (`self.GridGeneratorIndex`)))

(fn `SetHologramColor`
  (locals (Local_HologramColor :type "LinearColor Structure"))
  ;[0 1 1 0.5] New function added to change Hologram color
  (if (`self.CanPlaceTowerHere?`)
    (set `local.Local_HologramColor` (struct :`G` 1.0 :`B` 1.0 :`A` 1.0))
    (else
      (set `local.Local_HologramColor` (struct :`R` 1.0 :`A` 1.0))))
  (`MaterialInstanceDynamic.SetVectorParameterValue` (`self.HoloMaterial`) "GridColor" (`local.Local_HologramColor`)))

(fn `UpdateDisplayParameters`
  (params (GridCellIndex :type Integer) (GridGeneratorIndex :type Integer) (GridVector :type "Vector Structure") (GridGeneratorRotation :type "Rotator Structure") (GridCellStatus :type "/Game/FPSTowerDefenseToolkit/Blueprints/Enums/EGridCellStatus Enum") (HalfGridSize :type "Float (double-precision)"))
  ;[0 1 1 0.5] Updates display parameters based on input passed in from Tower Spawn Handler; Determines the state of the Holographic Tower; Function extended through child classes
  (set `self.GridCellIndex` GridCellIndex)
  (set `self.GridGeneratorIndex` GridGeneratorIndex)
  (set `self.FocusedGridVector` GridVector)
  (set `self.FocusedGridGeneratorRotation` GridGeneratorRotation)
  (set `self.FocusedGridCellStatus` GridCellStatus)
  (set `self.HalfGridSize` HalfGridSize))

(fn `UpdateTowerPlacementStatus`
  (params (`Yes?` :type Boolean))
  ;[0 1 1 0.5] Setter function used to update the tower placement status at the focused grid cell
  (set `self.CanPlaceTowerHere?` `Yes?`)
  (return))

(fn `UserConstructionScript`
  ;[0 1 1 0.5] Dynamic material instance created at spawn time, instead of letting Tower Spawn Manager handle it
  (bind _returnvalue (`KismetMaterialLibrary.CreateDynamicMaterialInstance` "/Game/FPSTowerDefenseToolkit/Materials/M_Holographic_Tower.M_Holographic_Tower"))
  (set `self.HoloMaterial` _returnvalue)
  (`PrimitiveComponent.SetMaterial` (`self.Tower`) 0 (`self.HoloMaterial`))
  (`PrimitiveComponent.SetMaterial` (`self.RangeDisplayMesh`) 0 (`self.HoloMaterial`))
  (`self.DeactivateHoloTower`) ; Keep the holographic display in a deactivated state until explicitly modified through activation requests
)