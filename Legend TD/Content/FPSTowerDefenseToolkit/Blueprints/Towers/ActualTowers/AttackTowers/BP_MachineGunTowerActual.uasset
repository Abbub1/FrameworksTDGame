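; Machine gun attack tower that tracks enemies entering its detection sphere and fires bullet projectiles at one target at a time.
; It picks the first in-range enemy with line of sight, retrying briefly when none qualifies.
; Looping timers yaw the gun toward the target and recheck sight each recharge cycle, firing or reacquiring.
; A Focus Fire component can manually override the target through an interface if sight is clear.
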(event `self.TargetDetectionSphere.OnComponentBeginOverlap`
  (params (OverlappedComponent :type "PrimitiveComponent Object Reference") (OtherActor :type "Actor Object Reference") (OtherComp :type "PrimitiveComponent Object Reference") (OtherBodyIndex :type Integer) (bFromSweep :type Boolean) (SweepResult :type "HitResult Structure (by ref)"))
  ;[0 1 1 0.5] Store reference to overlapping targets; Initialize target acquisition
  (bind _asbp_enemy_ai_parent (cast `/Game/FPSTowerDefenseToolkit/Blueprints/EnemyAI/BP_EnemyAI_Parent` OtherActor))
  (`KismetArrayLibrary.Array_Add` (`self.EnemyUnitsInRangeArray`) _asbp_enemy_ai_parent)
  (if (not (`self.SearchingForTargets?`))
    (set `self.SearchingForTargets?` true)
    (`self.AcquireNextTarget`)))

(event `self.TargetDetectionSphere.OnComponentEndOverlap`
  (params (OverlappedComponent :type "PrimitiveComponent Object Reference") (OtherActor :type "Actor Object Reference") (OtherComp :type "PrimitiveComponent Object Reference") (OtherBodyIndex :type Integer))
  ;[0 1 1 0.5] Remove stored enemy unit references based on end overlap events; If the actor is active target; lose the active target stored reference
  (bind _asbp_enemy_ai_parent (cast `/Game/FPSTowerDefenseToolkit/Blueprints/EnemyAI/BP_EnemyAI_Parent` OtherActor))
  (if (`KismetArrayLibrary.Array_Contains` (`self.EnemyUnitsInRangeArray`) _asbp_enemy_ai_parent)
    (`KismetArrayLibrary.Array_RemoveItem` (`self.EnemyUnitsInRangeArray`) _asbp_enemy_ai_parent)
    (if (== _asbp_enemy_ai_parent (`self.ActiveTarget`))
      (set `self.ActiveTarget` null))))

(event `AcquireNextTarget`
  ;[0 1 1 0.5] Chooses a target and starts attack timer
  (bind _success_ (`self.FindTarget`))
  (if _success_
    (`self.ActivateGunTargetingSystem`)
    (elif (> (`KismetArrayLibrary.Array_Length` (`self.EnemyUnitsInRangeArray`)) 0)
      (`KismetSystemLibrary.Delay` 0.2)
      (`self.AcquireNextTarget`) ; Search for potential targets again after a brief delay
      (else
        (set `self.SearchingForTargets?` false)))))

(event `/Game/FPSTowerDefenseToolkit/Blueprints/Interfaces/BPI_ManualTargetOverride.ActivateFocusFireSystem`
  (params (TargetActor :type "Actor Object Reference"))
  ;[0 1 0.4 0.5] BPI_ManualTargetOverride interface function - Requests the Focus Fire component to evaluate the designated target
  (`/Game/FPSTowerDefenseToolkit/Blueprints/CustomComponents/BPC_FocusFire.EvaluateManualTargetOverrideOrder` (`self.FocusFire`) (`self.EnemyUnitsInRangeArray`) TargetActor (`self.ActiveTarget`)))

(event `/Game/FPSTowerDefenseToolkit/Blueprints/Interfaces/BPI_ManualTargetOverride.OverrideActiveTarget`
  (params (NewTarget :type "Actor Object Reference"))
  ;[0 1 0.4 0.5] BPI_ManualTargetOverride interface function - Overrides active target with the Focus Fire target if Line of Sight can be established
  (bind _asbp_enemy_ai_parent (cast `/Game/FPSTowerDefenseToolkit/Blueprints/EnemyAI/BP_EnemyAI_Parent` NewTarget))
  (bind _success_ (`self.EvaluateLoSToTarget` _asbp_enemy_ai_parent))
  (if _success_
    (`self.DeactivateGunTargetingSystem`)
    (set `self.ActiveTarget` _asbp_enemy_ai_parent)
    (`self.ActivateGunTargetingSystem`)))

(fn `ActivateGunTargetingSystem`
  ;[0 1 1 0.5] Activates a timer driven Targeting system
  (bind _returnvalue (`KismetSystemLibrary.K2_SetTimer` null "FocusTowerGunOnActivetarget" 0.016667 true))
  (set `self.FocusTowerGunTimerHandle` _returnvalue)
  (bind _returnvalue_2 (`KismetSystemLibrary.K2_SetTimer` self "EvaluateActiveTargetStatus" (`self.RechargeTime`) true))
  (set `self.AttackTimerHandle` _returnvalue_2)
  (return))

(fn `AttackActiveTarget`
  ;[1 0 0 0.5] Attack active target
  (`|SpawnActorFromClass` "/Game/FPSTowerDefenseToolkit/Blueprints/Projectiles/BP_BulletProjectiles.BP_BulletProjectiles_C" (`SceneComponent.K2_GetComponentToWorld` (`self.BulletDirectionArrow`)) "AdjustIfPossibleButAlwaysSpawn" "OverrideRootScale" self (`self.OutputPerCycle`))
  (`GameplayStatics.PlaySoundAtLocation` "/Game/FPSTowerDefenseToolkit/Audio/FirstPerson_WeaponFire.FirstPerson_WeaponFire" (`SceneComponent.K2_GetComponentLocation` (`self.BulletDirectionArrow`))) ; Play firing sound
)

(fn `DeactivateGunTargetingSystem`
  ;[0 1 1 0.5] Deactivates the Targeting System
  (`KismetSystemLibrary.K2_ClearAndInvalidateTimerHandle` (`self.AttackTimerHandle`))
  (`KismetSystemLibrary.K2_ClearAndInvalidateTimerHandle` (`self.FocusTowerGunTimerHandle`))
  (return))

(fn `EvaluateActiveTargetStatus`
  ;[0 1 1 0.5] Perform validation & line trace checks for active target & determine appropriate course of action
  (`/Engine/EditorBlueprintResources/StandardMacros.IsValid` (`self.ActiveTarget`)
    (:`Is Valid`
      (bind _success_ (`self.EvaluateLoSToTarget` (`self.ActiveTarget`)))
      (if _success_
        (`self.AttackActiveTarget`)
        (else
          (`self.DeactivateGunTargetingSystem` :!label _label)
          (`self.AcquireNextTarget`))))
    (:`Is Not Valid`
      (goto _label))))

(fn `EvaluateLoSToTarget`
  (params (Target :type "/Game/FPSTowerDefenseToolkit/Blueprints/EnemyAI/BP_EnemyAI_Parent Object Reference"))
  (returns (`Success?` :type Boolean))
  (locals (Local_Target :type "/Game/FPSTowerDefenseToolkit/Blueprints/EnemyAI/BP_EnemyAI_Parent Object Reference"))
  ;[0 1 1 0.5] Determine if the tower has direct line of sight to the target
  (set `local.Local_Target` Target)
  (bind _outhit (`KismetSystemLibrary.LineTraceSingle` (`SceneComponent.K2_GetComponentLocation` (`self.BulletDirectionArrow`)) (`self.K2_GetActorLocation` (`local.Local_Target`)) "TraceTypeQuery1"))
  (return (== (`local.Local_Target`) (`.HitActor` (`GameplayStatics.BreakHitResult` _outhit)))))

(fn `FindTarget`
  (returns (`Success?` :type Boolean))
  (locals (`Local_TargetAcquired?` :type Boolean))
  ;[0 1 1 0.5] Select a new target from the 'EnemyUnitsInRange' array
  (set `local.Local_TargetAcquired?` false)
  (for _array_element (`self.EnemyUnitsInRangeArray`)
    (`/Engine/EditorBlueprintResources/StandardMacros.IsValid` _array_element
      (:`Is Valid`
        (bind _success_ (`self.EvaluateLoSToTarget` _array_element))
        (bind _output_get (set `local.Local_TargetAcquired?` _success_))
        (if _output_get
          (set `self.ActiveTarget` _array_element)
          (break)))))
  (return (`local.Local_TargetAcquired?`)))

(fn `FocusTowerGunOnActivetarget`
  (bind _towergun (`self.TowerGun`))
  ;[0 1 1 0.5] If Target is still in range/alive, turn the turret to face it
  (`/Engine/EditorBlueprintResources/StandardMacros.IsValid` (`self.ActiveTarget`)
    (:`Is Valid`
      (`SceneComponent.K2_SetWorldRotation` _towergun (`KismetMathLibrary.MakeRotator` (.roll (`SceneComponent.K2_GetComponentRotation` _towergun)) (.pitch (`SceneComponent.K2_GetComponentRotation` _towergun)) (.yaw (`KismetMathLibrary.FindLookAtRotation` (`SceneComponent.K2_GetComponentLocation` (`self.TowerGun`)) (`self.K2_GetActorLocation` (`self.ActiveTarget`))))) false false))))

(fn `UserConstructionScript`
  (`parent.UserConstructionScript`))