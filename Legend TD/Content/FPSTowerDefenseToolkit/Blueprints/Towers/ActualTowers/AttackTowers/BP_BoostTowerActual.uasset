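; Boost Tower for the tower defense toolkit that raises the damage of attack towers within its range, never boosting other Boost Towers.
; Towers entering the detection sphere receive OutputPerCycle as a damage boost, which is subtracted again from towers in range on EndPlay.
; Upgrading strips the old boost, runs the parent upgrade, then reapplies the new value.
; Sphere collision is enabled in the construction script for runtime spawns or in SetDefaultAttributes for editor-placed towers.
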(event `self.TargetDetectionSphere.OnComponentBeginOverlap`
  (params (OverlappedComponent :type "PrimitiveComponent Object Reference") (OtherActor :type "Actor Object Reference") (OtherComp :type "PrimitiveComponent Object Reference") (OtherBodyIndex :type Integer) (bFromSweep :type Boolean) (SweepResult :type "HitResult Structure (by ref)"))
  ;[0 1 1 0.5] Boost new overlapping towers
  (bind _asbp_attack_tower_actual_parent (cast `/Game/FPSTowerDefenseToolkit/Blueprints/Towers/ActualTowers/BP_AttackTowerActual_Parent` OtherActor))
  (`self.BoostSelectedTower` _asbp_attack_tower_actual_parent))

(event `self.ReceiveEndPlay`
  (params (EndPlayReason :type "EEndPlayReason Enum" :default "Destroyed"))
  ;[1 0 0 0.5] Remove Boost when before tower is destroyed
  (`self.RemoveBoostForAllTowersInRange`))

(event `self.UpgradeTower`
  ;[0 1 1 0.5] Remove boost for all towers in range & boost them again with the upgraded boost value
  (`self.RemoveBoostForAllTowersInRange`)
  (`parent.UpgradeTower`)
  (`self.BoostAllTowersInRange`))

(event `self.SetDefaultAttributes`
  (params (SelectedTowerDataArrayIndex :type Integer) (GridCellIndex :type Integer) (GridGeneratorIndex :type Integer) (TowerCost :type Integer) (OutputPerCycle :type "Float (single-precision)") (RechargeTime :type "Float (single-precision)") (Range :type "Float (single-precision)"))
  ;[0 1 1 0.5] If the Boost Tower was placed in the editor prior to game launch, then enable collision before setting the default range attribute
  (`PrimitiveComponent.SetCollisionEnabled` (`self.TargetDetectionSphere`) "QueryOnly")
  (`parent.SetDefaultAttributes` SelectedTowerDataArrayIndex GridCellIndex GridGeneratorIndex TowerCost OutputPerCycle RechargeTime Range))

(fn `BoostAllTowersInRange`
  ;[0 1 1 0.5] Boost all non-Boost Towers in Range
  (for _array_element (`PrimitiveComponent.GetOverlappingActors` (`self.TargetDetectionSphere`) "/Game/FPSTowerDefenseToolkit/Blueprints/Towers/ActualTowers/BP_AttackTowerActual_Parent.BP_AttackTowerActual_Parent_C")
    (bind _asbp_attack_tower_actual_parent (cast `/Game/FPSTowerDefenseToolkit/Blueprints/Towers/ActualTowers/BP_AttackTowerActual_Parent` _array_element))
    (`self.BoostSelectedTower` _asbp_attack_tower_actual_parent))
  (return))

(fn `BoostSelectedTower`
  (params (Tower :type "/Game/FPSTowerDefenseToolkit/Blueprints/Towers/ActualTowers/BP_AttackTowerActual_Parent Object Reference"))
  ;[0 1 1 0.5] Boost nearby tower as long as it's not a Boost Tower itself
  (cast `/Game/FPSTowerDefenseToolkit/Blueprints/Towers/ActualTowers/AttackTowers/BP_BoostTowerActual` Tower ; Do not boost other Boost Towers
    (:`CastFailed`
      (`self.ApplyDamageBoost` Tower (`self.OutputPerCycle`)))))

(fn `RemoveBoostForAllTowersInRange`
  ;[0 1 1 0.5] Remove Boost for all non-Boost Towers in Range
  (for _array_element (`PrimitiveComponent.GetOverlappingActors` (`self.TargetDetectionSphere`) "/Game/FPSTowerDefenseToolkit/Blueprints/Towers/ActualTowers/BP_AttackTowerActual_Parent.BP_AttackTowerActual_Parent_C")
    (bind _asbp_attack_tower_actual_parent (cast `/Game/FPSTowerDefenseToolkit/Blueprints/Towers/ActualTowers/BP_AttackTowerActual_Parent` _array_element))
    (`self.RemoveBoostForSelectedTower` _asbp_attack_tower_actual_parent))
  (return))

(fn `RemoveBoostForSelectedTower`
  (params (Tower :type "/Game/FPSTowerDefenseToolkit/Blueprints/Towers/ActualTowers/BP_AttackTowerActual_Parent Object Reference"))
  ;[1 0.5 0.2 0.5] Remove boost from nearby tower if it's not a Boost Tower itself
  (cast `/Game/FPSTowerDefenseToolkit/Blueprints/Towers/ActualTowers/AttackTowers/BP_BoostTowerActual` Tower ; Do not boost other Boost Towers
    (:`CastFailed`
      (`self.ApplyDamageBoost` Tower (* (`self.OutputPerCycle`) -1.0)))))

(fn `UserConstructionScript`
  (`parent.UserConstructionScript`)
  (cast `/Game/FPSTowerDefenseToolkit/Blueprints/BP_GameMode` (`GameplayStatics.GetGameMode`)) ; Fails for actors placed in the editor
  (`PrimitiveComponent.SetCollisionEnabled` (`self.TargetDetectionSphere`) "QueryOnly") ; If the Boost Tower is spawned in at runtime, then enable collision while executing the construction script
)