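; Shockwave tower actor that damages every enemy inside its detection sphere at once.
; Sphere overlaps maintain an array of enemies in range, and the first arrival starts the attack, which applies OutputPerCycle damage to each.
; A cylinder drops and rises as the pound animation, then a Tremor timer is set to repeat the cycle, though its time is zero.
; An empty array clears the timer and resets the tower.
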(event `self.TargetDetectionSphere.OnComponentBeginOverlap`
  (params (OverlappedComponent :type "PrimitiveComponent Object Reference") (OtherActor :type "Actor Object Reference") (OtherComp :type "PrimitiveComponent Object Reference") (OtherBodyIndex :type Integer) (bFromSweep :type Boolean) (SweepResult :type "HitResult Structure (by ref)"))
  (bind _cylinder4 (`self.Cylinder4`))
  ;[1 0.5 0.2 0.5] Activate the Tower and Deploy time delayed repeating shockwave damage to all enemy units in range
  (bind _asbp_enemy_ai_parent (cast `/Game/FPSTowerDefenseToolkit/Blueprints/EnemyAI/BP_EnemyAI_Parent` OtherActor))
  (`KismetArrayLibrary.Array_Add` (`self.EnemyUnitsInRangeArray`) _asbp_enemy_ai_parent)
  (if (not (`self.SearchingForTargets?`))
    (set `self.SearchingForTargets?` true)
    (`SceneComponent.K2_SetRelativeLocation` _cylinder4 (0.0 0.0 33.0) false false :!label _label)
    (`self.AttackEnemyUnits`)
    (`KismetSystemLibrary.Delay` 0.4)
    (`SceneComponent.K2_SetRelativeLocation` _cylinder4 (0.0 0.0 45.0) false false)
    (bind _returnvalue (`KismetSystemLibrary.K2_SetTimerDelegate` (delegate `Tremor`)))
    (set `self.AttackTimerHandle` _returnvalue)))

(event `Tremor`
  ;[1 0.5 0.2 0.5] Activate the Tower and Deploy time delayed repeating shockwave damage to all enemy units in range
  (goto _label))

(event `self.TargetDetectionSphere.OnComponentEndOverlap`
  (params (OverlappedComponent :type "PrimitiveComponent Object Reference") (OtherActor :type "Actor Object Reference") (OtherComp :type "PrimitiveComponent Object Reference") (OtherBodyIndex :type Integer))
  ;[0 1 1 0.5] Remove units that are outside range, update units in range array; If no enemy units in range, clear shockwave timer and deactivate tower.
  (bind _asbp_enemy_ai_parent (cast `/Game/FPSTowerDefenseToolkit/Blueprints/EnemyAI/BP_EnemyAI_Parent` OtherActor))
  (if (`KismetArrayLibrary.Array_Contains` (`self.EnemyUnitsInRangeArray`) _asbp_enemy_ai_parent)
    (`KismetArrayLibrary.Array_RemoveItem` (`self.EnemyUnitsInRangeArray`) _asbp_enemy_ai_parent)
    (if (not (> (`KismetArrayLibrary.Array_Length` (`self.EnemyUnitsInRangeArray`)) 0))
      (`KismetSystemLibrary.K2_ClearAndInvalidateTimerHandle` (`self.AttackTimerHandle`))
      (set `self.SearchingForTargets?` false)
      (`SceneComponent.K2_SetRelativeLocation` (`self.Cylinder4`) (0.0 0.0 45.0) false false))))

(fn `AttackEnemyUnits`
  ;[1 0 0 0.5] Attack all units in range
  (for _array_element (`self.EnemyUnitsInRangeArray`)
    (`/Engine/EditorBlueprintResources/StandardMacros.IsValid` _array_element
      (:`Is Valid`
        (`GameplayStatics.ApplyDamage` _array_element (`self.OutputPerCycle`) null self))))
  (return))

(fn `UserConstructionScript`
  (`parent.UserConstructionScript`))