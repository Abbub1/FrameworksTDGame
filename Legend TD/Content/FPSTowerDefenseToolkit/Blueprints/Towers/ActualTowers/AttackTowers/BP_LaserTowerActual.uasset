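; Laser attack tower that locks a beam onto one enemy in range and applies damage to it on a looping timer.
; A detection sphere tracks enemies, and the tower takes the first one passing a visibility line trace from its arrow.
; Each tick of the timer rechecks the target, then either damages it and moves the beam end or hides the beam and searches again.
; A Focus Fire interface can override the target given line of sight.
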(event `self.ReceiveBeginPlay`
  ;[0 1 1 0.5] Executes Parent Begin Play Logic & Creates a Laser Beam Emitter
  (`parent.ReceiveBeginPlay`)
  (`self.CreateLaserBeamEmitter`))

(event `self.TargetDetectionSphere.OnComponentBeginOverlap`
  (params (OverlappedComponent :type "PrimitiveComponent Object Reference") (OtherActor :type "Actor Object Reference") (OtherComp :type "PrimitiveComponent Object Reference") (OtherBodyIndex :type Integer) (bFromSweep :type Boolean) (SweepResult :type "HitResult Structure (by ref)"))
  ;[1 0.5 0.2 0.5] If enemy units are detected, activate the tower and start attack timer
  (bind _asbp_enemy_ai_parent (cast `/Game/FPSTowerDefenseToolkit/Blueprints/EnemyAI/BP_EnemyAI_Parent` OtherActor))
  (`KismetArrayLibrary.Array_Add` (`self.EnemyUnitsInRangeArray`) _asbp_enemy_ai_parent)
  (if (not (`self.SearchingForTargets?`))
    (set `self.SearchingForTargets?` true)
    (`self.AcquireNextTarget`)))

(event `self.TargetDetectionSphere.OnComponentEndOverlap`
  (params (OverlappedComponent :type "PrimitiveComponent Object Reference") (OtherActor :type "Actor Object Reference") (OtherComp :type "PrimitiveComponent Object Reference") (OtherBodyIndex :type Integer))
  ;[0 1 1 0.5] Updates the Enemy Units in range array; If no more units in range, deactivate the tower
  (bind _asbp_enemy_ai_parent (cast `/Game/FPSTowerDefenseToolkit/Blueprints/EnemyAI/BP_EnemyAI_Parent` OtherActor))
  (if (`KismetArrayLibrary.Array_Contains` (`self.EnemyUnitsInRangeArray`) _asbp_enemy_ai_parent)
    (`KismetArrayLibrary.Array_RemoveItem` (`self.EnemyUnitsInRangeArray`) _asbp_enemy_ai_parent)
    (if (== OtherActor (`self.ActiveTarget`))
      (set `self.ActiveTarget` null))))

(event `AcquireNextTarget`
  ;[0 1 1 0.5] Chooses a target and starts attack timer
  (bind _success_ (`self.FindTarget`))
  (if _success_
    (`self.ActivateLaserTargetingSystem`)
    (elif (> (`KismetArrayLibrary.Array_Length` (`self.EnemyUnitsInRangeArray`)) 0)
      (`KismetSystemLibrary.Delay` 0.2)
      (`self.AcquireNextTarget`) ; Search for potential targets again after a brief delay
      (else
        (set `self.SearchingForTargets?` false)))))

(event `/Game/FPSTowerDefenseToolkit/Blueprints/Interfaces/BPI_ManualTargetOverride.ActivateFocusFireSystem`
  (params (TargetActor :type "Actor Object Reference"))
  ;[0 1 0.4 0.5] BPI_ManualTargetOverride interface function - Requests the Focus Fire component to evaluate the designated target
  (`/Game/FPSTowerDefenseToolkit/Blueprints/CustomComponents/BPC_FocusFire.EvaluateManualTargetOverrideOrder` (`self.FocusFire`) (`self.EnemyUnitsInRangeArray`) TargetActor (`self.ActiveTarget`)))

(event `/Game/FPSTowerDefenseToolkit/Blueprints/Interfaces/BPI_ManualTargetOverride.OverrideActiveTarget`
  (params (NewTarget :type "Actor Object Reference"))
  (bind _attacktimerhandle (`self.AttackTimerHandle`))
  ;[0 1 0.4 0.5] BPI_ManualTargetOverride interface function - Overrides active target with the Focus Fire target if Line of Sight can be established
  (bind _asbp_enemy_ai_parent (cast `/Game/FPSTowerDefenseToolkit/Blueprints/EnemyAI/BP_EnemyAI_Parent` NewTarget))
  (bind _success_ (`self.EvaluateLoSToTarget` _asbp_enemy_ai_parent))
  (if _success_
    (if (`KismetSystemLibrary.K2_TimerExistsHandle` _attacktimerhandle)
      (`KismetSystemLibrary.K2_ClearAndInvalidateTimerHandle` _attacktimerhandle))
    (set `self.ActiveTarget` _asbp_enemy_ai_parent)
    (`self.ActivateLaserTargetingSystem`)))

(fn `ActivateLaserTargetingSystem`
  ;[0 1 1 0.5] Activates a timer driven Laser Targeting system
  (`self.EnableLaserBeamEmitter`)
  (bind _returnvalue (`KismetSystemLibrary.K2_SetTimer` null "EvaluateActiveTargetStatus" (`self.RechargeTime`) true))
  (set `self.AttackTimerHandle` _returnvalue)
  (return))

(fn `AttackActiveTarget`
  ;[1 0 0 0.5] Maintain laser beam focus on active target & apply damage
  (`self.UpdateLaserBeamTarget`)
  (`GameplayStatics.ApplyDamage` (`self.ActiveTarget`) (`self.OutputPerCycle`) null self))

(fn `CreateLaserBeamEmitter`
  ;[0 1 1 0.5] Creates a Laser Beam Emitter component
  (bind _returnvalue (`GameplayStatics.SpawnEmitterAtLocation` (`self.LaserBeamParticleSystem`) (`SceneComponent.K2_GetComponentLocation` (`self.Arrow`)) (struct) false))
  (set `self.LaserBeamEmitter` _returnvalue)
  (`self.DisableLaserBeamEmitter`) ; Disable the emitter by default
  (return))

(fn `DeactivateLaserTargetingSystem`
  ;[0 1 1 0.5] Deactivates the Laser Targeting System
  (`KismetSystemLibrary.K2_ClearAndInvalidateTimerHandle` (`self.AttackTimerHandle`))
  (`self.DisableLaserBeamEmitter`)
  (return))

(fn `DisableLaserBeamEmitter`
  ;[0 1 1 0.5] Disables the emitter to reduce operational costs
  (`ActorComponent.Deactivate` (`self.LaserBeamEmitter`))
  (`SceneComponent.SetHiddenInGame` (`self.LaserBeamEmitter`) true false)
  (`ActorComponent.SetComponentTickEnabled` (`self.LaserBeamEmitter`) false)
  (return))

(fn `EnableLaserBeamEmitter`
  ;[0 1 1 0.5] Enables the Laser Emitter component & sets it's default source/end points
  (`ParticleSystemComponent.SetBeamSourcePoint` (`self.LaserBeamEmitter`) 0 (`SceneComponent.K2_GetComponentLocation` (`self.Arrow`)) 0)
  (`ParticleSystemComponent.SetBeamEndPoint` (`self.LaserBeamEmitter`) 0 (`SceneComponent.K2_GetComponentLocation` (`/Game/FPSTowerDefenseToolkit/Blueprints/EnemyAI/BP_EnemyAI_Parent.UnitCore` (`self.ActiveTarget`))))
  (`ActorComponent.Activate` (`self.LaserBeamEmitter`) false)
  (`SceneComponent.SetHiddenInGame` (`self.LaserBeamEmitter`) false false)
  (`ActorComponent.SetComponentTickEnabled` (`self.LaserBeamEmitter`) true)
  (return))

(fn `EvaluateActiveTargetStatus`
  ;[0 1 1 0.5] Perform validation & line trace checks for active target & determine appropriate course of action
  (`/Engine/EditorBlueprintResources/StandardMacros.IsValid` (`self.ActiveTarget`)
    (:`Is Valid`
      (bind _success_ (`self.EvaluateLoSToTarget` (`self.ActiveTarget`)))
      (if _success_
        (`self.AttackActiveTarget`)
        (else
          (`KismetSystemLibrary.K2_ClearAndInvalidateTimerHandle` (`self.AttackTimerHandle`) :!label _label)
          (`self.DisableLaserBeamEmitter`)
          (`self.AcquireNextTarget`))))
    (:`Is Not Valid`
      (goto _label))))

(fn `EvaluateLoSToTarget`
  (params (Target :type "/Game/FPSTowerDefenseToolkit/Blueprints/EnemyAI/BP_EnemyAI_Parent Object Reference"))
  (returns (`Success?` :type Boolean))
  (locals (Local_Target :type "/Game/FPSTowerDefenseToolkit/Blueprints/EnemyAI/BP_EnemyAI_Parent Object Reference"))
  ;[0 1 1 0.5] Determine if the tower has direct line of sight to the target
  (set `local.Local_Target` Target)
  (bind _outhit (`KismetSystemLibrary.LineTraceSingle` (`SceneComponent.K2_GetComponentLocation` (`self.Arrow`)) (`self.K2_GetActorLocation` (`local.Local_Target`)) "TraceTypeQuery1"))
  (return (== (`local.Local_Target`) (`.HitActor` (`GameplayStatics.BreakHitResult` _outhit)))))

(fn `FindTarget`
  (returns (`Success?` :type Boolean))
  (locals (`Local_TargetAcquired?` :type Boolean))
  ;[0 1 1 0.5] Select a new target from the 'EnemyUnitsInRange' array
  (set `local.Local_TargetAcquired?` false)
  (for _array_element (`self.EnemyUnitsInRangeArray`)
    (`/Engine/EditorBlueprintResources/StandardMacros.IsValid` _array_element
      (:`Is Valid`
        (bind _success_ (`self.EvaluateLoSToTarget` _array_element))
        (bind _output_get (set `local.Local_TargetAcquired?` _success_))
        (if _output_get
          (set `self.ActiveTarget` _array_element)
          (break)))))
  (return (`local.Local_TargetAcquired?`)))

(fn `UpdateLaserBeamTarget`
  ;[0 1 1 0.5] Continuously update the laser beam end point based on the target location
  (`ParticleSystemComponent.SetBeamEndPoint` (`self.LaserBeamEmitter`) 0 (`SceneComponent.K2_GetComponentLocation` (`/Game/FPSTowerDefenseToolkit/Blueprints/EnemyAI/BP_EnemyAI_Parent.UnitCore` (`self.ActiveTarget`)))))

(fn `UserConstructionScript`
  (`parent.UserConstructionScript`))