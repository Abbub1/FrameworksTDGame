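; Placeable tower base for the tower defense grid, counted as a player resource and able to have a tower on it.
; Construction script spends one base and rebuilds nav paths when a game state exists; otherwise it snaps to the underlying grid generator's cell and yaw.
; Selling also sells any tower on top, refunds one base, and leaves pre-termination to the Game Mode.
; EndPlay rebuilds nav paths to update spline paths.
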(event `self.ReceiveEndPlay`
  (params (EndPlayReason :type "EEndPlayReason Enum" :default "Destroyed"))
  ;[0 1 1 0.5] Rebuild nav paths to update spline paths
  (`/Game/FPSTowerDefenseToolkit/Blueprints/BP_GameMode.RebuildNavPaths` (cast `/Game/FPSTowerDefenseToolkit/Blueprints/BP_GameMode` (`GameplayStatics.GetGameMode`) :!pure true)))

(event `self.ReturnTowerResources`
  ;[0 1 0.4 0.5] Update tower resources at creation & deletion of implementing actors
  (bind _asbp_player_state (cast `/Game/FPSTowerDefenseToolkit/Blueprints/BP_PlayerState` (`Controller.PlayerState` (`GameplayStatics.GetPlayerController` 0))))
  (`/Game/FPSTowerDefenseToolkit/Blueprints/BP_PlayerState.UpdateTowerBasesLeft` _asbp_player_state (`self.CalculateSellingPrice`)))

(event `self.UseTowerResources`
  (params (ResourceAmount :type Integer))
  ;[0 1 0.4 0.5] Update tower resources at creation & deletion of implementing actors
  (bind _asbp_player_state (cast `/Game/FPSTowerDefenseToolkit/Blueprints/BP_PlayerState` (`Controller.PlayerState` (`GameplayStatics.GetPlayerController` 0))))
  (`/Game/FPSTowerDefenseToolkit/Blueprints/BP_PlayerState.UpdateTowerBasesLeft` _asbp_player_state (* ResourceAmount -1)))

(event `/Game/FPSTowerDefenseToolkit/Blueprints/Interfaces/BPI_TowerFunctions.SellTower`
  (bind ((`Tower_27_DAC62711485A5B07DF08158DC082D797` _tower) (`GridStatus_19_DCC9ADC84265C7F51239C6A83D114BA1` _gridstatus)) (break `/Game/FPSTowerDefenseToolkit/Blueprints/Structs/Struct_GridCellData` (`KismetArrayLibrary.Array_Get` (`.GridGeneratorData_8_13E757544C1E18F1261E9C9C7CA2FC04` (break `/Game/FPSTowerDefenseToolkit/Blueprints/Structs/Struct_GridData` (`KismetArrayLibrary.Array_Get` (`/Game/FPSTowerDefenseToolkit/Blueprints/FunctionLibraries/BPFL_GetterFunctions.GetGridDataArray` self) (`self.GridGeneratorIndex`)))) (`self.GridCellIndex`))))
  ;[0 1 0.4 0.5] 'BPI_TowerFunctions' interface function to automatically handle return of tower resources & pre termination protocols
  (switch `/Game/FPSTowerDefenseToolkit/Blueprints/Enums/EGridCellStatus` _gridstatus
    (:`NewEnumerator1`
      _)
    (:`NewEnumerator2`
      (message `/Game/FPSTowerDefenseToolkit/Blueprints/Interfaces/BPI_TowerFunctions.SellTower` _tower) ; If a tower is placed on this tower base, sell it as well
    ))
  (`self.ReturnTowerResources`)
  (`/Game/FPSTowerDefenseToolkit/Blueprints/BP_GameMode.ReportTowerPendingDestroy` (cast `/Game/FPSTowerDefenseToolkit/Blueprints/BP_GameMode` (`GameplayStatics.GetGameMode`) :!pure true) self) ; Let Game Mode handle the pre termination protocols
)

(fn `CalculateSellingPrice`
  (returns (Returns :type Integer))
  ;[0 1 1 0.5] Overrides parent function; When selling a tower base, the player receives a new tower base to the arsenal
  (return 1))

(fn `UserConstructionScript`
  (locals (Local_GridGenerator :type "/Game/FPSTowerDefenseToolkit/Blueprints/GameplayActors/BP_PlanarGridGenerator Object Reference"))
  ;[0 1 1 0.5] Check location in World space to determine if it should be decommissioned; Anchors Tower Base to the Grid Floor
  (cast `/Game/FPSTowerDefenseToolkit/Blueprints/BP_GameState` (`GameplayStatics.GetGameState`)
    (:`then`
      (`self.UseTowerResources` 1) ; Call Interface function to use tower resources when the tower base is created
      (bind _asbp_game_mode (cast `/Game/FPSTowerDefenseToolkit/Blueprints/BP_GameMode` (`GameplayStatics.GetGameMode`)))
      (`/Game/FPSTowerDefenseToolkit/Blueprints/BP_GameMode.RebuildNavPaths` _asbp_game_mode) ; Rebuild nav paths to update spline paths [Only affects tower bases spawned during gameplay]
    )
    (:`CastFailed`
      (bind (_gridlinkedplatformexists_ _platformactor _tracehitlocation) (`self.GetGridGeneratorPlatform`)) ; Checks for an underlying grid generator platform
      (if _gridlinkedplatformexists_
        (bind _asbp_planar_grid_generator (cast `/Game/FPSTowerDefenseToolkit/Blueprints/GameplayActors/BP_PlanarGridGenerator` _platformactor))
        (bind _output_get (set `local.Local_GridGenerator` _asbp_planar_grid_generator))
        (bind (_gridcellindex _gridgeneratorindex _gridvector) (`/Game/FPSTowerDefenseToolkit/Blueprints/GameplayActors/BP_PlanarGridGenerator.RetrieveTraceHitGridData` _output_get _tracehitlocation))
        (bind _outactors (`GameplayStatics.GetAllActorsOfClass` "/Game/FPSTowerDefenseToolkit/Blueprints/GameplayActors/BP_TowerManager.BP_TowerManager_C"))
        (`self.K2_SetActorTransform` (`KismetMathLibrary.MakeTransform` (`KismetMathLibrary.MakeVector` (.x _gridvector) (.y _gridvector) (+ (`/Game/FPSTowerDefenseToolkit/Blueprints/GameplayActors/BP_TowerManager.TowerBaseZOffset` (`KismetArrayLibrary.Array_Get` _outactors)) (.z _gridvector))) (`KismetMathLibrary.MakeRotator` 0.0 0.0 (.yaw (`self.K2_GetActorRotation` (`local.Local_GridGenerator`)))) (1.0 1.0 1.0)) false true) ; Snaps to Grid
      ))))