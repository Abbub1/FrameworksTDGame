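; Parent Blueprint for attack towers in a tower defense game, adding the resource economy and keeping the target detection sphere sized to Range.
; Its construction script charges tower points during gameplay, otherwise snaps the tower to an underlying grid platform.
; Interface events handle selling, upgrades and upgrade-mode HUD stats using the tower data array.
; Upgrade cost grows exponentially with level; selling refunds modified total investment before GameMode handles removal.
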(event `self.ReceiveBeginPlay`
  ;[0 1 1 0.5] Updates the Total Setup Cost parameter & Collision Sphere Radius
  (set `self.TotalSetupCost` (`.TowerCost_5_E1AD7BEA4BEF28BC32CC68A787CFE968` (break `/Game/FPSTowerDefenseToolkit/Blueprints/Structs/Struct_TowerData` (`KismetArrayLibrary.Array_Get` (`/Game/FPSTowerDefenseToolkit/Blueprints/FunctionLibraries/BPFL_GetterFunctions.GetTowerDataArray`) (`self.TowerClassIndex`)))))
  (`SphereComponent.SetSphereRadius` (`self.TargetDetectionSphere`) (`self.Range`) true))

(event `self.ReturnTowerResources`
  ;[0 1 0.4 0.5] Automatically update tower resources at creation & deletion of implementing actors
  (bind _asbp_player_state (cast `/Game/FPSTowerDefenseToolkit/Blueprints/BP_PlayerState` (`Controller.PlayerState` (`GameplayStatics.GetPlayerController` 0))))
  (`/Game/FPSTowerDefenseToolkit/Blueprints/BP_PlayerState.UpdateTowerPoints` _asbp_player_state (`self.CalculateSellingPrice`)))

(event `self.UseTowerResources`
  (params (ResourceAmount :type Integer))
  ;[0 1 0.4 0.5] Automatically update tower resources at creation & deletion of implementing actors
  (bind _asbp_player_state (cast `/Game/FPSTowerDefenseToolkit/Blueprints/BP_PlayerState` (`Controller.PlayerState` (`GameplayStatics.GetPlayerController` 0))))
  (`/Game/FPSTowerDefenseToolkit/Blueprints/BP_PlayerState.UpdateTowerPoints` _asbp_player_state (* ResourceAmount -1)))

(event `/Game/FPSTowerDefenseToolkit/Blueprints/Interfaces/BPI_TowerFunctions.SellTower`
  ;[0 1 0.4 0.5] 'BPI_TowerFunctions' interface function to automatically handle return of tower resources & pre termination protocols
  (`self.ReturnTowerResources`)
  (`/Game/FPSTowerDefenseToolkit/Blueprints/BP_GameMode.ReportTowerPendingDestroy` (cast `/Game/FPSTowerDefenseToolkit/Blueprints/BP_GameMode` (`GameplayStatics.GetGameMode`) :!pure true) self) ; Let Game Mode handle the pre termination protocols
)

(event `/Game/FPSTowerDefenseToolkit/Blueprints/Interfaces/BPI_TowerFunctions.UpgradeTower`
  ;[0 1 0.4 0.5] 'BPI_TowerFunctions' interface function to handle tower upgrades
  (bind (_success_ _upgradecost) (`self.EvaluateTowerUpgradeRequirements`))
  (if _success_
    (`self.SetUpgradedTowerAttributes` _upgradecost)
    (`self.UseTowerResources` _upgradecost)))

(event `/Game/FPSTowerDefenseToolkit/Blueprints/Interfaces/BPI_HUDStatsUpdates.DisplayHUDStats`
  (bind _range (`self.Range`))
  (bind _towerlevel (`self.TowerLevel`))
  (bind _returnvalue (/ (`self.OutputPerCycle`) (`self.RechargeTime`)))
  (bind ((`TowerType_2_A3E4A46A4FD032BF10E0F890A310CA0B` _towertype) (`MaxUpgradeLevel_45_9AD5995F47810E3D0838F498F7F7A66E` _maxupgradelevel)) (break `/Game/FPSTowerDefenseToolkit/Blueprints/Structs/Struct_TowerData` (`KismetArrayLibrary.Array_Get` (`/Game/FPSTowerDefenseToolkit/Blueprints/FunctionLibraries/BPFL_GetterFunctions.GetTowerDataArray`) (`self.TowerClassIndex`))))
  (bind _returnvalue_2 (> _maxupgradelevel (`self.TowerLevel`)))
  ;[0 1 0.4 0.5] 'BPI_HUDStatsUpdates' interface function to display tower upgrade stats when focused by the player camera
  (switch `/Game/FPSTowerDefenseToolkit/Blueprints/Enums/EGameplayState` (`/Game/FPSTowerDefenseToolkit/Blueprints/FunctionLibraries/BPFL_GetterFunctions.GetGameplayState` self)
    (:`NewEnumerator0`
      (bind _asbp_player_controller (cast `/Game/FPSTowerDefenseToolkit/Blueprints/BP_PlayerController` (`GameplayStatics.GetPlayerController` 0)))
      (if _returnvalue_2
        (bind (_upgradedtowerlevel _upgradedoutputpercycle _upgradedrechargetime _upgradedrange) (`self.CalculateUpgradedTowerAttributes`))
        (`/Game/FPSTowerDefenseToolkit/Blueprints/BP_PlayerController.UpdateHUD_DisplayTowerUpgradeStats` _asbp_player_controller (`KismetTextLibrary.Conv_StringToText` (`|GetEnumeratorNameAsString` (`.TowerType_2_A3E4A46A4FD032BF10E0F890A310CA0B` (break `/Game/FPSTowerDefenseToolkit/Blueprints/Structs/Struct_TowerData` (`KismetArrayLibrary.Array_Get` (`/Game/FPSTowerDefenseToolkit/Blueprints/FunctionLibraries/BPFL_GetterFunctions.GetTowerDataArray`) (`self.TowerClassIndex`)))))) (`self.TowerLevel`) (/ (`self.OutputPerCycle`) (`self.RechargeTime`)) (`self.Range`) _returnvalue_2 _upgradedtowerlevel (/ _upgradedoutputpercycle _upgradedrechargetime) _upgradedrange (`self.CalculateTowerUpgradeCost`))
        (else
          (`/Game/FPSTowerDefenseToolkit/Blueprints/BP_PlayerController.UpdateHUD_DisplayTowerUpgradeStats` _asbp_player_controller (`KismetTextLibrary.Conv_StringToText` (`|GetEnumeratorNameAsString` _towertype)) _towerlevel _returnvalue _range _returnvalue_2 _towerlevel _returnvalue _range 0))))))

(event `self.SetUpgradedTowerAttributes`
  (params (UpgradeCost :type Integer))
  ;[0 1 1 0.5] Updates the Collision Sphere radius when the tower attributes get upgraded
  (`parent.SetUpgradedTowerAttributes` UpgradeCost)
  (`SphereComponent.SetSphereRadius` (`self.TargetDetectionSphere`) (`self.Range`) true))

(event `self.SetDefaultAttributes`
  (params (SelectedTowerDataArrayIndex :type Integer) (GridCellIndex :type Integer) (GridGeneratorIndex :type Integer) (TowerCost :type Integer) (OutputPerCycle :type "Float (single-precision)") (RechargeTime :type "Float (single-precision)") (Range :type "Float (single-precision)"))
  ;[0 1 1 0.5] Updates the Collision Sphere radius once the default attributes are set [Only applicable to towers placed in the editor]
  (`parent.SetDefaultAttributes` SelectedTowerDataArrayIndex GridCellIndex GridGeneratorIndex TowerCost OutputPerCycle RechargeTime Range)
  (`SphereComponent.SetSphereRadius` (`self.TargetDetectionSphere`) (`self.Range`) true))

(fn `CalculateSellingPrice`
  (returns (Returns :type Integer))
  ;[0 1 1 0.5] Overrides parent function; When selling a tower, the player receives tower resources back base on the total cost invested in the tower as well as a the unique Sell Modifer Cost for the tower
  (return (`KismetMathLibrary.FTrunc` (* (`self.TotalSetupCost`) (`.SellModifier_Cost_37_B09C6F514D028EF1AC97DEA8283A8420` (break `/Game/FPSTowerDefenseToolkit/Blueprints/Structs/Struct_TowerData` (`KismetArrayLibrary.Array_Get` (`/Game/FPSTowerDefenseToolkit/Blueprints/FunctionLibraries/BPFL_GetterFunctions.GetTowerDataArray`) (`self.TowerClassIndex`))))))))

(fn `CalculateTowerUpgradeCost`
  (returns (UpgradeCost :type Integer))
  (bind ((`TowerCost_5_E1AD7BEA4BEF28BC32CC68A787CFE968` _towercost) (`UpgradeModifier_Cost_32_50551FE946FF406F676A2DBBA10A1BB5` _upgrademodifier_cost)) (break `/Game/FPSTowerDefenseToolkit/Blueprints/Structs/Struct_TowerData` (`KismetArrayLibrary.Array_Get` (`/Game/FPSTowerDefenseToolkit/Blueprints/FunctionLibraries/BPFL_GetterFunctions.GetTowerDataArray`) (`self.TowerClassIndex`))))
  ;[0 1 1 0.5] Calculates the amount of resources required to upgrade the tower based on it's level & the unique upgrade modifier cost
  (return (`KismetMathLibrary.FTrunc` (* _towercost (`KismetMathLibrary.MultiplyMultiply_FloatFloat` _upgrademodifier_cost (`KismetMathLibrary.Conv_IntToDouble` (`self.TowerLevel`)))))))

(fn `EvaluateTowerUpgradeRequirements`
  (returns (`Success?` :type Boolean) (UpgradeCost :type Integer))
  (locals (Local_TowerUpgradeCost :type Integer))
  ;[0 1 1 0.5] Checks if the tower can be upgraded based on it's tower level as well as the availability of tower resources
  (bind _asbp_player_state (cast `/Game/FPSTowerDefenseToolkit/Blueprints/BP_PlayerState` (`Controller.PlayerState` (`GameplayStatics.GetPlayerController` 0)))
    (:`then`
      (set `local.Local_TowerUpgradeCost` (`self.CalculateTowerUpgradeCost`))
      (return (and (>= (`/Game/FPSTowerDefenseToolkit/Blueprints/BP_PlayerState.RetrieveTowerPoints` _asbp_player_state) (`local.Local_TowerUpgradeCost`)) (< (`self.TowerLevel`) (`.MaxUpgradeLevel_45_9AD5995F47810E3D0838F498F7F7A66E` (break `/Game/FPSTowerDefenseToolkit/Blueprints/Structs/Struct_TowerData` (`KismetArrayLibrary.Array_Get` (`/Game/FPSTowerDefenseToolkit/Blueprints/FunctionLibraries/BPFL_GetterFunctions.GetTowerDataArray`) (`self.TowerClassIndex`)))))) (`local.Local_TowerUpgradeCost`)))
    (:`CastFailed`
      (return false 0))))

(fn `UserConstructionScript`
  (locals (Local_GridGeneratorPlatform :type "Actor Object Reference"))
  ;[0 1 1 0.5] Checks tower location in World space to determine if it should be decommissioned; Anchors Tower to TowerBase
  (cast `/Game/FPSTowerDefenseToolkit/Blueprints/BP_GameState` (`GameplayStatics.GetGameState`)
    (:`then`
      (`self.UseTowerResources` (`self.TotalSetupCost`)) ; Use tower resources when the tower is created [Only affects towers spawned during gameplay]
    )
    (:`CastFailed`
      (bind (_gridlinkedplatformexists_ _platformactor _tracehitlocation) (`self.GetGridGeneratorPlatform`)) ; Checks for an underlying grid generator platform
      (if _gridlinkedplatformexists_
        (bind _output_get (set `local.Local_GridGeneratorPlatform` _platformactor))
        (bind (_gridcellindex _gridgeneratorindex _gridvector) (message `/Game/FPSTowerDefenseToolkit/Blueprints/Interfaces/BPI_GridLink.RetrieveTraceHitGridData` _output_get _tracehitlocation))
        (bind _outactors (`GameplayStatics.GetAllActorsOfClass` "/Game/FPSTowerDefenseToolkit/Blueprints/GameplayActors/BP_TowerManager.BP_TowerManager_C"))
        (`self.K2_SetActorTransform` (`KismetMathLibrary.MakeTransform` (`KismetMathLibrary.MakeVector` (.x _gridvector) (.y _gridvector) (+ (`/Game/FPSTowerDefenseToolkit/Blueprints/GameplayActors/BP_TowerManager.TowerZOffset` (`KismetArrayLibrary.Array_Get` _outactors)) (.z _gridvector))) (`KismetMathLibrary.MakeRotator` 0.0 0.0 (.yaw (`self.K2_GetActorRotation` (`local.Local_GridGeneratorPlatform`))))) false true) ; Snaps to Grid
      ))))