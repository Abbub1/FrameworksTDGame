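; Bullet projectile that damages valid targets on impact, fired by either enemy AI or non-enemy instigators.
; On hit, enemy shots damage only the player character or Power Core, while other shots damage only enemy AI; every hit destroys the projectile.
; When the instigator is an enemy, the construction script makes the collision component ignore the Pawn channel to prevent friendly-fire collisions between bots.
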(event `self.CollisionComponent.OnComponentHit`
  (params (HitComponent :type "PrimitiveComponent Object Reference") (OtherActor :type "Actor Object Reference") (OtherComp :type "PrimitiveComponent Object Reference") (NormalImpulse :type "Vector Structure") (Hit :type "HitResult Structure (by ref)"))
  (bind _returnvalue (`GameplayStatics.GetObjectClass` OtherActor))
  (bind _instigator (`self.Instigator`))
  (bind _damage (`self.Damage`))
  ;[1 0 0 0.5] Collision Response - Destroy Projectile & Apply Damage based on the instigator and the colliding actor
  (cast `/Game/FPSTowerDefenseToolkit/Blueprints/EnemyAI/BP_EnemyAI_Parent` (`self.GetInstigator`)
    (:`then`
      (if (or (== _returnvalue "/Game/FPSTowerDefenseToolkit/Blueprints/BP_PlayerCharacter.BP_PlayerCharacter_C") (== _returnvalue "/Game/FPSTowerDefenseToolkit/Blueprints/GameplayActors/BP_PowerCore.BP_PowerCore_C"))
        (`/Engine/EditorBlueprintResources/StandardMacros.IsValid` _instigator :!label _label
          (:`Is Valid`
            (`GameplayStatics.ApplyDamage` OtherActor _damage (`Pawn.GetController` _instigator)))
          (:`Is Not Valid`
            (`GameplayStatics.ApplyDamage` OtherActor _damage)))
        (`self.K2_DestroyActor`)
        (else
          (`self.K2_DestroyActor` :!label _label_2))))
    (:`CastFailed`
      (if (`KismetMathLibrary.ClassIsChildOf` (`GameplayStatics.GetObjectClass` OtherActor) "/Game/FPSTowerDefenseToolkit/Blueprints/EnemyAI/BP_EnemyAI_Parent.BP_EnemyAI_Parent_C")
        (goto _label)
        (else
          (goto _label_2))))))

(fn `UserConstructionScript`
  ;[0 1 1 0.5] Cancels out friendly fire collisions among AI Bots
  (cast `/Game/FPSTowerDefenseToolkit/Blueprints/EnemyAI/BP_EnemyAI_Parent` (`self.Instigator`))
  (`PrimitiveComponent.SetCollisionResponseToChannel` (`self.CollisionComponent`) "ECC_Pawn" "ECR_Ignore"))