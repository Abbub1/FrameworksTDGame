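; BP_CreepAIManager is the central registry of potential targets for enemy creeps in a tower defense game.
; Initialization puts the Power Core at a designated array index so its lookup stays fixed as targets are added.
; Registered Threat Analyzer creeps receive interface messages carrying the target's index when a threat is added or removed.
; Removal only notifies creeps, leaving the target array itself unchanged.
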(fn `AddNewPotentialTarget`
  (params (TargetActor :type "Actor Object Reference"))
  ;[0 1 1 0.5] Adds new Potential Target & alerts all Creeps that implement the Threat Analysis interface
  (bind _returnvalue (`KismetArrayLibrary.Array_Add` (`self.PotentialTargetsArray`) TargetActor))
  (for _array_element (`self.ThreatAnalyzerCreepsArray`)
    (message `/Game/FPSTowerDefenseToolkit/Blueprints/Interfaces/BPI_ThreatAnalysis.AddNewThreat` _array_element _returnvalue)))

(fn `AddNewThreatAnalyzerCreep`
  (params (CreepActor :type "Actor Object Reference"))
  ;[0 1 1 0.5] Updates the list containing references to all creeps that implement the Threat Analyzer interface
  (`KismetArrayLibrary.Array_Add` (`self.ThreatAnalyzerCreepsArray`) CreepActor))

(fn `InitializeCreepAIManager`
  (locals (OldCoreTargetIndex :type Integer :default 0))
  ;[0 1 1 0.5] Initializes the Creep Manager: Sets core as the designated first element of the Potential Targets Array [Ensures that no further changes are required for accessing the same after runtime updates to  the array]
  (`KismetArrayLibrary.Array_RemoveItem` (`self.PotentialTargetsArray`) (`/Game/FPSTowerDefenseToolkit/Blueprints/FunctionLibraries/BPFL_GetterFunctions.GetPowerCore` self))
  (`KismetArrayLibrary.Array_Insert` (`self.PotentialTargetsArray`) (`/Game/FPSTowerDefenseToolkit/Blueprints/FunctionLibraries/BPFL_GetterFunctions.GetPowerCore` self) (`self.PotentialTargetsArray_CoreIndex`))
  (return))

(fn `RemovePotentialTarget`
  (params (TargetActor :type "Actor Object Reference"))
  (locals (Local_TargetIndex :type Integer :default 0) (Local_TargetFound :type Boolean))
  ;[0 1 1 0.5] Removes a Potential Target & alerts all Creeps that implement the Threat Analysis interface
  (bind _output_get (set `local.Local_TargetIndex` (`KismetArrayLibrary.Array_Find` (`self.PotentialTargetsArray`) TargetActor)))
  (if (>= _output_get 0)
    (for _array_element (`self.ThreatAnalyzerCreepsArray`)
      (message `/Game/FPSTowerDefenseToolkit/Blueprints/Interfaces/BPI_ThreatAnalysis.RemoveThreat` _array_element (`local.Local_TargetIndex`)))))

(fn `RemoveThreatAnalyzerCreep`
  (params (CreepActor :type "Actor Object Reference"))
  ;[0 1 1 0.5] Updates the list containing references to all creeps that implement the Threat Analyzer interface
  (`KismetArrayLibrary.Array_RemoveItem` (`self.ThreatAnalyzerCreepsArray`) CreepActor))

(fn `RetrievePotentialTargetsArray`
  (returns (PotentialTargetsArray :type "Array of Actor Object Reference"))
  ;[0 1 1 0.5] Returns a list of all potential targets for creeps
  (return (`self.PotentialTargetsArray`)))

(fn `RetrievePowerCoreIndex`
  (returns (PotentialTargetsArray_CoreIndex :type Integer))
  ;[0 1 1 0.5] Returns the index of Power Core within the Potential Targets Array
  (return (`self.PotentialTargetsArray_CoreIndex`)))

(fn `UserConstructionScript`)