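; Ranged enemy creep AI that heads for the Power Core, diverts to threats and shoots bullet projectiles at them.
; Visual and damage perception feed weightings to the Threat Analyzer, which picks the active target for Threat Response to move, focus or attack.
; Components communicate through BPI interfaces, with target indices resolving into the Creep AI Manager's shared array.
; A timed placeholder attack pauses analysis and response; losing a target reverts to the core.
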(event `self.ReceiveAnyDamage`
  (params (Damage :type "Float (single-precision)") (DamageType :type "DamageType Object Reference") (InstigatedBy :type "Controller Object Reference") (DamageCauser :type "Actor Object Reference"))
  ;[1 0.5 0.2 0.5] Handles Incoming Damage Response
  (`parent.ReceiveAnyDamage` Damage DamageType InstigatedBy DamageCauser) ; Call parent event to handle health updates
  (`/Engine/EditorBlueprintResources/StandardMacros.IsValid` InstigatedBy
    (:`Is Valid`
      (if (> (`self.UnitHealth`) 0.0)
        (`/Game/FPSTowerDefenseToolkit/Blueprints/CustomComponents/BPC_DamagePerception.EvaluateDamageReceived` (`self.DamagePerception`) (`Controller.K2_GetPawn` InstigatedBy) Damage) ; Alert the Damage Perception Component
      ))))

(event `/Game/FPSTowerDefenseToolkit/Blueprints/Interfaces/BPI_VisualPerception.UpdateVisualPerceptionData`
  (params (`TargetInRange?` :type Boolean) (TargetIndex :type Integer) (TargetDistance :type "Float (single-precision)"))
  ;[0 1 0.4 0.5] BPI_VisualPerception interface function
  (`/Game/FPSTowerDefenseToolkit/Blueprints/CustomComponents/BPC_ThreatAnalyzer.UpdateVisualPerceptionWeightage` (`self.ThreatAnalyzer`) `TargetInRange?` TargetIndex TargetDistance (`self.VisionRange`)) ; Request the Threat Analyzer component to update the Visual Perception Threat Weightage for the target actor based on the distance
)

(event `/Game/FPSTowerDefenseToolkit/Blueprints/Interfaces/BPI_DamagePerception.UpdateDamagePerceptionData`
  (params (TargetIndex :type Integer) (DamageOverTimePercent :type "Float (single-precision)"))
  ;[0 1 0.4 0.5] BPI_DamagePerception interface function
  (`/Game/FPSTowerDefenseToolkit/Blueprints/CustomComponents/BPC_ThreatAnalyzer.UpdateDamagePerceptionWeightage` (`self.ThreatAnalyzer`) TargetIndex DamageOverTimePercent) ; Request the Threat Analyzer component to update the Damage Perception Threat Weightage for the target actor based on the damage inflicted by it
)

(event `/Game/FPSTowerDefenseToolkit/Blueprints/Interfaces/BPI_ThreatAnalysis.TargetAcquired`
  (params (TargetIndex :type Integer))
  ;[0 1 0.4 0.5] BPI_ThreatAnalysis interface functions
  (set `self.ActiveTargetIndex` TargetIndex) ; Set new Active Target Index based on the acquired target
  (`/Game/FPSTowerDefenseToolkit/Blueprints/CustomComponents/BPC_ThreatResponse.ActivateThreatResponse` (`self.ThreatResponse`)))

(event `/Game/FPSTowerDefenseToolkit/Blueprints/Interfaces/BPI_ThreatAnalysis.AddNewThreat`
  (params (TargetIndex :type Integer))
  ;[0 1 0.4 0.5] BPI_ThreatAnalysis interface functions
  (`/Game/FPSTowerDefenseToolkit/Blueprints/CustomComponents/BPC_ThreatAnalyzer.AddNewThreatElement` (`self.ThreatAnalyzer`) TargetIndex) ; Requests the Threat Analyzer component to add threat weightage information about a new target
)

(event `/Game/FPSTowerDefenseToolkit/Blueprints/Interfaces/BPI_ThreatAnalysis.TargetLost`
  (bind _potentialtargetsarray_coreindex (`/Game/FPSTowerDefenseToolkit/Blueprints/EnemyAI/BP_CreepAIManager.RetrievePowerCoreIndex` (`/Game/FPSTowerDefenseToolkit/Blueprints/FunctionLibraries/BPFL_GetterFunctions.GetCreepAIManager` self)))
  ;[0 1 0.4 0.5] BPI_ThreatAnalysis interface functions
  (if (!= (`self.ActiveTargetIndex`) _potentialtargetsarray_coreindex)
    (set `self.ActiveTargetIndex` _potentialtargetsarray_coreindex) ; Set target index for the Power Core as the Active Target Index
    (`/Game/FPSTowerDefenseToolkit/Blueprints/CustomComponents/BPC_ThreatResponse.DeactivateThreatResponse` (`self.ThreatResponse`))
    (`self.MoveToCore`)))

(event `/Game/FPSTowerDefenseToolkit/Blueprints/Interfaces/BPI_ThreatAnalysis.RemoveThreat`
  (params (TargetIndex :type Integer))
  ;[0 1 0.4 0.5] BPI_ThreatAnalysis interface functions
  (`/Game/FPSTowerDefenseToolkit/Blueprints/CustomComponents/BPC_ThreatAnalyzer.RemoveThreatElement` (`self.ThreatAnalyzer`) TargetIndex) ; Requests the Threat Analyzer component to delete threat weightage information about an existing target
)

(event `/Game/FPSTowerDefenseToolkit/Blueprints/Interfaces/BPI_ThreatResponse.MoveToActiveTarget`
  (bind _item (`KismetArrayLibrary.Array_Get` (`/Game/FPSTowerDefenseToolkit/Blueprints/EnemyAI/BP_CreepAIManager.RetrievePotentialTargetsArray` (`/Game/FPSTowerDefenseToolkit/Blueprints/FunctionLibraries/BPFL_GetterFunctions.GetCreepAIManager` self)) (`self.ActiveTargetIndex`)))
  ;[0 1 0.4 0.5] BPI_ThreatResponse interface functions
  (if (== (`self.ActiveTargetIndex`) (`/Game/FPSTowerDefenseToolkit/Blueprints/EnemyAI/BP_CreepAIManager.RetrievePowerCoreIndex` (`/Game/FPSTowerDefenseToolkit/Blueprints/FunctionLibraries/BPFL_GetterFunctions.GetCreepAIManager` self)))
    (`self.MoveToCore`)
    (else
      (`/Engine/EditorBlueprintResources/StandardMacros.IsValid` _item
        (:`Is Valid`
          (bind _returnvalue (`AIBlueprintHelperLibrary.GetAIController` self))
          (`AIController.MoveToActor` _returnvalue _item 0.0 false true false null true) ; Move towards the active target
        )))))

(event `/Game/FPSTowerDefenseToolkit/Blueprints/Interfaces/BPI_ThreatResponse.KeepActiveTargetInFocus`
  ;[0 1 0.4 0.5] BPI_ThreatResponse interface functions
  (`self.FocusViewOnTarget` (`KismetArrayLibrary.Array_Get` (`/Game/FPSTowerDefenseToolkit/Blueprints/EnemyAI/BP_CreepAIManager.RetrievePotentialTargetsArray` (`/Game/FPSTowerDefenseToolkit/Blueprints/FunctionLibraries/BPFL_GetterFunctions.GetCreepAIManager` self)) (`self.ActiveTargetIndex`))))

(event `/Game/FPSTowerDefenseToolkit/Blueprints/Interfaces/BPI_ThreatResponse.AttackActiveTarget`
  (bind _unitcore (`self.UnitCore`))
  (bind _item (`KismetArrayLibrary.Array_Get` (`/Game/FPSTowerDefenseToolkit/Blueprints/EnemyAI/BP_CreepAIManager.RetrievePotentialTargetsArray` (`/Game/FPSTowerDefenseToolkit/Blueprints/FunctionLibraries/BPFL_GetterFunctions.GetCreepAIManager` self)) (`self.ActiveTargetIndex`)))
  (bind _returnvalue (+ (`SceneComponent.K2_GetComponentLocation` _unitcore) (* (`SceneComponent.GetForwardVector` _unitcore) 50.0)))
  ;[0 1 0.4 0.5] BPI_ThreatResponse interface functions
  (`/Engine/EditorBlueprintResources/StandardMacros.IsValid` _item
    (:`Is Valid`
      (if (`KismetSystemLibrary.DoesImplementInterface` _item "/Game/FPSTowerDefenseToolkit/Blueprints/Interfaces/BPI_Targetable.BPI_Targetable_C")
        (`self.StartPlaceholderAttackAnimation`)
        (bind _targetlocation (message `/Game/FPSTowerDefenseToolkit/Blueprints/Interfaces/BPI_Targetable.RetrieveTargetableLocation` _item))
        (`|SpawnActorFromClass` "/Game/FPSTowerDefenseToolkit/Blueprints/Projectiles/BP_BulletProjectiles.BP_BulletProjectiles_C" (`KismetMathLibrary.MakeTransform` _returnvalue (`KismetMathLibrary.FindLookAtRotation` _returnvalue _targetlocation)) "AdjustIfPossibleButAlwaysSpawn" "OverrideRootScale" self (`self.AttackDamage`) self)
        (`KismetSystemLibrary.Delay` (`self.AttackAnimationDuration`))
        (`self.EndPlaceholderAttackAnimation`)))))

(event `/Game/FPSTowerDefenseToolkit/Blueprints/Interfaces/BPI_ThreatResponse.CancelMoveToActiveTarget`
  ;[0 1 0.4 0.5] BPI_ThreatResponse interface functions
  (bind _returnvalue (`AIBlueprintHelperLibrary.GetAIController` self))
  (`Controller.StopMovement` _returnvalue))

(event `self.StartPlaceholderAttackAnimation`
  ;[0 1 1 0.5] Placeholder function [used instead of real attack animation driven approach] to prevent the bot from performing new actions
  (`/Game/FPSTowerDefenseToolkit/Blueprints/CustomComponents/BPC_ThreatAnalyzer.DeactivateThreatAnalysis` (`self.ThreatAnalyzer`))
  (`/Game/FPSTowerDefenseToolkit/Blueprints/CustomComponents/BPC_ThreatResponse.DisableThreatResponseEvaluation` (`self.ThreatResponse`))
  (set `self.AttackAnimationActive?` true))

(event `self.EndPlaceholderAttackAnimation`
  ;[0 1 1 0.5] Reverts the bot to it's default state once the attack animation has been completed
  (`/Game/FPSTowerDefenseToolkit/Blueprints/CustomComponents/BPC_ThreatResponse.EnableThreatResponseEvaluation` (`self.ThreatResponse`))
  (`/Game/FPSTowerDefenseToolkit/Blueprints/CustomComponents/BPC_ThreatAnalyzer.ActivateThreatAnalysis` (`self.ThreatAnalyzer`))
  (set `self.AttackAnimationActive?` false))

(fn `RetrieveAttackAnimationStatus`
  (returns (`IsActive?` :type Boolean))
  ;[0 1 0.4 0.5] BPI_ThreatResponse interface function
  (return (`self.AttackAnimationActive?`)))

(fn `RetrieveDamagePerceptionRequisites`
  (returns (MaxHP :type "Float (double-precision)") (PotentialTargets :type "Array of Actor Object Reference"))
  ;[0 1 0.5 0.4] BPI_DamagePerception interface function [Used by the Damage Perception component to retrieve information pertinent to it's working
  (return (`self.MaxHealth`) (`/Game/FPSTowerDefenseToolkit/Blueprints/EnemyAI/BP_CreepAIManager.RetrievePotentialTargetsArray` (`/Game/FPSTowerDefenseToolkit/Blueprints/FunctionLibraries/BPFL_GetterFunctions.GetCreepAIManager` self))))

(fn `RetrieveThreatAnalysisRequisites`
  (returns (ActiveTargetIndex :type Integer) (PotentialTargets :type "Array of Actor Object Reference"))
  ;[0 1 0.4 0.5] BPI_ThreatAnalysis interface function [Used by the Threat Analysis component to retrieve information pertinent to it's working
  (return (`self.ActiveTargetIndex`) (`/Game/FPSTowerDefenseToolkit/Blueprints/EnemyAI/BP_CreepAIManager.RetrievePotentialTargetsArray` (`/Game/FPSTowerDefenseToolkit/Blueprints/FunctionLibraries/BPFL_GetterFunctions.GetCreepAIManager` self))))

(fn `RetrieveTraceDistanceToActiveTarget`
  (returns (TargetDistance :type "Float (double-precision)") (`TraceHitSuccess?` :type Boolean) (OwnerAttackRange :type "Float (double-precision)"))
  ;[0 1 0.4 0.5] BPI_ThreatResponse interface function [Used by the Threat Response component to retrieve information pertinent to it's working
  (bind (_targetdistance _targetinrange_) (`/Game/FPSTowerDefenseToolkit/Blueprints/CustomComponents/BPC_ThreatAnalyzer.RetrieveTargetDistance` (`self.ThreatAnalyzer`) (`self.ActiveTargetIndex`) (`self.VisionRange`))) ; Requests the Threat Analysis component to determine the spatial relation to the specified target
  (return _targetdistance _targetinrange_ (`self.AttackRange`)))

(fn `RetrieveVisualPerceptionRequisites`
  (returns (VisionRange :type "Float (double-precision)") (VisionAngle :type "Float (double-precision)") (ActiveTargetIndex :type Integer) (PotentialTargets :type "Array of Actor Object Reference"))
  ;[0 1 0.4 0.5] BPI_VisualPerception interface function [Used by the Visual Perception component to retrieve information pertinent to it's working
  (return (`self.VisionRange`) (`self.VisionAngle`) (`self.ActiveTargetIndex`) (`/Game/FPSTowerDefenseToolkit/Blueprints/EnemyAI/BP_CreepAIManager.RetrievePotentialTargetsArray` (`/Game/FPSTowerDefenseToolkit/Blueprints/FunctionLibraries/BPFL_GetterFunctions.GetCreepAIManager` self))))

(fn `UserConstructionScript`
  (`parent.UserConstructionScript`))