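; Game state for a tower defense FPS that tracks the current gameplay mode, mission success and mission statistics.
; Changing the gameplay state also asks the player controller to update HUD visibility, and initialization sets the default Tower Build mode.
; Simple update and getter functions accumulate damage and kills separately for the player and towers, and expose them with the mission result to other Blueprints.
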(fn `InitializeGameState`
  ;[0 1 1 0.5] Initialize the Game State by setting the default state to Tower Build Mode
  (`self.UpdateGameplayState` "NewEnumerator1")
  (return))

(fn `RetrieveGameplayState`
  (returns (GameplayState :type "/Game/FPSTowerDefenseToolkit/Blueprints/Enums/EGameplayState Enum"))
  ;[0 1 1 0.5] Getter function used by other blueprints to retrieve the Gameplay State
  (return (`self.GameplayState`)))

(fn `RetrieveMissionStats`
  (returns (DamageInflictedByPlayer :type "Float (double-precision)") (DamageInflictedByTowers :type "Float (double-precision)") (NumberOfPlayerKills :type Integer) (NumberOfTowerKills :type Integer))
  ;[0 1 1 0.5] Version 1.0: Returns the mission stats
  (return (`self.DamageInflictedByPlayer`) (`self.DamageInflictedByTowers`) (`self.NumberOfPlayerKills`) (`self.NumberOfTowerKills`)))

(fn `RetrieveMissionStatus`
  (returns (`MissionSuccess?` :type Boolean))
  ;[0 1 1 0.5] Getter function used by other blueprints to retrieve the mission status
  (return (`self.MissionSuccess?`)))

(fn `UpdateGameplayState`
  (params (NewGameplayState :type "/Game/FPSTowerDefenseToolkit/Blueprints/Enums/EGameplayState Enum"))
  ;[0 1 1 0.5] Updates the Gameplay state; Requests the player controller to make necessary HUD changes for the new state
  (set `self.GameplayState` NewGameplayState)
  (bind _asbp_player_controller (cast `/Game/FPSTowerDefenseToolkit/Blueprints/BP_PlayerController` (`GameplayStatics.GetPlayerController` 0)))
  (`/Game/FPSTowerDefenseToolkit/Blueprints/BP_PlayerController.UpdateHUD_StateBasedVisibility` _asbp_player_controller (`self.GameplayState`)))

(fn `UpdateMissionStatus`
  (params (`Success?` :type Boolean))
  ;[0 1 1 0.5] Update the mission status of the current level
  (set `self.MissionSuccess?` `Success?`)
  (return))

(fn `UpdateStats_PlayerInflictedDamage`
  (params (DamageIncrement :type "Float (double-precision)"))
  ;[0 1 1 0.5] Version 1.9: Updates the amount of damage inflicted by the player
  (set `self.DamageInflictedByPlayer` (+ (`self.DamageInflictedByPlayer`) DamageIncrement))
  (return))

(fn `UpdateStats_PlayerKills`
  ;[0 1 1 0.5] Version 1.9: Updates the number of kills scored by the player
  (set `self.NumberOfPlayerKills` (+ (`self.NumberOfPlayerKills`) 1))
  (return))

(fn `UpdateStats_TowerInflictedDamage`
  (params (DamageIncrement :type "Float (double-precision)"))
  ;[0 1 1 0.5] Version 1.9: Updates the amount of damage inflicted by the towers
  (set `self.DamageInflictedByTowers` (+ (`self.DamageInflictedByTowers`) DamageIncrement))
  (return))

(fn `UpdateStats_TowerKills`
  ;[0 1 1 0.5] Version 1.9: Updates the number of kills scored by the towers
  (set `self.NumberOfTowerKills` (+ (`self.NumberOfTowerKills`) 1))
  (return))

(fn `UserConstructionScript`)