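; Actor component that picks the most relevant threat for its owner, which must implement BPI_ThreatAnalysis, and registers that owner with the Creep AI Manager.
; It keeps per-target weights: visual scales inversely with distance, damage accumulates to a cap.
; A looping timer reports the highest combined weight or target loss to the owner through interface messages.
; An active-target bonus makes challengers exceed the current target by a margin before switching.
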(event `self.ReceiveBeginPlay`
  ;[0 1 1 0.5] Initiate the threat analyzer functionality if the owning actor meets the compabitibility requirements
  (if (`KismetSystemLibrary.DoesImplementInterface` (`self.GetOwner`) "/Game/FPSTowerDefenseToolkit/Blueprints/Interfaces/BPI_ThreatAnalysis.BPI_ThreatAnalysis_C")
    (`/Game/FPSTowerDefenseToolkit/Blueprints/EnemyAI/BP_CreepAIManager.AddNewThreatAnalyzerCreep` (`/Game/FPSTowerDefenseToolkit/Blueprints/FunctionLibraries/BPFL_GetterFunctions.GetCreepAIManager` self) (`self.GetOwner`)) ; Alerts the Creep AI Manager about the presence of the owning actor
    (`self.CreateThreatWeightageArray`)
    (`self.ActivateThreatAnalysis`)
    (else
      (`self.DisplayOwnerIncompatibilityWarning`))))

(event `ActivateThreatAnalysis`
  ;[0 1 1 0.5] Activates timed evaluation of Threat Weightage Array to determine the most relevant threat at any point of time
  (`self.EvaluateThreatWeightageArray`)
  (bind _returnvalue (`KismetSystemLibrary.K2_SetTimer` null "EvaluateThreatWeightageArray" (`self.ThreatWeightageEvaluationTimerInterval`) true))
  (set `self.EvaluateThreatWeightageArrayTimerHandle` _returnvalue))

(event `DeactivateThreatAnalysis`
  (bind _evaluatethreatweightagearraytimerhandle (`self.EvaluateThreatWeightageArrayTimerHandle`))
  ;[0 1 1 0.5] Deactivates Threat Evaluation Timer
  (if (`KismetSystemLibrary.K2_TimerExistsHandle` _evaluatethreatweightagearraytimerhandle)
    (`KismetSystemLibrary.K2_ClearAndInvalidateTimerHandle` _evaluatethreatweightagearraytimerhandle)))

(event `self.ReceiveEndPlay`
  (params (EndPlayReason :type "EEndPlayReason Enum" :default "Destroyed"))
  ;[0 1 1 0.5] Request the Creep AI Manager to remove the owning actor from the list of potential targets
  (`/Game/FPSTowerDefenseToolkit/Blueprints/EnemyAI/BP_CreepAIManager.RemoveThreatAnalyzerCreep` (`/Game/FPSTowerDefenseToolkit/Blueprints/FunctionLibraries/BPFL_GetterFunctions.GetCreepAIManager` self) (`self.GetOwner`)))

(fn `AddNewThreatElement`
  (params (Index :type Integer))
  ;[0 1 1 0.5] Adds a new element to the Threat Weightage Array
  (`KismetArrayLibrary.Array_Set` (`self.ThreatWeightageArray`) Index (make `/Game/FPSTowerDefenseToolkit/Blueprints/Structs/Struct_ThreatWeightageData` Index 0.0 0.0) true))

(fn `CreateThreatWeightageArray`
  ;[0 1 1 0.5] Creates a Threat Weightage Array using the list of potential targets
  (bind (_activetargetindex _potentialtargets) (message `/Game/FPSTowerDefenseToolkit/Blueprints/Interfaces/BPI_ThreatAnalysis.RetrieveThreatAnalysisRequisites` (`self.GetOwner`)))
  (for (_ _array_index) _potentialtargets
    (`KismetArrayLibrary.Array_Set` (`self.ThreatWeightageArray`) _array_index (make `/Game/FPSTowerDefenseToolkit/Blueprints/Structs/Struct_ThreatWeightageData` _array_index 0.0 0.0) true))
  (return))

(fn `DisplayOwnerIncompatibilityWarning`
  ;[0 0 0 0.5] Prints a warning message if the owning actor does not implement the requisite interface
  (`KismetSystemLibrary.PrintString` (`KismetStringLibrary.Concat_StrStr` "Warning: [Class: BPC_VisualPerception] Owning actor '" (`KismetSystemLibrary.GetDisplayName` (`self.GetOwner`)) "' does not implement requisite interface")))

(fn `EvaluateThreatWeightageArray`
  (locals (Local_HighestThreatWeightage :type "Float (double-precision)" :default 0.0) (Local_HighestThreatIndex :type Integer :default 0) (`Local_NewPossibleThreat?` :type Boolean) (Local_ActiveTargetIndex :type Integer :default 0))
  (bind _returnvalue (`self.GetOwner`))
  ;[0 1 1 0.5] Evaluates the Threat Weightage Array & provides the test results to the owning actor
  (if (> (`KismetArrayLibrary.Array_Length` (`self.ThreatWeightageArray`)) 0)
    (for _array_element (`self.ThreatWeightageArray`)
      (bind (_targetindex _threatweight_visualperception _threatweight_damageperception) (break `/Game/FPSTowerDefenseToolkit/Blueprints/Structs/Struct_ThreatWeightageData` _array_element))
      (bind _returnvalue_2 (+ _threatweight_visualperception _threatweight_damageperception))
      (if (> _returnvalue_2 (`local.Local_HighestThreatWeightage`))
        (set `local.Local_NewPossibleThreat?` true)
        (set `local.Local_HighestThreatIndex` _targetindex)
        (set `local.Local_HighestThreatWeightage` _returnvalue_2)))
    (if (`local.Local_NewPossibleThreat?`)
      (bind _activetargetindex (message `/Game/FPSTowerDefenseToolkit/Blueprints/Interfaces/BPI_ThreatAnalysis.RetrieveThreatAnalysisRequisites` _returnvalue))
      (if (== _activetargetindex (`local.Local_HighestThreatIndex`))
        (message `/Game/FPSTowerDefenseToolkit/Blueprints/Interfaces/BPI_ThreatAnalysis.TargetAcquired` (`self.GetOwner`) (`local.Local_HighestThreatIndex`) :!label _label) ; Pass information about the most relevant threat element to the owning actor
        (else
          (bind ((`ThreatWeight_VisualPerception_9_B2789CBA406A50E202FEFCB88C908446` _threatweight_visualperception_2) (`ThreatWeight_DamagePerception_10_225E1D814B121CF28ACFE6B05A5133F2` _threatweight_damageperception_2)) (break `/Game/FPSTowerDefenseToolkit/Blueprints/Structs/Struct_ThreatWeightageData` (`KismetArrayLibrary.Array_Get` (`self.ThreatWeightageArray`) _activetargetindex)))
          (if (> (`local.Local_HighestThreatWeightage`) (+ _threatweight_visualperception_2 _threatweight_damageperception_2 (`self.ActiveTargetBonusWeightage`)))
            (goto _label))))
      (else
        (message `/Game/FPSTowerDefenseToolkit/Blueprints/Interfaces/BPI_ThreatAnalysis.TargetLost` _returnvalue) ; If no relevant threat detected, report the same to the owning actor
      ))))

(fn `RemoveThreatElement`
  (params (Index :type Integer))
  ;[0 1 1 0.5] Removes an existing element from the Threat Weightage Array
  (if (< Index (`KismetArrayLibrary.Array_Length` (`self.ThreatWeightageArray`)))
    (`KismetArrayLibrary.Array_Remove` (`self.ThreatWeightageArray`) Index)))

(fn `RetrieveTargetDistance`
  (params (TargetIndex :type Integer) (OwnerVisionRange :type "Float (double-precision)"))
  (returns (TargetDistance :type "Float (double-precision)") (`TargetInRange?` :type Boolean))
  (bind _maxvisualperceptionweightage (`self.MaxVisualPerceptionWeightage`))
  (bind ((`ThreatWeight_VisualPerception_9_B2789CBA406A50E202FEFCB88C908446` _threatweight_visualperception)) (break `/Game/FPSTowerDefenseToolkit/Blueprints/Structs/Struct_ThreatWeightageData` (`KismetArrayLibrary.Array_Get` (`self.ThreatWeightageArray`) TargetIndex)))
  ;[0 1 1 0.5] Calculates trace distance to the target entity by using a reverse workflow on it's Visual Perception Weightage
  (if (> _threatweight_visualperception 0.0)
    (return (* OwnerVisionRange (/ (- _maxvisualperceptionweightage _threatweight_visualperception) _maxvisualperceptionweightage)) true) ; Target inside visual range: Returns trace distance
    (else
      (return 0.0 false) ; Target outside visual range
    )))

(fn `UpdateDamagePerceptionWeightage`
  (params (TargetIndex :type Integer) (DamageOverTimePercent :type "Float (double-precision)"))
  (bind (_targetindex _threatweight_visualperception _threatweight_damageperception) (break `/Game/FPSTowerDefenseToolkit/Blueprints/Structs/Struct_ThreatWeightageData` (`KismetArrayLibrary.Array_Get` (`self.ThreatWeightageArray`) TargetIndex)))
  ;[0 1 1 0.5] Calculates the new Damage Perception weightage for the associated entity based on the information provided by the owning actor
  (`self.UpdateThreatWeightageArray` TargetIndex (make `/Game/FPSTowerDefenseToolkit/Blueprints/Structs/Struct_ThreatWeightageData` _targetindex _threatweight_visualperception (`KismetMathLibrary.FClamp` (+ _threatweight_damageperception (* DamageOverTimePercent (`self.MaxDamagePerceptionWeightage`))) 0.0 (`self.MaxDamagePerceptionWeightage`)))))

(fn `UpdateThreatWeightageArray`
  (params (TargetIndex :type Integer) (TargetThreatWeightageData :type "/Game/FPSTowerDefenseToolkit/Blueprints/Structs/Struct_ThreatWeightageData Structure"))
  ;[0 1 1 0.5] Updates the Threat Weightage Array with the new weightage data
  (`KismetArrayLibrary.Array_Set` (`self.ThreatWeightageArray`) TargetIndex TargetThreatWeightageData))

(fn `UpdateVisualPerceptionWeightage`
  (params (`TargetInRange?` :type Boolean) (TargetIndex :type Integer) (TargetTraceDistance :type "Float (double-precision)") (OwnerVisionRange :type "Float (double-precision)"))
  (locals (Local_NewVisualPerceptionWeightage :type "Float (double-precision)"))
  (bind (_targetindex _threatweight_visualperception _threatweight_damageperception) (break `/Game/FPSTowerDefenseToolkit/Blueprints/Structs/Struct_ThreatWeightageData` (`KismetArrayLibrary.Array_Get` (`self.ThreatWeightageArray`) TargetIndex)))
  ;[0 1 1 0.5] Calculates the new Visual Perception weightage for the associated entity based on the information provided by the owning actor
  (if `TargetInRange?`
    (set `local.Local_NewVisualPerceptionWeightage` (* (- 1.0 (/ TargetTraceDistance OwnerVisionRange)) (`self.MaxVisualPerceptionWeightage`)))
    (else
      (set `local.Local_NewVisualPerceptionWeightage` 0.0)))
  (`self.UpdateThreatWeightageArray` TargetIndex (make `/Game/FPSTowerDefenseToolkit/Blueprints/Structs/Struct_ThreatWeightageData` _targetindex (`KismetMathLibrary.FClamp` (`local.Local_NewVisualPerceptionWeightage`) 0.0 (`self.MaxVisualPerceptionWeightage`)) _threatweight_damageperception)))