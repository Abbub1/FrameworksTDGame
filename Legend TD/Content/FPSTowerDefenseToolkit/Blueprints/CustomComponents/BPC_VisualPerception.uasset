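; BPC_VisualPerception is an actor component that gives its owner timed sight checks on potential targets.
; On a looping timer it pulls range, angle and target list from the owner through BPI_VisualPerception, warning if that interface is missing.
; BPI_Targetable targets pass distance, view-cone and Camera-channel line trace tests, with the active target skipping the cone test.
; Each valid target's visibility and distance is reported back to the owner.
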(event `self.ReceiveBeginPlay`
  ;[0 1 1 0.5] Initiate timed vision checks if the owning actor meets the compabitibility requirements
  (if (`KismetSystemLibrary.DoesImplementInterface` (`self.GetOwner`) "/Game/FPSTowerDefenseToolkit/Blueprints/Interfaces/BPI_VisualPerception.BPI_VisualPerception_C")
    (bind _returnvalue (`KismetSystemLibrary.K2_SetTimer` null "VisionCheck" (`self.VisionCheckTimerInterval`) true))
    (set `self.VisionCheckTimerHandle` _returnvalue)
    (else
      (`self.DisplayOwnerIncompatibilityWarning`))))

(event `self.ReceiveEndPlay`
  (params (EndPlayReason :type "EEndPlayReason Enum" :default "Destroyed"))
  (bind _visionchecktimerhandle (`self.VisionCheckTimerHandle`))
  ;[0 1 1 0.5] Clear timers before getting destroyed
  (if (`KismetSystemLibrary.K2_TimerExistsHandle` _visionchecktimerhandle)
    (`KismetSystemLibrary.K2_ClearAndInvalidateTimerHandle` _visionchecktimerhandle)))

(fn `DisplayOwnerIncompatibilityWarning`
  ;[0 0 0 0.5] Prints a warning message if the owning actor does not implement the requisite interface
  (`KismetSystemLibrary.PrintString` (`KismetStringLibrary.Concat_StrStr` "Warning: [Class: BPC_VisualPerception] Owning actor '" (`KismetSystemLibrary.GetDisplayName` (`self.GetOwner`)) "' does not implement requisite interface")))

(fn `VisionCheck`
  (locals (Local_TargetActor :type "Actor Object Reference") (Local_TargetIndex :type Integer :default 0) (Local_VisionRange :type "Float (double-precision)") (Local_VisionAngle :type "Float (double-precision)") (Local_ActiveTargetIndex :type Integer :default 0))
  ;[0 1 1 0.5] Performs a combination of need based spatial checks for all potential targets & relays the information to the parent actor
  (bind (_visionrange _visionangle _activetargetindex _potentialtargets) (message `/Game/FPSTowerDefenseToolkit/Blueprints/Interfaces/BPI_VisualPerception.RetrieveVisualPerceptionRequisites` (`self.GetOwner`))) ; Retrieves all requisite parameters from the owning actor
  (set `local.Local_VisionRange` _visionrange)
  (set `local.Local_VisionAngle` _visionangle)
  (set `local.Local_ActiveTargetIndex` _activetargetindex)
  (for (_array_element _array_index) _potentialtargets
    (bind _output_get (set `local.Local_TargetActor` _array_element))
    (`/Engine/EditorBlueprintResources/StandardMacros.IsValid` _output_get
      (:`Is Valid`
        (set `local.Local_TargetIndex` _array_index)
        (if (`KismetSystemLibrary.DoesImplementInterface` (`local.Local_TargetActor`) "/Game/FPSTowerDefenseToolkit/Blueprints/Interfaces/BPI_Targetable.BPI_Targetable_C")
          (bind _correcteddistance (message `/Game/FPSTowerDefenseToolkit/Blueprints/Interfaces/BPI_Targetable.GetCorrectedDistanceToActor` (`local.Local_TargetActor`) (`Actor.K2_GetActorLocation` (`self.GetOwner`))))
          (if (<= _correcteddistance (`local.Local_VisionRange`))
            (if (== (`local.Local_ActiveTargetIndex`) (`local.Local_TargetIndex`))
              (bind _outhit (`KismetSystemLibrary.LineTraceSingle` (`Actor.K2_GetActorLocation` (`self.GetOwner`)) (`Actor.K2_GetActorLocation` (`local.Local_TargetActor`)) "TraceTypeQuery2" :!label _label)) ; Line trace checks
              (bind (_bblockinghit _binitialoverlap _time _location _impactpoint _normal _impactnormal _physmat _hitactor) (`GameplayStatics.BreakHitResult` _outhit))
              (if (== (`local.Local_TargetActor`) _hitactor)
                (message `/Game/FPSTowerDefenseToolkit/Blueprints/Interfaces/BPI_VisualPerception.UpdateVisualPerceptionData` (`self.GetOwner`) true (`local.Local_TargetIndex`) (`KismetMathLibrary.VSize` (- _location (`Actor.K2_GetActorLocation` (`self.GetOwner`))))) ; Target in Range: Trace Distance information sent to owning actor
                (else
                  (message `/Game/FPSTowerDefenseToolkit/Blueprints/Interfaces/BPI_VisualPerception.UpdateVisualPerceptionData` (`self.GetOwner`) false (`local.Local_TargetIndex`) 0.0 :!label _label_2) ; Target not in Range
                ))
              (elif (<= (`KismetMathLibrary.DegAcos` (`KismetMathLibrary.Dot_VectorVector` (`Actor.GetActorForwardVector` (`self.GetOwner`)) (`KismetMathLibrary.Normal` (- (`Actor.K2_GetActorLocation` (`local.Local_TargetActor`)) (`Actor.K2_GetActorLocation` (`self.GetOwner`)))))) (`local.Local_VisionAngle`))
                (goto _label)
                (else
                  (goto _label_2))))
            (else
              (goto _label_2)))
          (else
            (goto _label_2)))))))