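; Threat response component that decides whether its owning actor attacks or approaches its active target in the tower defense toolkit.
; While active, a looping timer checks trace hit and distance against attack range, choosing attack when in range and move otherwise.
; Attacking starts a looping lock-on timer and, unless an attack animation is running, cancels movement and orders an attack; moving or deactivating clears lock-on.
; All queries and orders reach the owner as messages.
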(event `ActivateThreatResponse`
  ;[0 1 1 0.5] Activates Threat Response Evaluation
  (if (not (`self.IsActive?`))
    (set `self.IsActive?` true)
    (`self.EnableThreatResponseEvaluation`)))

(event `DeactivateThreatResponse`
  ;[0 1 1 0.5] Deactivate Threat Response Evaluation & Target Lock On
  (if (`self.IsActive?`)
    (set `self.IsActive?` false)
    (`self.ThreatResponseInstruction_DisableTargetLockOn`)
    (`self.DisableThreatResponseEvaluation`)))

(fn `DisableThreatResponseEvaluation`
  (bind _evaluatethreatresponsetoactivetargettimerhandle (`self.EvaluateThreatResponseToActiveTargetTimerHandle`))
  ;[0 1 1 0.5] Deactivates the Threat Response Evaluation timer
  (if (`KismetSystemLibrary.K2_TimerExistsHandle` _evaluatethreatresponsetoactivetargettimerhandle)
    (`KismetSystemLibrary.K2_ClearAndInvalidateTimerHandle` _evaluatethreatresponsetoactivetargettimerhandle))
  (return))

(fn `EnableThreatResponseEvaluation`
  ;[0 1 1 0.5] Activates timed threat response evaluations for the active target
  (`self.EvaluateThreatResponseToActiveTarget`)
  (bind _returnvalue (`KismetSystemLibrary.K2_SetTimer` null "EvaluateThreatResponseToActiveTarget" (`self.EvaluateThreatResponseToActiveTargetTimerInterval`) true))
  (set `self.EvaluateThreatResponseToActiveTargetTimerHandle` _returnvalue)
  (return))

(fn `EvaluateThreatResponseToActiveTarget`
  ;[0 1 1 0.5] Issues threat response instructions to the owning actor based on the spatial relation with the active target actor
  (bind (_targetdistance _tracehitsuccess_ _ownerattackrange) (message `/Game/FPSTowerDefenseToolkit/Blueprints/Interfaces/BPI_ThreatResponse.RetrieveTraceDistanceToActiveTarget` (`self.GetOwner`)))
  (if _tracehitsuccess_
    (if (< _targetdistance _ownerattackrange)
      (`self.ThreatResponseInstruction_AttackTarget`)
      (else
        (`self.ThreatResponseInstruction_MoveToTarget` :!label _label)))
    (else
      (goto _label))))

(fn `ThreatResponseInstruction_AttackTarget`
  ;[0 1 1 0.5] Requests the owner to lock on to & attack the active target
  (bind _isactive_ (message `/Game/FPSTowerDefenseToolkit/Blueprints/Interfaces/BPI_ThreatResponse.RetrieveAttackAnimationStatus` (`self.GetOwner`)))
  (if _isactive_
    (if (not (`KismetSystemLibrary.K2_TimerExistsHandle` (`self.LockOnToActiveTargetTimerHandle`)))
      (`self.ThreatResponseInstruction_LockOnToActiveTarget`)
      (bind _returnvalue (`KismetSystemLibrary.K2_SetTimer` null "ThreatResponseInstruction_LockOnToActiveTarget" (`self.LockOnToActiveTargetTimerInterval`) true))
      (set `self.LockOnToActiveTargetTimerHandle` _returnvalue))
    (else
      (message `/Game/FPSTowerDefenseToolkit/Blueprints/Interfaces/BPI_ThreatResponse.CancelMoveToActiveTarget` (`self.GetOwner`)) ; Instructs the owner to stop all movement orders
      (if (not (`KismetSystemLibrary.K2_TimerExistsHandle` (`self.LockOnToActiveTargetTimerHandle`)))
        (`self.ThreatResponseInstruction_LockOnToActiveTarget`)
        (bind _returnvalue_2 (`KismetSystemLibrary.K2_SetTimer` null "ThreatResponseInstruction_LockOnToActiveTarget" (`self.LockOnToActiveTargetTimerInterval`) true))
        (set `self.LockOnToActiveTargetTimerHandle` _returnvalue_2))
      (message `/Game/FPSTowerDefenseToolkit/Blueprints/Interfaces/BPI_ThreatResponse.AttackActiveTarget` (`self.GetOwner`)))))

(fn `ThreatResponseInstruction_DisableTargetLockOn`
  (bind _lockontoactivetargettimerhandle (`self.LockOnToActiveTargetTimerHandle`))
  ;[0 1 1 0.5] Disables the target lock on system
  (if (`KismetSystemLibrary.K2_TimerExistsHandle` _lockontoactivetargettimerhandle)
    (`KismetSystemLibrary.K2_ClearAndInvalidateTimerHandle` _lockontoactivetargettimerhandle))
  (return))

(fn `ThreatResponseInstruction_LockOnToActiveTarget`
  ;[0 1 1 0.5] Instructs the owner to keep the active target in focus
  (message `/Game/FPSTowerDefenseToolkit/Blueprints/Interfaces/BPI_ThreatResponse.KeepActiveTargetInFocus` (`self.GetOwner`)))

(fn `ThreatResponseInstruction_MoveToTarget`
  ;[0 1 1 0.5] Requests the owner to disable the lock on system & move to the active target
  (`self.ThreatResponseInstruction_DisableTargetLockOn`)
  (message `/Game/FPSTowerDefenseToolkit/Blueprints/Interfaces/BPI_ThreatResponse.MoveToActiveTarget` (`self.GetOwner`)))