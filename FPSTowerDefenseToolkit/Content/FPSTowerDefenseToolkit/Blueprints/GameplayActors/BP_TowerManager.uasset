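; Tower manager actor for a tower defense game that handles building, removing and tracking towers, tower bases and traps on the grid.
; Positions a holographic preview from trace hits on grid-linked actors, then spawns or destroys actors from tower data and updates the Grid Manager.
; At startup it builds the selectable tower list, registers editor-placed towers and initializes the HUD list.
; It also checks spawn-to-Power Core nav paths and relays focus-fire orders.
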(fn `AddNewFocusFireCallResponder`
  (params (Actor :type "Actor Object Reference"))
  ;[0 1 1 0.5] Updates the list of actors that can respond to Focus Fire orders
  (`KismetArrayLibrary.Array_Add` (`self.FocusFireCallResponders`) Actor)
  (return))

(fn `AddTowerBaseEntryToSelectedTowerDataArray`
  ;[0 1 1 0.5] Add a Tower Base data element at the top of the Selected Tower Data Array
  (for (_array_element _array_index) (`/Game/FPSTowerDefenseToolkit/Blueprints/FunctionLibraries/BPFL_GetterFunctions.GetTowerDataArray`)
    (switch `/Game/FPSTowerDefenseToolkit/Blueprints/Enums/ETowerType` (`.TowerType_2_A3E4A46A4FD032BF10E0F890A310CA0B` (break `/Game/FPSTowerDefenseToolkit/Blueprints/Structs/Struct_TowerData` _array_element))
      (:`NewEnumerator0`
        (`KismetArrayLibrary.Array_Insert` (`self.SelectedTowerClassIndexArray`) _array_index) ; Add Tower Base information  at the top of the array, since it is always selected by default
        (break))))
  (return))

(fn `CreateSelectedTowerDataArray`
  ;[0 1 1 0.5] Create/Restructure SelectedTowerDataArray to store information about the list of towers available to the player
  (if (`/Game/FPSTowerDefenseToolkit/Blueprints/BP_GameMode.SelectTowersAtLevelStart?` (cast `/Game/FPSTowerDefenseToolkit/Blueprints/BP_GameMode` (`GameplayStatics.GetGameMode`) :!pure true))
    (`self.DeleteUnselectedEntriesFromSelectedTowerDataArray`)
    (`self.AddTowerBaseEntryToSelectedTowerDataArray`)
    (else
      (for (_ _array_index) (`/Game/FPSTowerDefenseToolkit/Blueprints/FunctionLibraries/BPFL_GetterFunctions.GetTowerDataArray`)
        (`KismetArrayLibrary.Array_Set` (`self.SelectedTowerClassIndexArray`) _array_index _array_index true))))
  (bind _asbp_game_mode (cast `/Game/FPSTowerDefenseToolkit/Blueprints/BP_GameMode` (`GameplayStatics.GetGameMode`))
    (:`then`
      (set `/Game/FPSTowerDefenseToolkit/Blueprints/BP_GameMode.MaxNumberOfTowerTypes` (`KismetArrayLibrary.Array_Length` (`self.SelectedTowerClassIndexArray`)) _asbp_game_mode))
    (:`CastFailed`
      _))
  (return))

(fn `DeleteUnselectedEntriesFromSelectedTowerDataArray`
  (locals (Local_IndexDecrementValue :type Integer) (Local_NumberOfIterations :type Integer))
  ;[0 1 1 0.5] Removed all unselected entries from the Selected Tower Data Array [Unselected elements will retain the default value of '-1']
  (`KismetArrayLibrary.Array_RemoveItem` (`self.SelectedTowerClassIndexArray`) -1)
  (return))

(fn `DestroyHoloTower`
  (bind _holographictower (`self.HolographicTower`))
  ;[1 0 0 0.5] Destroy Holographic Tower actor
  (`/Engine/EditorBlueprintResources/StandardMacros.IsValid` _holographictower
    (:`Is Valid`
      (`self.K2_DestroyActor` _holographictower))
    (:`Is Not Valid`
      _))
  (return))

(fn `DestroyTower`
  (params (TowerActor :type "/Game/FPSTowerDefenseToolkit/Blueprints/Towers/BP_TowerActual_Parent Object Reference"))
  (locals (Local_HitActor :type "/Game/FPSTowerDefenseToolkit/Blueprints/Towers/BP_TowerActual_Parent Object Reference") (Local_GridGeneratorData :type "Array of /Game/FPSTowerDefenseToolkit/Blueprints/Structs/Struct_GridCellData Structure") (Local_GridVector :type "Vector Structure") (Local_TowerActor :type "/Game/FPSTowerDefenseToolkit/Blueprints/Towers/BP_TowerActual_Parent Object Reference") (Local_GridGeneratorIndex :type Integer) (Local_TowerBase :type "/Game/FPSTowerDefenseToolkit/Blueprints/Towers/BP_TowerActual_Parent Object Reference"))
  (bind _local_hitactor (`local.Local_HitActor`))
  (bind _local_toweractor (`local.Local_TowerActor`))
  (bind _local_gridgeneratorindex (`local.Local_GridGeneratorIndex`))
  (bind _gridmanagerref (`/Game/FPSTowerDefenseToolkit/Blueprints/FunctionLibraries/BPFL_GetterFunctions.GetGridManager` self))
  (bind _gridcellindex (`/Game/FPSTowerDefenseToolkit/Blueprints/Towers/BP_TowerActual_Parent.GridCellIndex` (`local.Local_HitActor`)))
  (bind (_item_floorgridindex _item_gridgeneratordata) (break `/Game/FPSTowerDefenseToolkit/Blueprints/Structs/Struct_GridData` (`KismetArrayLibrary.Array_Get` (`/Game/FPSTowerDefenseToolkit/Blueprints/FunctionLibraries/BPFL_GetterFunctions.GetGridDataArray` self) (`/Game/FPSTowerDefenseToolkit/Blueprints/Towers/BP_TowerActual_Parent.GridGeneratorIndex` (`local.Local_HitActor`)))))
  (bind ((`GridVector_10_7F7B6B8542ECC301E9FFB082D723054A` _gridvector) (`TowerBase_22_A82984B14E502491E7BEEEB7AF49775B` _towerbase) (`Tower_27_DAC62711485A5B07DF08158DC082D797` _tower)) (break `/Game/FPSTowerDefenseToolkit/Blueprints/Structs/Struct_GridCellData` (`KismetArrayLibrary.Array_Get` (`local.Local_GridGeneratorData`) (`/Game/FPSTowerDefenseToolkit/Blueprints/Towers/BP_TowerActual_Parent.GridCellIndex` (`local.Local_HitActor`)))))
  ;[1 0 0 0.5] Destroy Tower & Update Grid Data
  (set `local.Local_HitActor` TowerActor)
  (set `local.Local_GridGeneratorIndex` _item_floorgridindex)
  (set `local.Local_GridGeneratorData` _item_gridgeneratordata)
  (set `local.Local_GridVector` _gridvector)
  (set `local.Local_TowerBase` _towerbase)
  (set `local.Local_TowerActor` _tower)
  (switch `/Game/FPSTowerDefenseToolkit/Blueprints/Enums/ETowerType` (`.TowerType_2_A3E4A46A4FD032BF10E0F890A310CA0B` (break `/Game/FPSTowerDefenseToolkit/Blueprints/Structs/Struct_TowerData` (`KismetArrayLibrary.Array_Get` (`/Game/FPSTowerDefenseToolkit/Blueprints/FunctionLibraries/BPFL_GetterFunctions.GetTowerDataArray`) (`/Game/FPSTowerDefenseToolkit/Blueprints/Towers/BP_TowerActual_Parent.TowerClassIndex` (`local.Local_HitActor`)))))
    (:`NewEnumerator0`
      (`/Game/FPSTowerDefenseToolkit/Blueprints/GameplayActors/BP_GridManager.UpdateGridDataArray` (`/Game/FPSTowerDefenseToolkit/Blueprints/FunctionLibraries/BPFL_GetterFunctions.GetGridManager` self) (`/Game/FPSTowerDefenseToolkit/Blueprints/Towers/BP_TowerActual_Parent.GridCellIndex` (`local.Local_HitActor`)) (`local.Local_GridGeneratorIndex`) null null "NewEnumerator0")
      (`/Engine/EditorBlueprintResources/StandardMacros.IsValid` _local_toweractor
        (:`Is Valid`
          (`self.K2_DestroyActor` _local_toweractor))
        (:`Is Not Valid`
          _)))
    (:`NewEnumerator2`
      (`/Game/FPSTowerDefenseToolkit/Blueprints/GameplayActors/BP_GridManager.UpdateGridDataArray` _gridmanagerref _gridcellindex _local_gridgeneratorindex (`local.Local_TowerBase`) null "NewEnumerator1" :!label _label))
    (:`NewEnumerator1`
      (goto _label))
    (:`NewEnumerator3`
      (goto _label))
    (:`NewEnumerator6`
      (goto _label))
    (:`NewEnumerator4`
      (goto _label))
    (:`NewEnumerator5`
      (`/Game/FPSTowerDefenseToolkit/Blueprints/GameplayActors/BP_GridManager.UpdateGridDataArray` _gridmanagerref _gridcellindex _local_gridgeneratorindex null null "NewEnumerator0")))
  (`/Engine/EditorBlueprintResources/StandardMacros.IsValid` _local_hitactor
    (:`Is Valid`
      (`self.K2_DestroyActor` _local_hitactor))
    (:`Is Not Valid`
      _))
  (return))

(fn `DisplayHoloTower`
  (bind _holographictower (`self.HolographicTower`))
  ;[0 1 1 0.5] Display Holographic Tower & Enable collision components, if any
  (`/Engine/EditorBlueprintResources/StandardMacros.IsValid` _holographictower
    (:`Is Valid`
      (`/Game/FPSTowerDefenseToolkit/Blueprints/Towers/BP_TowerHolo_Parent.ActivateHoloTower` _holographictower))))

(fn `FocusFireOnTarget`
  (params (DesignatedTarget :type "Actor Object Reference"))
  ;[0 1 1 0.5] Requests all actors capable of manual target overrides to respond to the Focus Fire order
  (for _array_element (`self.FocusFireCallResponders`)
    (message `/Game/FPSTowerDefenseToolkit/Blueprints/Interfaces/BPI_ManualTargetOverride.ActivateFocusFireSystem` _array_element DesignatedTarget))
  (return))

(fn `HideHoloTower`
  (bind _holographictower (`self.HolographicTower`))
  ;[1 0 0 0.5] Hide Holographic Tower & Disable collision components, if any
  (`/Engine/EditorBlueprintResources/StandardMacros.IsValid` _holographictower
    (:`Is Valid`
      (`/Game/FPSTowerDefenseToolkit/Blueprints/Towers/BP_TowerHolo_Parent.DeactivateHoloTower` _holographictower))))

(fn `InitializeTowerManager`
  ;[0 1 1 0.5] Initialize the Tower Manager actor at level start
  (`self.CreateSelectedTowerDataArray`)
  (`self.UpdateGridDataWithDefaultTowers`)
  (bind _asbp_player_controller (cast `/Game/FPSTowerDefenseToolkit/Blueprints/BP_PlayerController` (`GameplayStatics.GetPlayerController` 0))
    (:`then`
      (`/Game/FPSTowerDefenseToolkit/Blueprints/BP_PlayerController.UpdateHUD_InitializeTowerListBox` _asbp_player_controller (`self.SelectedTowerClassIndexArray`)))
    (:`CastFailed`
      (`KismetSystemLibrary.PrintString` "WARNING! - Player Controller cast failed; Function - InitializeTowerManager; Class - TowerManager")))
  (return))

(fn `RemoveFocusFireCallResponder`
  (params (Actor :type "Actor Object Reference"))
  ;[0 1 1 0.5] Updates the list of actors that can respond to Focus Fire orders
  (`KismetArrayLibrary.Array_RemoveItem` (`self.FocusFireCallResponders`) Actor)
  (return))

(fn `ResizeSelectedTowerDataArrayForLoadoutMenu`
  ;[0 1 1 0.5] Used to create the default template for Tower List boxes in the Loadout Screen
  (for _ (range 1 (+ (`/Game/FPSTowerDefenseToolkit/Blueprints/BP_GameMode.RetrieveMaxNumberOfTowerTypes` (cast `/Game/FPSTowerDefenseToolkit/Blueprints/BP_GameMode` (`GameplayStatics.GetGameMode`) :!pure true)) 1))
    (`KismetArrayLibrary.Array_Add` (`self.SelectedTowerClassIndexArray`) -1) ; Set default values to '-1' [Once a tower has been selected, this index gets replaced with the tower class index
  )
  (return))

(fn `RetrieveHoloTowerGridData`
  (returns (`CanPlaceTowerHere?` :type Boolean) (GridCellIndex :type Integer) (GridGeneratorIndex :type Integer))
  ;[0 1 1 0.5] Retrieve the tower placement status as well as the grid data for the current location of the holographic tower
  (bind (_canplacetowerhere_ _gridcellindex _gridgeneratorindex) (`/Game/FPSTowerDefenseToolkit/Blueprints/Towers/BP_TowerHolo_Parent.RetrieveTowerPlacementData` (`self.HolographicTower`)))
  (return _canplacetowerhere_ _gridcellindex _gridgeneratorindex))

(fn `RetrieveSelectedTowerIndexArray`
  (returns (SelectedTowerIndexArray :type "Array of Integer"))
  ;[0 1 1 0.5] Returns the Selected Tower Class Index Array
  (return (`self.SelectedTowerClassIndexArray`)))

(fn `RetrieveTowerDataAtSelectedIndex`
  (params (Index :type Integer))
  (returns (Item :type "/Game/FPSTowerDefenseToolkit/Blueprints/Structs/Struct_TowerData Structure"))
  ;[0 1 1 0.5] Getter function to retrieve information about a specific tower
  (return (`KismetArrayLibrary.Array_Get` (`/Game/FPSTowerDefenseToolkit/Blueprints/FunctionLibraries/BPFL_GetterFunctions.GetTowerDataArray`) (`KismetArrayLibrary.Array_Get` (`self.SelectedTowerClassIndexArray`) Index))))

(fn `SetSelectedTowerIndex`
  (params (SelectedIndex :type Integer))
  ;[0 1 1 0.5] New Setter function called from the Tower Button widget
  (set `self.SelectedTowerIndex` SelectedIndex)
  (return))

(fn `SpawnHoloTower`
  (params (ActiveTowerSpawnIndex :type Integer))
  (locals (Local_SpawnTransform :type "Transform Structure"))
  ;[0 1 1 0.5] Spawn Holographic Tower based on the tower selection data obtained from player input
  (bind _returnvalue (`|SpawnActorFromClass` (`.TowerHoloClass_8_C68353AC409E8A26F3121E88812927A3` (break `/Game/FPSTowerDefenseToolkit/Blueprints/Structs/Struct_TowerData` (`KismetArrayLibrary.Array_Get` (`/Game/FPSTowerDefenseToolkit/Blueprints/FunctionLibraries/BPFL_GetterFunctions.GetTowerDataArray`) (`KismetArrayLibrary.Array_Get` (`self.SelectedTowerClassIndexArray`) ActiveTowerSpawnIndex)))) (`local.Local_SpawnTransform`) "AlwaysSpawn" "OverrideRootScale"))
  (set `self.HolographicTower` _returnvalue)
  (return))

(fn `SpawnTower`
  (params (GridCellIndex :type Integer) (GridGeneratorIndex :type Integer) (SelectedTowerSpawnIndex :type Integer))
  (returns (`RebuildNavMesh?` :type Boolean))
  (locals (Local_GridGeneratorData :type "Array of /Game/FPSTowerDefenseToolkit/Blueprints/Structs/Struct_GridCellData Structure") (Local_GridVector :type "Vector Structure") (Local_GridGeneratorRotation :type "Rotator Structure") (Local_TowerBase :type "/Game/FPSTowerDefenseToolkit/Blueprints/Towers/BP_TowerActual_Parent Object Reference") (Local_GridCellIndex :type Integer) (Local_GridGeneratorIndex :type Integer) (Local_SelectedTowerClassIndex :type Integer))
  (bind ((`TowerActualClass_11_41ABC5A1403E43ECD46758910D8A244E` _toweractualclass) (`TowerCost_5_E1AD7BEA4BEF28BC32CC68A787CFE968` _towercost)) (break `/Game/FPSTowerDefenseToolkit/Blueprints/Structs/Struct_TowerData` (`KismetArrayLibrary.Array_Get` (`/Game/FPSTowerDefenseToolkit/Blueprints/FunctionLibraries/BPFL_GetterFunctions.GetTowerDataArray`) (`local.Local_SelectedTowerClassIndex`))))
  (bind ((`TowerActualClass_11_41ABC5A1403E43ECD46758910D8A244E` _toweractualclass_2) (`TowerCost_5_E1AD7BEA4BEF28BC32CC68A787CFE968` _towercost_2) (`OutputPerCycle_40_5EC60E33458BED011A82C48845D6AF3D` _outputpercycle) (`RateOfFire_42_1D868C4D4FFB074C2303678C9CD9239A` _rateoffire) (`Range_48_39E967E0488907FD121A08BC38367E69` _range)) (break `/Game/FPSTowerDefenseToolkit/Blueprints/Structs/Struct_TowerData` (`KismetArrayLibrary.Array_Get` (`/Game/FPSTowerDefenseToolkit/Blueprints/FunctionLibraries/BPFL_GetterFunctions.GetTowerDataArray`) (`local.Local_SelectedTowerClassIndex`))))
  (bind ((`TowerActualClass_11_41ABC5A1403E43ECD46758910D8A244E` _toweractualclass_3) (`TowerCost_5_E1AD7BEA4BEF28BC32CC68A787CFE968` _towercost_3) (`OutputPerCycle_40_5EC60E33458BED011A82C48845D6AF3D` _outputpercycle_2) (`RateOfFire_42_1D868C4D4FFB074C2303678C9CD9239A` _rateoffire_2) (`Range_48_39E967E0488907FD121A08BC38367E69` _range_2)) (break `/Game/FPSTowerDefenseToolkit/Blueprints/Structs/Struct_TowerData` (`KismetArrayLibrary.Array_Get` (`/Game/FPSTowerDefenseToolkit/Blueprints/FunctionLibraries/BPFL_GetterFunctions.GetTowerDataArray`) (`local.Local_SelectedTowerClassIndex`))))
  (bind ((`GridVector_10_7F7B6B8542ECC301E9FFB082D723054A` _gridvector) (`TowerBase_22_A82984B14E502491E7BEEEB7AF49775B` _towerbase)) (break `/Game/FPSTowerDefenseToolkit/Blueprints/Structs/Struct_GridCellData` (`KismetArrayLibrary.Array_Get` (`local.Local_GridGeneratorData`) (`local.Local_GridCellIndex`))))
  (bind ((`GridGeneratorData_8_13E757544C1E18F1261E9C9C7CA2FC04` _gridgeneratordata) (`GridGenerator_11_12BAB4C14F1F8A4F6CC67291E8C35A58` _gridgenerator)) (break `/Game/FPSTowerDefenseToolkit/Blueprints/Structs/Struct_GridData` (`KismetArrayLibrary.Array_Get` (`/Game/FPSTowerDefenseToolkit/Blueprints/FunctionLibraries/BPFL_GetterFunctions.GetGridDataArray` self) (`local.Local_GridGeneratorIndex`))))
  ;[0 1 1 0.5] Spawn Actual Towers & Update the Grid Data
  (set `local.Local_GridCellIndex` GridCellIndex)
  (set `local.Local_GridGeneratorIndex` GridGeneratorIndex)
  (set `local.Local_SelectedTowerClassIndex` (`KismetArrayLibrary.Array_Get` (`self.SelectedTowerClassIndexArray`) SelectedTowerSpawnIndex))
  (set `local.Local_GridGeneratorData` _gridgeneratordata)
  (set `local.Local_GridGeneratorRotation` (`self.K2_GetActorRotation` _gridgenerator))
  (set `local.Local_GridVector` _gridvector)
  (set `local.Local_TowerBase` _towerbase)
  (switch `/Game/FPSTowerDefenseToolkit/Blueprints/Enums/ETowerType` (`.TowerType_2_A3E4A46A4FD032BF10E0F890A310CA0B` (break `/Game/FPSTowerDefenseToolkit/Blueprints/Structs/Struct_TowerData` (`KismetArrayLibrary.Array_Get` (`/Game/FPSTowerDefenseToolkit/Blueprints/FunctionLibraries/BPFL_GetterFunctions.GetTowerDataArray`) (`local.Local_SelectedTowerClassIndex`))))
    (:`NewEnumerator0`
      (bind _returnvalue (`|SpawnActorFromClass` _toweractualclass (`KismetMathLibrary.MakeTransform` (`KismetMathLibrary.MakeVector` (.x (`local.Local_GridVector`)) (.y (`local.Local_GridVector`)) (+ (.z (`local.Local_GridVector`)) (`self.TowerBaseZOffset`))) (`KismetMathLibrary.MakeRotator` 0.0 0.0 (.yaw (`local.Local_GridGeneratorRotation`))) (1.0 1.0 1.0)) "AlwaysSpawn" "OverrideRootScale" null _towercost 1.0 1.0 (`local.Local_GridCellIndex`) (`local.Local_GridGeneratorIndex`) (`local.Local_SelectedTowerClassIndex`)))
      (`/Game/FPSTowerDefenseToolkit/Blueprints/GameplayActors/BP_GridManager.UpdateGridDataArray` (`/Game/FPSTowerDefenseToolkit/Blueprints/FunctionLibraries/BPFL_GetterFunctions.GetGridManager` self) (`local.Local_GridCellIndex`) (`local.Local_GridGeneratorIndex`) _returnvalue null "NewEnumerator1")
      (return true) ; Rebuild nav mesh after placing tower bases
    )
    (:`NewEnumerator2`
      (bind _returnvalue_2 (`|SpawnActorFromClass` _toweractualclass_2 (`KismetMathLibrary.MakeTransform` (`KismetMathLibrary.MakeVector` (.x (`local.Local_GridVector`)) (.y (`local.Local_GridVector`)) (+ (.z (`local.Local_GridVector`)) (`self.TowerZOffset`))) (`KismetMathLibrary.MakeRotator` 0.0 0.0 (.yaw (`local.Local_GridGeneratorRotation`))) (1.0 1.0 1.0)) "AlwaysSpawn" "OverrideRootScale" null _towercost_2 _outputpercycle (/ 1.0 _rateoffire) (`local.Local_GridCellIndex`) (`local.Local_GridGeneratorIndex`) (`local.Local_SelectedTowerClassIndex`) _range :!label _label))
      (`/Game/FPSTowerDefenseToolkit/Blueprints/GameplayActors/BP_GridManager.UpdateGridDataArray` (`/Game/FPSTowerDefenseToolkit/Blueprints/FunctionLibraries/BPFL_GetterFunctions.GetGridManager` self) (`local.Local_GridCellIndex`) (`local.Local_GridGeneratorIndex`) (`.TowerBase_22_A82984B14E502491E7BEEEB7AF49775B` (break `/Game/FPSTowerDefenseToolkit/Blueprints/Structs/Struct_GridCellData` (`KismetArrayLibrary.Array_Get` (`.GridGeneratorData_8_13E757544C1E18F1261E9C9C7CA2FC04` (break `/Game/FPSTowerDefenseToolkit/Blueprints/Structs/Struct_GridData` (`KismetArrayLibrary.Array_Get` (`/Game/FPSTowerDefenseToolkit/Blueprints/FunctionLibraries/BPFL_GetterFunctions.GetGridDataArray` self) (`local.Local_GridGeneratorIndex`)))) (`local.Local_GridCellIndex`)))) _returnvalue_2 "NewEnumerator2"))
    (:`NewEnumerator1`
      (goto _label))
    (:`NewEnumerator3`
      (goto _label))
    (:`NewEnumerator6`
      (goto _label))
    (:`NewEnumerator4`
      (goto _label))
    (:`NewEnumerator5`
      (bind _returnvalue_3 (`|SpawnActorFromClass` _toweractualclass_3 (`KismetMathLibrary.MakeTransform` (`KismetMathLibrary.MakeVector` (.x (`local.Local_GridVector`)) (.y (`local.Local_GridVector`)) (+ (.z (`local.Local_GridVector`)) (`self.TrapZOffset`))) (`local.Local_GridGeneratorRotation`) (1.0 1.0 1.0)) "AlwaysSpawn" "OverrideRootScale" null _towercost_3 _outputpercycle_2 (/ 1.0 _rateoffire_2) (`local.Local_GridCellIndex`) (`local.Local_GridGeneratorIndex`) (`local.Local_SelectedTowerClassIndex`) _range_2))
      (`/Game/FPSTowerDefenseToolkit/Blueprints/GameplayActors/BP_GridManager.UpdateGridDataArray` (`/Game/FPSTowerDefenseToolkit/Blueprints/FunctionLibraries/BPFL_GetterFunctions.GetGridManager` self) (`local.Local_GridCellIndex`) (`local.Local_GridGeneratorIndex`) null _returnvalue_3 "NewEnumerator3")))
  (return false))

(fn `UpdateGridDataWithDefaultTowers`
  (locals (Local_GridGeneratorIndex :type Integer) (Local_GridVector :type "Vector Structure") (Local_HitLocation :type "Vector Structure" :default (0.0 0.0 0.0)) (Local_TowerActor :type "/Game/FPSTowerDefenseToolkit/Blueprints/Towers/BP_TowerActual_Parent Object Reference") (Local_GridCellIndex :type Integer))
  (bind _local_toweractor (`local.Local_TowerActor`))
  (bind _local_toweractor_2 (`local.Local_TowerActor`))
  (bind _local_toweractor_3 (`local.Local_TowerActor`))
  (bind ((`TowerBase_22_A82984B14E502491E7BEEEB7AF49775B` _towerbase) (`GridStatus_19_DCC9ADC84265C7F51239C6A83D114BA1` _gridstatus)) (break `/Game/FPSTowerDefenseToolkit/Blueprints/Structs/Struct_GridCellData` (`KismetArrayLibrary.Array_Get` (`.GridGeneratorData_8_13E757544C1E18F1261E9C9C7CA2FC04` (break `/Game/FPSTowerDefenseToolkit/Blueprints/Structs/Struct_GridData` (`KismetArrayLibrary.Array_Get` (`/Game/FPSTowerDefenseToolkit/Blueprints/FunctionLibraries/BPFL_GetterFunctions.GetGridDataArray` self) (`local.Local_GridGeneratorIndex`)))) (`local.Local_GridCellIndex`))))
  ;[0 1 1 0.5] Update Grid Data Array with Towers placed in the level editor
  (bind _outactors (`GameplayStatics.GetAllActorsOfClass` "/Game/FPSTowerDefenseToolkit/Blueprints/Towers/ActualTowers/BP_TowerBaseActual.BP_TowerBaseActual_C"))
  (for _array_element _outactors
    (bind _output_get (set `local.Local_TowerActor` _array_element))
    (bind (_gridlinkedplatformexists_ _platformactor _tracehitlocation) (`/Game/FPSTowerDefenseToolkit/Blueprints/Towers/BP_TowerActual_Parent.GetGridGeneratorPlatform` _output_get))
    (if _gridlinkedplatformexists_
      (bind (_gridcellindex _gridgeneratorindex) (message `/Game/FPSTowerDefenseToolkit/Blueprints/Interfaces/BPI_GridLink.RetrieveTraceHitGridData` _platformactor _tracehitlocation))
      (set `local.Local_GridCellIndex` _gridcellindex)
      (set `local.Local_GridGeneratorIndex` _gridgeneratorindex)
      (switch `/Game/FPSTowerDefenseToolkit/Blueprints/Enums/EGridCellStatus` (`.GridStatus_19_DCC9ADC84265C7F51239C6A83D114BA1` (break `/Game/FPSTowerDefenseToolkit/Blueprints/Structs/Struct_GridCellData` (`KismetArrayLibrary.Array_Get` (`.GridGeneratorData_8_13E757544C1E18F1261E9C9C7CA2FC04` (break `/Game/FPSTowerDefenseToolkit/Blueprints/Structs/Struct_GridData` (`KismetArrayLibrary.Array_Get` (`/Game/FPSTowerDefenseToolkit/Blueprints/FunctionLibraries/BPFL_GetterFunctions.GetGridDataArray` self) (`local.Local_GridGeneratorIndex`)))) (`local.Local_GridCellIndex`))))
        (:`NewEnumerator0`
          (`/Game/FPSTowerDefenseToolkit/Blueprints/GameplayActors/BP_GridManager.UpdateGridDataArray` (`/Game/FPSTowerDefenseToolkit/Blueprints/FunctionLibraries/BPFL_GetterFunctions.GetGridManager` self) (`local.Local_GridCellIndex`) (`local.Local_GridGeneratorIndex`) _local_toweractor_2 null "NewEnumerator1")
          (for (_array_element_2 _array_index) (`/Game/FPSTowerDefenseToolkit/Blueprints/FunctionLibraries/BPFL_GetterFunctions.GetTowerDataArray`) :!label _label
            (bind ((`TowerActualClass_11_41ABC5A1403E43ECD46758910D8A244E` _toweractualclass) (`TowerCost_5_E1AD7BEA4BEF28BC32CC68A787CFE968` _towercost) (`OutputPerCycle_40_5EC60E33458BED011A82C48845D6AF3D` _outputpercycle) (`RateOfFire_42_1D868C4D4FFB074C2303678C9CD9239A` _rateoffire) (`Range_48_39E967E0488907FD121A08BC38367E69` _range)) (break `/Game/FPSTowerDefenseToolkit/Blueprints/Structs/Struct_TowerData` _array_element_2))
            (if (== (`GameplayStatics.GetObjectClass` (`local.Local_TowerActor`)) _toweractualclass)
              (`/Game/FPSTowerDefenseToolkit/Blueprints/Towers/BP_TowerActual_Parent.SetDefaultAttributes` (`local.Local_TowerActor`) _array_index (`local.Local_GridCellIndex`) (`local.Local_GridGeneratorIndex`) _towercost _outputpercycle (/ 1.0 _rateoffire) _range)
              (break))))
        (:`NewEnumerator1`
          (`self.K2_DestroyActor` _local_toweractor_2 :!label _label_2))
        (:`NewEnumerator2`
          (goto _label_2))
        (:`NewEnumerator3`
          (goto _label_2)))
      (else
        (`self.K2_DestroyActor` (`local.Local_TowerActor`)))))
  (bind _outactors_2 (`GameplayStatics.GetAllActorsOfClass` "/Game/FPSTowerDefenseToolkit/Blueprints/Towers/ActualTowers/BP_AttackTowerActual_Parent.BP_AttackTowerActual_Parent_C"))
  (for _array_element_3 _outactors_2
    (bind _output_get_2 (set `local.Local_TowerActor` _array_element_3))
    (bind (_gridlinkedplatformexists__2 _platformactor_2 _tracehitlocation_2) (`/Game/FPSTowerDefenseToolkit/Blueprints/Towers/BP_TowerActual_Parent.GetGridGeneratorPlatform` _output_get_2))
    (if _gridlinkedplatformexists__2
      (bind (_gridcellindex_2 _gridgeneratorindex_2) (message `/Game/FPSTowerDefenseToolkit/Blueprints/Interfaces/BPI_GridLink.RetrieveTraceHitGridData` _platformactor_2 _tracehitlocation_2))
      (set `local.Local_GridCellIndex` _gridcellindex_2)
      (set `local.Local_GridGeneratorIndex` _gridgeneratorindex_2)
      (switch `/Game/FPSTowerDefenseToolkit/Blueprints/Enums/EGridCellStatus` _gridstatus
        (:`NewEnumerator0`
          _)
        (:`NewEnumerator1`
          (`/Game/FPSTowerDefenseToolkit/Blueprints/GameplayActors/BP_GridManager.UpdateGridDataArray` (`/Game/FPSTowerDefenseToolkit/Blueprints/FunctionLibraries/BPFL_GetterFunctions.GetGridManager` self) (`local.Local_GridCellIndex`) (`local.Local_GridGeneratorIndex`) _towerbase _local_toweractor "NewEnumerator2")
          (goto _label))
        (:`NewEnumerator2`
          _)
        (:`NewEnumerator3`
          _))
      (`self.K2_DestroyActor` _local_toweractor)
      (else
        (`self.K2_DestroyActor` (`local.Local_TowerActor`)))))
  (bind _outactors_3 (`GameplayStatics.GetAllActorsOfClass` "/Game/FPSTowerDefenseToolkit/Blueprints/Towers/ActualTowers/BP_TrapActual.BP_TrapActual_C"))
  (for _array_element_4 _outactors_3
    (bind _output_get_3 (set `local.Local_TowerActor` _array_element_4))
    (bind (_gridlinkedplatformexists__3 _platformactor_3 _tracehitlocation_3) (`/Game/FPSTowerDefenseToolkit/Blueprints/Towers/BP_TowerActual_Parent.GetGridGeneratorPlatform` _output_get_3))
    (if _gridlinkedplatformexists__3
      (bind (_gridcellindex_3 _gridgeneratorindex_3) (message `/Game/FPSTowerDefenseToolkit/Blueprints/Interfaces/BPI_GridLink.RetrieveTraceHitGridData` _platformactor_3 _tracehitlocation_3))
      (set `local.Local_GridCellIndex` _gridcellindex_3)
      (set `local.Local_GridGeneratorIndex` _gridgeneratorindex_3)
      (switch `/Game/FPSTowerDefenseToolkit/Blueprints/Enums/EGridCellStatus` (`.GridStatus_19_DCC9ADC84265C7F51239C6A83D114BA1` (break `/Game/FPSTowerDefenseToolkit/Blueprints/Structs/Struct_GridCellData` (`KismetArrayLibrary.Array_Get` (`.GridGeneratorData_8_13E757544C1E18F1261E9C9C7CA2FC04` (break `/Game/FPSTowerDefenseToolkit/Blueprints/Structs/Struct_GridData` (`KismetArrayLibrary.Array_Get` (`/Game/FPSTowerDefenseToolkit/Blueprints/FunctionLibraries/BPFL_GetterFunctions.GetGridDataArray` self) (`local.Local_GridGeneratorIndex`)))) (`local.Local_GridCellIndex`))))
        (:`NewEnumerator0`
          (`/Game/FPSTowerDefenseToolkit/Blueprints/GameplayActors/BP_GridManager.UpdateGridDataArray` (`/Game/FPSTowerDefenseToolkit/Blueprints/FunctionLibraries/BPFL_GetterFunctions.GetGridManager` self) (`local.Local_GridCellIndex`) (`local.Local_GridGeneratorIndex`) null _local_toweractor_3 "NewEnumerator3")
          (goto _label))
        (:`NewEnumerator1`
          _)
        (:`NewEnumerator2`
          _)
        (:`NewEnumerator3`
          _))
      (`self.K2_DestroyActor` _local_toweractor_3)
      (else
        (`self.K2_DestroyActor` (`local.Local_TowerActor`)))))
  (return))

(fn `UpdateHoloTowerState`
  (params (TraceHitLocation :type "Vector Structure") (FocusedActor :type "Actor Object Reference"))
  (locals (Local_HitActor :type "Actor Object Reference") (Local_HitLocation :type "Vector Structure" :default (0.0 0.0 0.0)))
  ;[0 1 1 0.5] Handles placement of Holographic Towers in Tower Build Mode
  (set `local.Local_HitLocation` TraceHitLocation)
  (bind _output_get (set `local.Local_HitActor` FocusedActor))
  (if (`KismetSystemLibrary.DoesImplementInterface` _output_get "/Game/FPSTowerDefenseToolkit/Blueprints/Interfaces/BPI_GridLink.BPI_GridLink_C")
    (bind (_gridcellindex _gridgeneratorindex) (message `/Game/FPSTowerDefenseToolkit/Blueprints/Interfaces/BPI_GridLink.RetrieveTraceHitGridData` (`local.Local_HitActor`) (`local.Local_HitLocation`))) ; Retrieve Grid Data at the trace hit location
    (bind ((`GridGeneratorData_8_13E757544C1E18F1261E9C9C7CA2FC04` _gridgeneratordata) (`GridGenerator_11_12BAB4C14F1F8A4F6CC67291E8C35A58` _gridgenerator)) (break `/Game/FPSTowerDefenseToolkit/Blueprints/Structs/Struct_GridData` (`KismetArrayLibrary.Array_Get` (`/Game/FPSTowerDefenseToolkit/Blueprints/FunctionLibraries/BPFL_GetterFunctions.GetGridDataArray` self) _gridgeneratorindex)))
    (bind ((`GridVector_10_7F7B6B8542ECC301E9FFB082D723054A` _gridvector) (`GridStatus_19_DCC9ADC84265C7F51239C6A83D114BA1` _gridstatus)) (break `/Game/FPSTowerDefenseToolkit/Blueprints/Structs/Struct_GridCellData` (`KismetArrayLibrary.Array_Get` _gridgeneratordata _gridcellindex)))
    (`/Game/FPSTowerDefenseToolkit/Blueprints/Towers/BP_TowerHolo_Parent.UpdateDisplayParameters` (`self.HolographicTower`) _gridcellindex _gridgeneratorindex _gridvector (`self.K2_GetActorRotation` _gridgenerator) _gridstatus (`/Game/FPSTowerDefenseToolkit/Blueprints/GameplayActors/BP_GridManager.RetrieveHalfGridCellSize` (`/Game/FPSTowerDefenseToolkit/Blueprints/FunctionLibraries/BPFL_GetterFunctions.GetGridManager` self)))
    (else
      (`self.HideHoloTower`))))

(fn `UpdateSelectedTowerDataArrayElement`
  (params (Index :type Integer) (TowerClassIndex :type Integer))
  ;[0 1 1 0.5] Updates the elements of Selected Tower Data Array
  (`KismetArrayLibrary.Array_Set` (`self.SelectedTowerClassIndexArray`) Index TowerClassIndex)
  (return))

(fn `UserConstructionScript`)

(fn `ValidateNavPath`
  (returns (`NavPathAvailable?` :type Boolean))
  (locals (`Local_ActivateTowerSpawn?` :type Boolean) (Local_TargetLocation :type "Vector Structure"))
  ;[0 1 1 0.5] Check if Nav path exists from all Enemy Spawn Points to the Power Core
  (for _array_element (`/Game/FPSTowerDefenseToolkit/Blueprints/FunctionLibraries/BPFL_GetterFunctions.GetEnemySpawnPointActors` self)
    (bind _output_get (set `local.Local_TargetLocation` (`NavigationSystem.ProjectPointToNavigation` (`self.K2_GetActorLocation` (`/Game/FPSTowerDefenseToolkit/Blueprints/FunctionLibraries/BPFL_GetterFunctions.GetPowerCore` self)))))
    (bind _returnvalue (`NavigationSystem.FindPathToLocationSynchronously` (`NavigationSystem.ProjectPointToNavigation` (`self.K2_GetActorLocation` _array_element)) _output_get))
    (bind _pathpoints (`NavigationPath.PathPoints` _returnvalue))
    (bind _returnvalue_2 (`KismetArrayLibrary.Array_Length` _pathpoints))
    (if (== _returnvalue_2 0)
      (set `local.Local_ActivateTowerSpawn?` false :!label _label)
      (break)
      (elif (== (`KismetArrayLibrary.Array_Get` _pathpoints (- _returnvalue_2 1)) (`local.Local_TargetLocation`) :`ErrorTolerance` 10.0)
        (set `local.Local_ActivateTowerSpawn?` true)
        (else
          (goto _label)))))
  (return (`local.Local_ActivateTowerSpawn?`)))