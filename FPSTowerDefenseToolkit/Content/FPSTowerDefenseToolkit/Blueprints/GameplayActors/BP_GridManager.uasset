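; BP_GridManager is the central store of level grid data for tower placement in the tower defense game.
; On manual initialization it finds every planar grid generator, assigns each an index, and builds a nested array of their cells.
; An update function rewrites one cell's tower base, tower and status by generator and cell index.
; Getters expose the data, cell size and half size precomputed in the construction script.
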(fn `InitializeGridDataArray`
  (locals (Local_GridGeneratorData :type "Array of /Game/FPSTowerDefenseToolkit/Blueprints/Structs/Struct_GridCellData Structure"))
  ;[0 1 1 0.5] Set up the base template for Grid Data Array using the Grid Generators placed throughout the level
  (bind _outactors (`GameplayStatics.GetAllActorsOfClass` (`self.PlanarGridGeneratorClassRef`)))
  (for (_array_element _array_index) _outactors
    (`/Game/FPSTowerDefenseToolkit/Blueprints/GameplayActors/BP_PlanarGridGenerator.SetGeneratorIndex` _array_element _array_index)
    (for _array_element_2 (`/Game/FPSTowerDefenseToolkit/Blueprints/Base/BP_GridGenerator.GridArray` _array_element)
      (`KismetArrayLibrary.Array_Add` (`local.Local_GridGeneratorData`) (make `/Game/FPSTowerDefenseToolkit/Blueprints/Structs/Struct_GridCellData` _array_element_2)))
    (`KismetArrayLibrary.Array_Add` (`self.GridDataArray`) (make `/Game/FPSTowerDefenseToolkit/Blueprints/Structs/Struct_GridData` (`/Game/FPSTowerDefenseToolkit/Blueprints/Base/BP_GridGenerator.GeneratorIndex` _array_element) (`local.Local_GridGeneratorData`) _array_element))
    (`KismetArrayLibrary.Array_Clear` (`local.Local_GridGeneratorData`)))
  (return))

(fn `InitializeGridManager`
  ;[0 1 1 0.5] Used to initialize the Grid Manager manually instead of relying on the Begin Play Event
  (`self.InitializeGridDataArray`)
  (return))

(fn `RetrieveGridCellSize`
  (returns (GridCellSize :type "Float (double-precision)"))
  ;[0 1 1 0.5] Getter function used by other blueprints to retrieve the default grid cell size
  (return (`self.GridCellSize`)))

(fn `RetrieveGridDataArray`
  (returns (GridDataArray :type "Array of /Game/FPSTowerDefenseToolkit/Blueprints/Structs/Struct_GridData Structure"))
  ;[0 1 1 0.5] Getter function used by other blueprints to retrieve the Grid Data Array
  (return (`self.GridDataArray`)))

(fn `RetrieveHalfGridCellSize`
  (returns (HalfGridCellSize :type "Float (double-precision)"))
  ;[0 1 1 0.5] Getter function used by other blueprints to retrieve the value of half the default grid cell size for the level
  (return (`self.HalfGridCellSize`)))

(fn `UpdateGridDataArray`
  (params (GridCellIndex :type Integer) (GridGeneratorIndex :type Integer) (TowerBase :type "/Game/FPSTowerDefenseToolkit/Blueprints/Towers/BP_TowerActual_Parent Object Reference") (TowerActor :type "/Game/FPSTowerDefenseToolkit/Blueprints/Towers/BP_TowerActual_Parent Object Reference") (GridStatus :type "/Game/FPSTowerDefenseToolkit/Blueprints/Enums/EGridCellStatus Enum"))
  (locals (Local_GridGeneratorData :type "Array of /Game/FPSTowerDefenseToolkit/Blueprints/Structs/Struct_GridCellData Structure") (Local_GridCellIndex :type Integer) (Local_GridGeneratorIndex :type Integer))
  (bind ((`FloorGridIndex_2_04C183AE4F7B8E23A5CDB4AA42FF3348` _floorgridindex) (`GridGenerator_11_12BAB4C14F1F8A4F6CC67291E8C35A58` _gridgenerator)) (break `/Game/FPSTowerDefenseToolkit/Blueprints/Structs/Struct_GridData` (`KismetArrayLibrary.Array_Get` (`self.GridDataArray`) (`local.Local_GridGeneratorIndex`))))
  ;[0 1 1 0.5] Handles update to the Grid Data Array
  (set `local.Local_GridCellIndex` GridCellIndex)
  (set `local.Local_GridGeneratorIndex` GridGeneratorIndex)
  (set `local.Local_GridGeneratorData` (`.GridGeneratorData_8_13E757544C1E18F1261E9C9C7CA2FC04` (break `/Game/FPSTowerDefenseToolkit/Blueprints/Structs/Struct_GridData` (`KismetArrayLibrary.Array_Get` (`self.GridDataArray`) (`local.Local_GridGeneratorIndex`)))))
  (`KismetArrayLibrary.Array_Set` (`local.Local_GridGeneratorData`) (`local.Local_GridCellIndex`) (make `/Game/FPSTowerDefenseToolkit/Blueprints/Structs/Struct_GridCellData` (`.GridVector_10_7F7B6B8542ECC301E9FFB082D723054A` (break `/Game/FPSTowerDefenseToolkit/Blueprints/Structs/Struct_GridCellData` (`KismetArrayLibrary.Array_Get` (`local.Local_GridGeneratorData`) (`local.Local_GridCellIndex`)))) TowerBase TowerActor GridStatus))
  (`KismetArrayLibrary.Array_Set` (`self.GridDataArray`) (`local.Local_GridGeneratorIndex`) (make `/Game/FPSTowerDefenseToolkit/Blueprints/Structs/Struct_GridData` _floorgridindex (`local.Local_GridGeneratorData`) _gridgenerator))
  (return))

(fn `UserConstructionScript`
  (set `self.HalfGridCellSize` (/ (`self.GridCellSize`) 2.0)) ; Stored as a variable to prevent the need for runtime calculations to get this value
)