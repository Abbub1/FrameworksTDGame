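; Wave manager for a tower defense FPS that runs creep waves and build phases across repeating cycles.
; StartNextWave enters combat, waits for the navmesh rebuild, then runs a unit-, group- or threat-budget-based generator through enemy spawn points.
; When spawning ends and all tracked creeps are gone, it shows mission success or allocates tower resources and optionally starts a countdown.
; The cycle number scales creeps, with threat scaling by its square root.
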(event `InitiateUnitBasedWaveGeneration`
  (bind _currentindex (`self.CurrentIndex`))
  (bind ((`CreepSpawnData_6_C86291F94B6B8B06B97CF99F2EFCC313` _creepspawndata)) (break `/Game/FPSTowerDefenseToolkit/Blueprints/Structs/Struct_WaveData` (`KismetArrayLibrary.Array_Get` (`self.WaveDataArray`) (`self.GetWaveIndexWithinCurrentCycle`))))
  (bind ((`CreepClass_2_BC7DEC434676EC1EE45BAAA39F01649B` _creepclass) (`SpawnPoint_5_6417E044448D462F83BA2F95A0695DCB` _spawnpoint) (`SpawnStartingTime_8_3347AF684F8DD88646A07698C33E9B64` _spawnstartingtime)) (break `/Game/FPSTowerDefenseToolkit/Blueprints/Structs/Struct_CreepSpawnData` (`KismetArrayLibrary.Array_Get` _creepspawndata (`self.CurrentIndex`))))
  ;[1 0.5 0.2 0.5] Spawns AI Bots on a unit by unit basis, as specified by the Designer; Allows more direct control over the spawning system, but testing can get tedious when dealing with large number of units
  (set `self.CurrentIndex` 0)
  (`KismetSystemLibrary.Delay` (- _spawnstartingtime (`self.SpawnStartingTime`)) :!label _label)
  (`/Engine/EditorBlueprintResources/StandardMacros.IsValid` _spawnpoint
    (:`Is Valid`
      (`/Game/FPSTowerDefenseToolkit/Blueprints/GameplayActors/BP_EnemySpawnPoint.SpawnCreep` _spawnpoint _creepclass (`self.CurrentCycle`))
      (if (< _currentindex (- (`KismetArrayLibrary.Array_Length` _creepspawndata) 1))
        (set `self.CurrentIndex` (+ _currentindex 1)) ; Increment the Current Index to access the spawn data for the next creep in the active wave
        (goto _label)
        (else
          (set `self.WaveSpawnOver?` true))))
    (:`Is Not Valid`
      (`KismetSystemLibrary.PrintString` "Warning: Invalid Enemy Spawn Point; Terminating Wave Generation"))))

(event `InitiateGroupBasedWaveGeneration`
  (bind _currentcycle (`self.CurrentCycle`))
  ;[1 0.5 0.2 0.5] Spawn AI Bots as groups using parameters like spawn start time, number of units in a group, spawn point, etc; Kind of a middle ground between Unit Based & Threat Based generators with regards to control over and testing the spawning system
  (set `self.NumberOfActiveSpawnGroups` 0)
  (for _array_element (`.CreepSpawnData_6_C86291F94B6B8B06B97CF99F2EFCC313` (break `/Game/FPSTowerDefenseToolkit/Blueprints/Structs/Struct_WaveData` (`KismetArrayLibrary.Array_Get` (`self.WaveDataArray`) (`self.GetWaveIndexWithinCurrentCycle`))))
    (bind ((`CreepClass_2_BC7DEC434676EC1EE45BAAA39F01649B` _creepclass) (`SpawnPoint_5_6417E044448D462F83BA2F95A0695DCB` _spawnpoint) (`SpawnStartingTime_8_3347AF684F8DD88646A07698C33E9B64` _spawnstartingtime) (`NumberOfUnits_11_8695B9FB4400F0DD8B85E5878E89BBB4` _numberofunits) (`SpawnInterval_14_7BA2E3F545E39E40D12C3EA67F4B2BE6` _spawninterval)) (break `/Game/FPSTowerDefenseToolkit/Blueprints/Structs/Struct_CreepSpawnData` _array_element))
    (`/Engine/EditorBlueprintResources/StandardMacros.IsValid` _spawnpoint
      (:`Is Valid`
        (set `self.NumberOfActiveSpawnGroups` (+ (`self.NumberOfActiveSpawnGroups`) 1))
        (switch `/Game/FPSTowerDefenseToolkit/Blueprints/Enums/EEnemyType` (defaults `/Game/FPSTowerDefenseToolkit/Blueprints/GameplayActors/BP_WaveManager` _creepclass)
          (:`NewEnumerator0`
            (`/Game/FPSTowerDefenseToolkit/Blueprints/GameplayActors/BP_EnemySpawnPoint.SpawnCreepBatch_CoreBomberClass` _spawnpoint _spawnstartingtime _numberofunits _spawninterval _creepclass _currentcycle))
          (:`NewEnumerator1`
            (`/Game/FPSTowerDefenseToolkit/Blueprints/GameplayActors/BP_EnemySpawnPoint.SpawnCreepBatch_MeleeClass` _spawnpoint _spawnstartingtime _numberofunits _spawninterval _creepclass _currentcycle))
          (:`NewEnumerator2`
            (`/Game/FPSTowerDefenseToolkit/Blueprints/GameplayActors/BP_EnemySpawnPoint.SpawnCreepBatch_RangedClass` _spawnpoint _spawnstartingtime _numberofunits _spawninterval _creepclass _currentcycle))))
      (:`Is Not Valid`
        (`KismetSystemLibrary.PrintString` "Warning: Invalid Enemy Spawn Point; Terminating Wave Generation")))))

(event `DecrementNumberOfActiveSpawnGroups`
  ;[1 0.5 0.2 0.5] Spawn AI Bots as groups using parameters like spawn start time, number of units in a group, spawn point, etc; Kind of a middle ground between Unit Based & Threat Based generators with regards to control over and testing the spawning system
  (bind _output_get (set `self.NumberOfActiveSpawnGroups` (- (`self.NumberOfActiveSpawnGroups`) 1))) ; Decrement the number of active batch spawners
  (if (not (> _output_get 0))
    (set `self.WaveSpawnOver?` true)))

(event `InitiateThreatBasedWaveGeneration`
  (bind ((`SpawnInterval_14_7BA2E3F545E39E40D12C3EA67F4B2BE6` _spawninterval) (`MaxThreatRating_16_EADF805D43B4C7313A226680A47221D7` _maxthreatrating) (`CreepClasses_20_6D0B12B04CA590C8184635BBD8A422B9` _creepclasses)) (break `/Game/FPSTowerDefenseToolkit/Blueprints/Structs/Struct_CreepSpawnData` (`KismetArrayLibrary.Array_Get` (`.CreepSpawnData_6_C86291F94B6B8B06B97CF99F2EFCC313` (break `/Game/FPSTowerDefenseToolkit/Blueprints/Structs/Struct_WaveData` (`KismetArrayLibrary.Array_Get` (`self.WaveDataArray`) (`self.GetWaveIndexWithinCurrentCycle`)))))))
  ;[1 0.5 0.2 0.5] Spawns AI Bots until the threat rating of the wave reaches the specified critical point; Bot types can be specified for each wave, but less direct control over the spawning system. However, easy to test random waves by changing bot types & Threat Rating.
  (for (_ _array_index) _creepclasses
    (`KismetArrayLibrary.Array_Add` (`self.EnemyTypeIntRefArray`) _array_index) ; Number of types of creeps in the active wave
  )
  (set `self.NextSpawnDelay` _spawninterval)
  (set `self.MaxThreatRating` (* _maxthreatrating (`KismetMathLibrary.Sqrt` (`KismetMathLibrary.Conv_IntToDouble` (`self.CurrentCycle`))))) ; Store the maximum creep threat rating for the active wave
  (if (> (`KismetArrayLibrary.Array_Length` (`self.EnemyTypeIntRefArray`)) 0) :!label _label_2
    (bind _output_get (set `self.CurrentEnemyTypeIntRef` (`self.GetRandomArrayElement` (`self.EnemyTypeIntRefArray`)))) ; Get index for any one of the designated creep types for the active wave
    (bind _item (`KismetArrayLibrary.Array_Get` _creepclasses _output_get))
    (bind _returnvalue (+ (* (`KismetMathLibrary.Sqrt` (`KismetMathLibrary.Conv_IntToDouble` (`self.CurrentCycle`))) (defaults `/Game/FPSTowerDefenseToolkit/Blueprints/EnemyAI/BP_EnemyAI_CoreBomber` _item)) (`self.CurrentThreatRating`)))
    (if (> _returnvalue (`self.MaxThreatRating`))
      (`KismetArrayLibrary.Array_RemoveItem` (`self.EnemyTypeIntRefArray`) (`self.CurrentEnemyTypeIntRef`)) ; Since the threat rating of the selected creep type > remaining threat rating points for the wave, do not consider it during the remaining iterations
      (goto _label_2)
      (else
        (`KismetSystemLibrary.Delay` (`self.NextSpawnDelay`))
        (set `self.CurrentThreatRating` _returnvalue) ; Total accumulated threat rating after spawning the creep
        (`/Game/FPSTowerDefenseToolkit/Blueprints/GameplayActors/BP_EnemySpawnPoint.SpawnCreep` (`self.GetRandomArrayElement` (`/Game/FPSTowerDefenseToolkit/Blueprints/FunctionLibraries/BPFL_GetterFunctions.GetEnemySpawnPointActors` self)) _item (`self.CurrentCycle`))
        (goto _label_2)))
    (else
      (set `self.WaveSpawnOver?` true)
      (set `self.CurrentThreatRating` 0.0))))

(event `StartNextWave`
  (bind _startwavetimerhandle (`self.StartWaveTimerHandle`))
  ;[0 1 1 0.5] Activates Combat Mode; Initializes AI spawning system based on the Wave Generator type
  (if (`KismetSystemLibrary.K2_TimerExistsHandle` _startwavetimerhandle)
    (`KismetSystemLibrary.K2_ClearAndInvalidateTimerHandle` _startwavetimerhandle) ; If player manually starts the next wave, cancel any existing Start Wave Timer
  )
  (bind _asbp_player_character (cast `/Game/FPSTowerDefenseToolkit/Blueprints/BP_PlayerCharacter` (`GameplayStatics.GetPlayerCharacter` 0))
    (:`then`
      (`/Game/FPSTowerDefenseToolkit/Blueprints/BP_PlayerCharacter.ExecuteWaveActivationPrerequisites` _asbp_player_character))
    (:`CastFailed`
      _))
  (`/Game/FPSTowerDefenseToolkit/Blueprints/BP_GameState.UpdateGameplayState` (cast `/Game/FPSTowerDefenseToolkit/Blueprints/BP_GameState` (`GameplayStatics.GetGameState`) :!pure true) "NewEnumerator2") ; Set Gameplay State to Combat Mode before starting a new wave
  (`/Game/FPSTowerDefenseToolkit/Blueprints/GameplayActors/BP_TowerManager.DestroyHoloTower` (`/Game/FPSTowerDefenseToolkit/Blueprints/FunctionLibraries/BPFL_GetterFunctions.GetTowerManager` self)) ; Destroy Holo Towers before starting a new wave
  (for _array_element (`/Game/FPSTowerDefenseToolkit/Blueprints/FunctionLibraries/BPFL_GetterFunctions.GetEnemySpawnPointActors` self)
    (`/Game/FPSTowerDefenseToolkit/Blueprints/GameplayActors/BP_EnemySpawnPoint.HideWaveSpawnInformation` _array_element))
  (`KismetSystemLibrary.Delay` 0.12)
  (if (`NavigationSystem.IsNavigationBeingBuilt`) :!label _label_3
    (`KismetSystemLibrary.Delay` 0.05)
    (goto _label_3)
    (else
      (set `self.WaveSpawnOver?` false)
      (`KismetArrayLibrary.Array_Clear` (`self.CreepActorsArray`)) ; Reset the Creep Actors Array before starting a new wave
      (switch `/Game/FPSTowerDefenseToolkit/Blueprints/Enums/EWaveGenerator` (`self.WaveGeneratorType`)
        (:`NewEnumerator0`
          (`self.InitiateUnitBasedWaveGeneration`))
        (:`NewEnumerator1`
          (`self.InitiateGroupBasedWaveGeneration`))
        (:`NewEnumerator2`
          (`self.InitiateThreatBasedWaveGeneration`))))))

(fn `AllocateTowerResources`
  (bind ((`TowerBaseAvailability_5_452A62234445A9CBD5F3FD84FD7A88CF` _towerbaseavailability) (`TowerPointAvailability_9_97DA1A3E40338BDAC473058220D3625C` _towerpointavailability)) (break `/Game/FPSTowerDefenseToolkit/Blueprints/Structs/Struct_ResourceAllocationData` (`KismetArrayLibrary.Array_Get` (`self.ResourceAllocationData`) (`self.GetWaveIndexWithinCurrentCycle`))))
  ;[0 1 1 0.5] Allocated tower bases & tower points to the player based on the wave number & data stored in the Resource Allocation Data array
  (bind _asbp_player_state (cast `/Game/FPSTowerDefenseToolkit/Blueprints/BP_PlayerState` (`Controller.PlayerState` (`GameplayStatics.GetPlayerController` 0)))
    (:`then`
      (`/Game/FPSTowerDefenseToolkit/Blueprints/BP_PlayerState.UpdateTowerBasesLeft` _asbp_player_state _towerbaseavailability)
      (`/Game/FPSTowerDefenseToolkit/Blueprints/BP_PlayerState.UpdateTowerPoints` _asbp_player_state _towerpointavailability)
      (return))
    (:`CastFailed`
      (return))))

(fn `EvaluateWaveTerminationStatus`
  (params (DestroyedCreep :type "/Game/FPSTowerDefenseToolkit/Blueprints/EnemyAI/BP_EnemyAI_Parent Object Reference"))
  ;[0 1 1 0.5] Handles Wave Termination & End Game logic
  (`KismetArrayLibrary.Array_RemoveItem` (`self.CreepActorsArray`) DestroyedCreep)
  (`self.K2_DestroyActor` DestroyedCreep)
  (if (`self.WaveSpawnOver?`)
    (if (== (`KismetArrayLibrary.Array_Length` (`self.CreepActorsArray`)) 0)
      (if (== (+ (`self.GetWaveIndexWithinCurrentCycle`) 1) (`self.WavesPerCycle`))
        (if (== (`self.CurrentCycle`) (`self.NumberOfCycles`))
          (bind _asbp_player_hud (cast `/Game/FPSTowerDefenseToolkit/Blueprints/BP_PlayerHUD` (`PlayerController.GetHUD` (`GameplayStatics.GetPlayerController` 0))))
          (`/Game/FPSTowerDefenseToolkit/Blueprints/BP_PlayerHUD.DisplayMissionSummary` _asbp_player_hud true) ; Mission Success
          (else
            (set `self.CurrentCycle` (+ (`self.CurrentCycle`) 1))
            (set `self.CurrentWave` (+ (`self.CurrentWave`) 1) :!label _label)
            (`/Game/FPSTowerDefenseToolkit/Blueprints/BP_GameState.UpdateGameplayState` (cast `/Game/FPSTowerDefenseToolkit/Blueprints/BP_GameState` (`GameplayStatics.GetGameState`) :!pure true) "NewEnumerator1")
            (`self.AllocateTowerResources`) ; Allocate Tower Resources to the player to prepare for the next wave
            (bind _asbp_player_character (cast `/Game/FPSTowerDefenseToolkit/Blueprints/BP_PlayerCharacter` (`GameplayStatics.GetPlayerCharacter` 0))
              (:`then`
                (`/Game/FPSTowerDefenseToolkit/Blueprints/BP_PlayerCharacter.SetDefaultTowerSpawn` _asbp_player_character))
              (:`CastFailed`
                _))
            (for _array_element (`/Game/FPSTowerDefenseToolkit/Blueprints/BP_GameMode.RetrieveEnemySpawnPointActors` (cast `/Game/FPSTowerDefenseToolkit/Blueprints/BP_GameMode` (`GameplayStatics.GetGameMode`) :!pure true))
              (`/Game/FPSTowerDefenseToolkit/Blueprints/GameplayActors/BP_EnemySpawnPoint.DisplayWaveSpawnInformation` _array_element) ; Display creep spawn counter data for the next wave
            )
            (bind _asbp_player_controller (cast `/Game/FPSTowerDefenseToolkit/Blueprints/BP_PlayerController` (`GameplayStatics.GetPlayerController` 0))
              (:`then`
                (`/Game/FPSTowerDefenseToolkit/Blueprints/BP_PlayerController.UpdateHUD_CurrentWaveNumber` _asbp_player_controller (`self.CurrentWave`)))
              (:`CastFailed`
                _))
            (if (`self.TimedWaveStarts?`)
              (`self.StartWaveCountDownTimer`))))
        (else
          (goto _label))))))

(fn `ExecuteWaveTimer`
  (bind _wavetimercountdownvalue (`self.WaveTimerCountDownValue`))
  ;[0 1 1 0.5] Updates the wave timer countdown in the Tower Build HUD; Starts new wave once the timer runs out
  (if (> (`self.WaveTimerCountDownValue`) 0.0)
    (bind _asbp_player_controller (cast `/Game/FPSTowerDefenseToolkit/Blueprints/BP_PlayerController` (`GameplayStatics.GetPlayerController` 0)))
    (`/Game/FPSTowerDefenseToolkit/Blueprints/BP_PlayerController.UpdateHUD_WaveCountDownTimer` _asbp_player_controller _wavetimercountdownvalue) ; Request Player Controller to handle  GameHUD updates
    (set `self.WaveTimerCountDownValue` (- _wavetimercountdownvalue 1.0))
    (else
      (`self.StartNextWave`)
      (set `self.WaveTimerCountDownValue` 0.0))))

(fn `GetWaveIndexWithinCurrentCycle`
  (returns (WaveIndex :type Integer))
  ;[0 1 1 0.5] Calculate the index of the active wave within the current cycle [Index in this context being information stored about the corresponding wave in relevant arrays]
  (return (mod (- (`self.CurrentWave`) 1) (`self.WavesPerCycle`))))

(fn `InitializeWaveManager`
  ;[0 1 1 0.5] Initialize the Wave Manager actor manually instead of relying on the Begin Play event
  (`self.ValidateResourceAllocationData`)
  (`self.AllocateTowerResources`)
  (bind _asbp_player_controller (cast `/Game/FPSTowerDefenseToolkit/Blueprints/BP_PlayerController` (`GameplayStatics.GetPlayerController` 0))
    (:`then`
      (`/Game/FPSTowerDefenseToolkit/Blueprints/BP_PlayerController.UpdateHUD_InitializeWaveNumberData` _asbp_player_controller (`self.CurrentWave`) (== (`self.NumberOfCycles`) 0) (* (`self.NumberOfCycles`) (`self.WavesPerCycle`)))
      (if (`self.TimedWaveStarts?`)
        (`self.StartWaveCountDownTimer`))
      (return))
    (:`CastFailed`
      (return))))

(fn `RetrieveCreepActorsArray`
  (returns (CreepActorsArray :type "Array of /Game/FPSTowerDefenseToolkit/Blueprints/EnemyAI/BP_EnemyAI_Parent Object Reference"))
  ;[0 1 1 0.5] Retrieves a list of all creep actors in the level
  (return (`self.CreepActorsArray`)))

(fn `RetrieveCurrentWave`
  (returns (CurrentWave :type Integer))
  ;[0 1 1 0.5] Getter function used by other blueprints to retrieve the current wave number
  (return (`self.CurrentWave`)))

(fn `RetrieveGroupBasedCreepSpawnCountData`
  (params (EnemySpawnPoint :type "/Game/FPSTowerDefenseToolkit/Blueprints/GameplayActors/BP_EnemySpawnPoint Object Reference"))
  (returns (CreepSpawnCountData :type "Array of /Game/FPSTowerDefenseToolkit/Blueprints/Structs/Struct_CreepSpawnCounter Structure"))
  (locals (Local_EnemySpawnPoint :type "/Game/FPSTowerDefenseToolkit/Blueprints/GameplayActors/BP_EnemySpawnPoint Object Reference") (Local_CreepSpawnCountData :type "Array of /Game/FPSTowerDefenseToolkit/Blueprints/Structs/Struct_CreepSpawnCounter Structure"))
  ;[0 1 1 0.5] Return creep spawn count data for the given enemy spawn point, during the upcoming wave
  (set `local.Local_EnemySpawnPoint` EnemySpawnPoint)
  (for _array_element (`.CreepSpawnData_6_C86291F94B6B8B06B97CF99F2EFCC313` (break `/Game/FPSTowerDefenseToolkit/Blueprints/Structs/Struct_WaveData` (`KismetArrayLibrary.Array_Get` (`self.WaveDataArray`) (`self.GetWaveIndexWithinCurrentCycle`))))
    (bind ((`CreepClass_2_BC7DEC434676EC1EE45BAAA39F01649B` _creepclass) (`SpawnPoint_5_6417E044448D462F83BA2F95A0695DCB` _spawnpoint) (`NumberOfUnits_11_8695B9FB4400F0DD8B85E5878E89BBB4` _numberofunits)) (break `/Game/FPSTowerDefenseToolkit/Blueprints/Structs/Struct_CreepSpawnData` _array_element))
    (if (== (`local.Local_EnemySpawnPoint`) _spawnpoint)
      (`KismetArrayLibrary.Array_Set` (`local.Local_CreepSpawnCountData`) (`KismetArrayLibrary.Array_Length` (`local.Local_CreepSpawnCountData`)) (make `/Game/FPSTowerDefenseToolkit/Blueprints/Structs/Struct_CreepSpawnCounter` _creepclass _numberofunits) true)))
  (return (`local.Local_CreepSpawnCountData`)))

(fn `RetrieveUnitBasedCreepSpawnCountData`
  (params (EnemySpawnPoint :type "/Game/FPSTowerDefenseToolkit/Blueprints/GameplayActors/BP_EnemySpawnPoint Object Reference"))
  (returns (CreepSpawnCountData :type "Array of /Game/FPSTowerDefenseToolkit/Blueprints/Structs/Struct_CreepSpawnCounter Structure"))
  (locals (Local_EnemySpawnPoint :type "/Game/FPSTowerDefenseToolkit/Blueprints/GameplayActors/BP_EnemySpawnPoint Object Reference") (Local_CreepSpawnCountData :type "Array of /Game/FPSTowerDefenseToolkit/Blueprints/Structs/Struct_CreepSpawnCounter Structure") (`Local_UseExistingArrayElement?` :type Boolean :default false) (Local_ArraySetIndex :type Integer))
  ;[0 1 1 0.5] Return creep spawn count data for the given enemy spawn point, during the upcoming wave
  (set `local.Local_EnemySpawnPoint` EnemySpawnPoint)
  (for _array_element (`.CreepSpawnData_6_C86291F94B6B8B06B97CF99F2EFCC313` (break `/Game/FPSTowerDefenseToolkit/Blueprints/Structs/Struct_WaveData` (`KismetArrayLibrary.Array_Get` (`self.WaveDataArray`) (`self.GetWaveIndexWithinCurrentCycle`))))
    (bind ((`CreepClass_2_BC7DEC434676EC1EE45BAAA39F01649B` _creepclass) (`SpawnPoint_5_6417E044448D462F83BA2F95A0695DCB` _spawnpoint)) (break `/Game/FPSTowerDefenseToolkit/Blueprints/Structs/Struct_CreepSpawnData` _array_element))
    (if (== (`local.Local_EnemySpawnPoint`) _spawnpoint)
      (for (_array_element_2 _array_index) (`local.Local_CreepSpawnCountData`)
        (bind _returnvalue (== (`.CreepClass_2_2DE533F549F279ED8122FDB2D4DAA879` (break `/Game/FPSTowerDefenseToolkit/Blueprints/Structs/Struct_CreepSpawnCounter` _array_element_2)) _creepclass))
        (if _returnvalue
          (set `local.Local_UseExistingArrayElement?` _returnvalue)
          (set `local.Local_ArraySetIndex` _array_index)
          (break)))
      (if (not (`local.Local_UseExistingArrayElement?`))
        (set `local.Local_ArraySetIndex` (`KismetArrayLibrary.Array_Length` (`local.Local_CreepSpawnCountData`))))
      (`KismetArrayLibrary.Array_Set` (`local.Local_CreepSpawnCountData`) (`local.Local_ArraySetIndex`) (make `/Game/FPSTowerDefenseToolkit/Blueprints/Structs/Struct_CreepSpawnCounter` _creepclass (+ (`.SpawnCount_5_CE1F85634C4076BE092AA08D0F7997D5` (break `/Game/FPSTowerDefenseToolkit/Blueprints/Structs/Struct_CreepSpawnCounter` (`KismetArrayLibrary.Array_Get` (`local.Local_CreepSpawnCountData`) (`local.Local_ArraySetIndex`)))) 1)) true)))
  (return (`local.Local_CreepSpawnCountData`)))

(fn `RetrieveWaveGeneratorType`
  (returns (WaveGeneratorType :type "/Game/FPSTowerDefenseToolkit/Blueprints/Enums/EWaveGenerator Enum"))
  ;[0 1 1 0.5] Getter function used by other blueprints to retrieve the wave generator type
  (return (`self.WaveGeneratorType`)))

(fn `StartWaveCountDownTimer`
  ;[0 1 1 0.5] Start the wave countdown timer
  (set `self.WaveTimerCountDownValue` (`self.WaveTimerInterval`)) ; Set Countdown Starter Value
  (bind _asbp_player_controller (cast `/Game/FPSTowerDefenseToolkit/Blueprints/BP_PlayerController` (`GameplayStatics.GetPlayerController` 0)))
  (`/Game/FPSTowerDefenseToolkit/Blueprints/BP_PlayerController.UpdateHUD_DisplayWaveCountDownTimer` _asbp_player_controller (`self.WaveTimerCountDownValue`))
  (`self.ExecuteWaveTimer`)
  (bind _returnvalue (`KismetSystemLibrary.K2_SetTimer` null "ExecuteWaveTimer" 1.0 true))
  (set `self.StartWaveTimerHandle` _returnvalue))

(fn `UpdateCreepActorsArray`
  (params (SpawnedCreepActor :type "/Game/FPSTowerDefenseToolkit/Blueprints/EnemyAI/BP_EnemyAI_Parent Object Reference (by ref)"))
  (locals (Local_SpawnTransform :type "Transform Structure"))
  ;[0 1 1 0.5] Maintains a record of all creeps present in the level
  (`KismetArrayLibrary.Array_Add` (`self.CreepActorsArray`) SpawnedCreepActor)
  (return))

(fn `UserConstructionScript`
  ;[0 1 1 0.5] Gets the number of waves per cycle based on the type of wave generator
  (set `self.WavesPerCycle` (`KismetArrayLibrary.Array_Length` (`self.WaveDataArray`))))

(fn `ValidateResourceAllocationData`
  (bind _returnvalue (`KismetArrayLibrary.Array_Length` (`self.ResourceAllocationData`)))
  (bind _returnvalue_2 (`KismetArrayLibrary.Array_Length` (`self.ResourceAllocationData`)))
  ;[0 1 1 0.5] Auto correct the number of entries in Resource Allocation Data by comparing it to the number of waves per cycle
  (if (> (`self.WavesPerCycle`) (`KismetArrayLibrary.Array_Length` (`self.ResourceAllocationData`)))
    (for _index (range 1 (+ (- (`self.WavesPerCycle`) _returnvalue_2) 1))
      (`KismetArrayLibrary.Array_Add` (`self.ResourceAllocationData`) (make `/Game/FPSTowerDefenseToolkit/Blueprints/Structs/Struct_ResourceAllocationData` (+ _index _returnvalue_2))))
    (elif (< (`self.WavesPerCycle`) (`KismetArrayLibrary.Array_Length` (`self.ResourceAllocationData`)))
      (for _ (range 1 (+ (- _returnvalue (`self.WavesPerCycle`)) 1))
        (`KismetArrayLibrary.Array_Remove` (`self.ResourceAllocationData`) (- _returnvalue 1))))))