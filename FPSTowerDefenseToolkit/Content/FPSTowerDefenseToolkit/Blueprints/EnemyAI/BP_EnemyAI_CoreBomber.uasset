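; Enemy AI bomber creep that attacks only the Power Core, blowing itself up once it gets within attack range.
; It feeds its Visual Perception component the vision settings and the core, taken from the Creep AI Manager, as sole potential target via BPI_VisualPerception.
; When perception reports the core in range, it stops, focuses on it, waits out a placeholder animation delay, applies damage and triggers its termination protocols.
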(event `/Game/FPSTowerDefenseToolkit/Blueprints/Interfaces/BPI_VisualPerception.UpdateVisualPerceptionData`
  (params (`TargetInRange?` :type Boolean) (TargetIndex :type Integer) (TargetDistance :type "Float (single-precision)"))
  (bind _creepaimanager (`/Game/FPSTowerDefenseToolkit/Blueprints/FunctionLibraries/BPFL_GetterFunctions.GetCreepAIManager` self))
  (bind _item (`KismetArrayLibrary.Array_Get` (`/Game/FPSTowerDefenseToolkit/Blueprints/EnemyAI/BP_CreepAIManager.RetrievePotentialTargetsArray` _creepaimanager) (`/Game/FPSTowerDefenseToolkit/Blueprints/EnemyAI/BP_CreepAIManager.RetrievePowerCoreIndex` _creepaimanager)))
  ;[0 1 0.4 0.5] BPI_VisualPerception interface function: Responds to target based on the information provided by the Visual Perception component
  (if (and `TargetInRange?` (< TargetDistance (`self.AttackRange`)))
    (bind _returnvalue (`AIBlueprintHelperLibrary.GetAIController` self))
    (`Controller.StopMovement` _returnvalue)
    (`self.FocusViewOnTarget` _item) ; Look at the target
    (`KismetSystemLibrary.Delay` (`self.AttackAnimationDuration`)) ; Placeholder delay for attack animation
    (`GameplayStatics.ApplyDamage` _item (`self.AttackDamage`))
    (`self.ActivateTerminationProtocols` null) ; Initiate Self Destruction logic
  ))

(fn `RetrieveVisualPerceptionRequisites`
  (returns (VisionRange :type "Float (double-precision)") (VisionAngle :type "Float (double-precision)") (ActiveTargetIndex :type Integer) (PotentialTargets :type "Array of Actor Object Reference"))
  (bind _creepaimanager (`/Game/FPSTowerDefenseToolkit/Blueprints/FunctionLibraries/BPFL_GetterFunctions.GetCreepAIManager` self))
  ;[0 1 0.4 0.5] BPI_VisualPerception interface function [Used by the Visual Perception component to retrieve information pertinent to it's working]
  (return (`self.VisionRange`) (`self.VisionAngle`) (`self.ActiveTargetIndex`) (`|MakeArray` (`KismetArrayLibrary.Array_Get` (`/Game/FPSTowerDefenseToolkit/Blueprints/EnemyAI/BP_CreepAIManager.RetrievePotentialTargetsArray` _creepaimanager) (`/Game/FPSTowerDefenseToolkit/Blueprints/EnemyAI/BP_CreepAIManager.RetrievePowerCoreIndex` _creepaimanager)))))

(fn `UserConstructionScript`
  (`parent.UserConstructionScript`))