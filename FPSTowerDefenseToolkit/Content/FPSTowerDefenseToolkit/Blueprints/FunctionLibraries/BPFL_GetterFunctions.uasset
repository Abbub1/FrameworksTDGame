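; Blueprint function library of global getters for the tower defense game's shared managers, actors and state.
; HUD state, the active HUD widget and tower data come from BP_GameInstance, so they work in any level using that instance.
; Managers, spawn points, the power core, grid data and selected towers route through BP_GameMode, while gameplay state comes from BP_GameState with a success flag.
; Game Mode and Game State getters return fallback values when their cast fails.
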(fn `GetActiveHUDWidget`
  (returns (ActiveHUDWidget :type "UserWidget Object Reference"))
  ;[0 1 1 0.5] Getter function to access the Active HUD Widget; Can be used from any level as long as the required Game Instance is set
  (return (`/Game/FPSTowerDefenseToolkit/Blueprints/BP_GameInstance.RetrieveActiveHUDWidget` (cast `/Game/FPSTowerDefenseToolkit/Blueprints/BP_GameInstance` (`GameplayStatics.GetGameInstance` null) :!pure true))))

(fn `GetCreepAIManager`
  (params (WorldContextObject :type "Object Object Reference"))
  (returns (CreepAIManager :type "/Game/FPSTowerDefenseToolkit/Blueprints/EnemyAI/BP_CreepAIManager Object Reference"))
  (bind _asbp_game_mode (cast `/Game/FPSTowerDefenseToolkit/Blueprints/BP_GameMode` (`GameplayStatics.GetGameMode` WorldContextObject))
    (:`then`
      (return (`/Game/FPSTowerDefenseToolkit/Blueprints/BP_GameMode.RetrieveCreepAIManager` _asbp_game_mode)))
    (:`CastFailed`
      (return null))))

(fn `GetEnemySpawnPointActors`
  (params (WorldContextObject :type "Object Object Reference"))
  (returns (EnemySpawnPointActors :type "Array of /Game/FPSTowerDefenseToolkit/Blueprints/GameplayActors/BP_EnemySpawnPoint Object Reference"))
  ;[0 1 1 0.5] Getter function to retrieve an array containing references to all Enemy Spawn Point actors
  (bind _asbp_game_mode (cast `/Game/FPSTowerDefenseToolkit/Blueprints/BP_GameMode` (`GameplayStatics.GetGameMode` WorldContextObject))
    (:`then`
      (return (`/Game/FPSTowerDefenseToolkit/Blueprints/BP_GameMode.RetrieveEnemySpawnPointActors` _asbp_game_mode)))
    (:`CastFailed`
      (return (`|MakeArray` null :!type "/Game/FPSTowerDefenseToolkit/Blueprints/GameplayActors/BP_EnemySpawnPoint Object Reference")))))

(fn `GetGameplayState`
  (params (WorldContextObject :type "Object Object Reference"))
  (returns (GameplayState :type "/Game/FPSTowerDefenseToolkit/Blueprints/Enums/EGameplayState Enum") (bSuccess :type Boolean))
  ;[0 1 1 0.5] Getter function to retrieve the Gameplay State
  (bind _asbp_game_state (cast `/Game/FPSTowerDefenseToolkit/Blueprints/BP_GameState` (`GameplayStatics.GetGameState` WorldContextObject))
    (:`then`
      (return (`/Game/FPSTowerDefenseToolkit/Blueprints/BP_GameState.RetrieveGameplayState` _asbp_game_state) true))
    (:`CastFailed`
      (return "NewEnumerator2" false))))

(fn `GetGridDataArray`
  (params (WorldContextObject :type "Object Object Reference"))
  (returns (GridDataArray :type "Array of /Game/FPSTowerDefenseToolkit/Blueprints/Structs/Struct_GridData Structure"))
  ;[0 1 1 0.5] Getter function to retrieve the Grid Data Array
  (bind _asbp_game_mode (cast `/Game/FPSTowerDefenseToolkit/Blueprints/BP_GameMode` (`GameplayStatics.GetGameMode` WorldContextObject))
    (:`then`
      (return (`/Game/FPSTowerDefenseToolkit/Blueprints/GameplayActors/BP_GridManager.RetrieveGridDataArray` (`/Game/FPSTowerDefenseToolkit/Blueprints/BP_GameMode.RetrieveGridManager` _asbp_game_mode))))
    (:`CastFailed`
      (return (`|MakeArray` (struct) :!type "/Game/FPSTowerDefenseToolkit/Blueprints/Structs/Struct_GridData Structure")))))

(fn `GetGridManager`
  (params (WorldContextObject :type "Object Object Reference"))
  (returns (GridManagerRef :type "/Game/FPSTowerDefenseToolkit/Blueprints/GameplayActors/BP_GridManager Object Reference"))
  ;[0 1 1 0.5] Getter function to retrieve the Grid Manager
  (bind _asbp_game_mode (cast `/Game/FPSTowerDefenseToolkit/Blueprints/BP_GameMode` (`GameplayStatics.GetGameMode` WorldContextObject))
    (:`then`
      (return (`/Game/FPSTowerDefenseToolkit/Blueprints/BP_GameMode.RetrieveGridManager` _asbp_game_mode)))
    (:`CastFailed`
      (return null))))

(fn `GetHUDState`
  (returns (HUDState :type "/Game/FPSTowerDefenseToolkit/Blueprints/Enums/EHUDState Enum"))
  ;[0 1 1 0.5] Getter function to retrieve the high level HUD state; Can be used from any level as long as the required Game Instance is set
  (return (`/Game/FPSTowerDefenseToolkit/Blueprints/BP_GameInstance.RetrieveHUDState` (cast `/Game/FPSTowerDefenseToolkit/Blueprints/BP_GameInstance` (`GameplayStatics.GetGameInstance` null) :!pure true))))

(fn `GetPowerCore`
  (params (WorldContextObject :type "Object Object Reference"))
  (returns (PowerCore :type "/Game/FPSTowerDefenseToolkit/Blueprints/GameplayActors/BP_PowerCore Object Reference"))
  ;[0 1 1 0.5] Getter function to retrieve the Power Core
  (bind _asbp_game_mode (cast `/Game/FPSTowerDefenseToolkit/Blueprints/BP_GameMode` (`GameplayStatics.GetGameMode` WorldContextObject))
    (:`then`
      (return (`/Game/FPSTowerDefenseToolkit/Blueprints/BP_GameMode.RetrievePowerCore` _asbp_game_mode)))
    (:`CastFailed`
      (return null))))

(fn `GetSelectedTowerClassIndexArray`
  (params (WorldContextObject :type "Object Object Reference"))
  (returns (SelectedTowerIndexArray :type "Array of Integer"))
  (bind _asbp_game_mode (cast `/Game/FPSTowerDefenseToolkit/Blueprints/BP_GameMode` (`GameplayStatics.GetGameMode` WorldContextObject))
    (:`then`
      (return (`/Game/FPSTowerDefenseToolkit/Blueprints/GameplayActors/BP_TowerManager.RetrieveSelectedTowerIndexArray` (`/Game/FPSTowerDefenseToolkit/Blueprints/BP_GameMode.RetrieveTowerManager` _asbp_game_mode))))
    (:`CastFailed`
      (return (`|MakeArray` -1)))))

(fn `GetTowerDataArray`
  (returns (TowerDataArray :type "Array of /Game/FPSTowerDefenseToolkit/Blueprints/Structs/Struct_TowerData Structure"))
  ;[0 1 1 0.5] Getter function to retrieve the Tower Data Array; Can be used from any level as long as the required Game Instance is set
  (return (`/Game/FPSTowerDefenseToolkit/Blueprints/BP_GameInstance.RetrieveTowerDataArray` (cast `/Game/FPSTowerDefenseToolkit/Blueprints/BP_GameInstance` (`GameplayStatics.GetGameInstance` null) :!pure true))))

(fn `GetTowerManager`
  (params (WorldContextObject :type "Object Object Reference"))
  (returns (TowerManagerRef :type "/Game/FPSTowerDefenseToolkit/Blueprints/GameplayActors/BP_TowerManager Object Reference"))
  ;[0 1 1 0.5] Getter function to retrieve the Tower Manager
  (bind _asbp_game_mode (cast `/Game/FPSTowerDefenseToolkit/Blueprints/BP_GameMode` (`GameplayStatics.GetGameMode` WorldContextObject))
    (:`then`
      (return (`/Game/FPSTowerDefenseToolkit/Blueprints/BP_GameMode.RetrieveTowerManager` _asbp_game_mode)))
    (:`CastFailed`
      (return null))))

(fn `GetWaveManager`
  (params (WorldContextObject :type "Object Object Reference"))
  (returns (WaveManager :type "/Game/FPSTowerDefenseToolkit/Blueprints/GameplayActors/BP_WaveManager Object Reference"))
  ;[0 1 1 0.5] Getter function to retrieve the Wave Manager
  (bind _asbp_game_mode (cast `/Game/FPSTowerDefenseToolkit/Blueprints/BP_GameMode` (`GameplayStatics.GetGameMode` WorldContextObject))
    (:`then`
      (return (`/Game/FPSTowerDefenseToolkit/Blueprints/BP_GameMode.RetrieveWaveManager` _asbp_game_mode)))
    (:`CastFailed`
      (return null))))