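; Floor trap tower for tower defense that periodically damages every enemy inside its box collision.
; An overlap wakes a deactivated trap, which applies damage on a looping timer, recharges, then re-fires if targets remain, tinting its dynamic material per state.
; Interface events handle upgrades, selling and HUD stats through player tower points.
; The construction script charges the cost when a game state exists, otherwise snaps to the grid platform for editor placement.
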(event `self.ReceiveBeginPlay`
  ;[0 1 1 0.5] Updates the Total Setup Cost parameter
  (set `self.TotalSetupCost` (`.TowerCost_5_E1AD7BEA4BEF28BC32CC68A787CFE968` (break `/Game/FPSTowerDefenseToolkit/Blueprints/Structs/Struct_TowerData` (`KismetArrayLibrary.Array_Get` (`/Game/FPSTowerDefenseToolkit/Blueprints/FunctionLibraries/BPFL_GetterFunctions.GetTowerDataArray`) (`self.TowerClassIndex`))))))

(event `self.BoxCollision.OnComponentBeginOverlap`
  (params (OverlappedComponent :type "PrimitiveComponent Object Reference") (OtherActor :type "Actor Object Reference") (OtherComp :type "PrimitiveComponent Object Reference") (OtherBodyIndex :type Integer) (bFromSweep :type Boolean) (SweepResult :type "HitResult Structure (by ref)"))
  ;[1 0.5 0.2 0.5] Detect enemy units; Activate trap if it is currently in deactivated state
  (bind _asbp_enemy_ai_parent (cast `/Game/FPSTowerDefenseToolkit/Blueprints/EnemyAI/BP_EnemyAI_Parent` OtherActor))
  (switch `/Game/FPSTowerDefenseToolkit/Blueprints/Enums/ETowerStatus` (`self.TrapStatus`)
    (:`NewEnumerator0`
      (`KismetArrayLibrary.Array_Add` (`self.EnemyUnitsInRangeArray`) _asbp_enemy_ai_parent :!label _label))
    (:`NewEnumerator1`
      (goto _label))
    (:`NewEnumerator2`
      (`KismetArrayLibrary.Array_Add` (`self.EnemyUnitsInRangeArray`) _asbp_enemy_ai_parent)
      ;[1 0 0 0.5] Apply flame damage to enemy units; Recharge the trap & Finally check for new targets
      (set `self.TrapStatus` "NewEnumerator0" :!label _label_2)
      (`MaterialInstanceDynamic.SetVectorParameterValue` (`self.MID_Trap`) "Color" (struct :`G` 1.0 :`B` 1.0 :`A` 1.0))
      (bind _returnvalue (`KismetSystemLibrary.K2_SetTimer` null "AttackEnemyUnits" (`self.ApplyDamageInterval`) true))
      (set `self.AttackTimerHandle` _returnvalue)
      (`KismetSystemLibrary.Delay` (`self.ActiveTrapDuration`)) ; Attack Enemy Units for a specified amount of time
      (`KismetSystemLibrary.K2_ClearAndInvalidateTimerHandle` (`self.AttackTimerHandle`)) ; Stop attack timer
      (set `self.TrapStatus` "NewEnumerator1") ; Switch to recharge mode
      (`MaterialInstanceDynamic.SetVectorParameterValue` (`self.MID_Trap`) "Color" (struct :`R` 0.25 :`G` 0.25 :`B` 0.25 :`A` 1.0))
      (`KismetSystemLibrary.Delay` (`self.RechargeTime`)) ; Wait to recharge the trap
      (`self.AcquireNewTarget`) ; Check for overlapping targets again
    )))

(event `AcquireNewTarget`
  ;[0 1 1 0.5] Check for enemy units in range; Deactivate the trap if none detected, else Initiate attack logic
  (if (> (`KismetArrayLibrary.Array_Length` (`self.EnemyUnitsInRangeArray`)) 0)
    (goto _label_2)
    (else
      (set `self.TrapStatus` "NewEnumerator2")
      (`MaterialInstanceDynamic.SetVectorParameterValue` (`self.MID_Trap`) "Color" (struct :`R` 1.0 :`G` 1.0 :`B` 1.0 :`A` 1.0)))))

(event `self.ReturnTowerResources`
  ;[0 1 0.4 0.5] Automatically update tower resources at creation & deletion of implementing actors
  (bind _asbp_player_state (cast `/Game/FPSTowerDefenseToolkit/Blueprints/BP_PlayerState` (`Controller.PlayerState` (`GameplayStatics.GetPlayerController` 0))))
  (`/Game/FPSTowerDefenseToolkit/Blueprints/BP_PlayerState.UpdateTowerPoints` _asbp_player_state (`self.CalculateSellingPrice`)))

(event `self.BoxCollision.OnComponentEndOverlap`
  (params (OverlappedComponent :type "PrimitiveComponent Object Reference") (OtherActor :type "Actor Object Reference") (OtherComp :type "PrimitiveComponent Object Reference") (OtherBodyIndex :type Integer))
  ;[1 0 0 0.5] Update EnemyUnitsInRangeArray
  (bind _asbp_enemy_ai_parent (cast `/Game/FPSTowerDefenseToolkit/Blueprints/EnemyAI/BP_EnemyAI_Parent` OtherActor))
  (if (`KismetArrayLibrary.Array_Contains` (`self.EnemyUnitsInRangeArray`) _asbp_enemy_ai_parent)
    (`KismetArrayLibrary.Array_RemoveItem` (`self.EnemyUnitsInRangeArray`) _asbp_enemy_ai_parent)))

(event `self.UseTowerResources`
  (params (ResourceAmount :type Integer))
  ;[0 1 0.4 0.5] Automatically update tower resources at creation & deletion of implementing actors
  (bind _asbp_player_state (cast `/Game/FPSTowerDefenseToolkit/Blueprints/BP_PlayerState` (`Controller.PlayerState` (`GameplayStatics.GetPlayerController` 0))))
  (`/Game/FPSTowerDefenseToolkit/Blueprints/BP_PlayerState.UpdateTowerPoints` _asbp_player_state (* ResourceAmount -1)))

(event `/Game/FPSTowerDefenseToolkit/Blueprints/Interfaces/BPI_HUDStatsUpdates.DisplayHUDStats`
  (bind _range (`self.Range`))
  (bind _towerlevel (`self.TowerLevel`))
  (bind _returnvalue (/ (`self.OutputPerCycle`) (`self.RechargeTime`)))
  (bind ((`TowerType_2_A3E4A46A4FD032BF10E0F890A310CA0B` _towertype) (`MaxUpgradeLevel_45_9AD5995F47810E3D0838F498F7F7A66E` _maxupgradelevel)) (break `/Game/FPSTowerDefenseToolkit/Blueprints/Structs/Struct_TowerData` (`KismetArrayLibrary.Array_Get` (`/Game/FPSTowerDefenseToolkit/Blueprints/FunctionLibraries/BPFL_GetterFunctions.GetTowerDataArray`) (`self.TowerClassIndex`))))
  (bind _returnvalue_2 (> _maxupgradelevel (`self.TowerLevel`)))
  ;[0 1 0.4 0.5] 'BPI_HUDStatsUpdates' interface function to display tower upgrade stats when focused by the player camera
  (switch `/Game/FPSTowerDefenseToolkit/Blueprints/Enums/EGameplayState` (`/Game/FPSTowerDefenseToolkit/Blueprints/FunctionLibraries/BPFL_GetterFunctions.GetGameplayState` self)
    (:`NewEnumerator0`
      (bind _asbp_player_controller (cast `/Game/FPSTowerDefenseToolkit/Blueprints/BP_PlayerController` (`GameplayStatics.GetPlayerController` 0)))
      (if _returnvalue_2
        (bind (_upgradedtowerlevel _upgradedoutputpercycle _upgradedrechargetime _upgradedrange) (`self.CalculateUpgradedTowerAttributes`))
        (`/Game/FPSTowerDefenseToolkit/Blueprints/BP_PlayerController.UpdateHUD_DisplayTowerUpgradeStats` _asbp_player_controller (`KismetTextLibrary.Conv_StringToText` (`|GetEnumeratorNameAsString` (`.TowerType_2_A3E4A46A4FD032BF10E0F890A310CA0B` (break `/Game/FPSTowerDefenseToolkit/Blueprints/Structs/Struct_TowerData` (`KismetArrayLibrary.Array_Get` (`/Game/FPSTowerDefenseToolkit/Blueprints/FunctionLibraries/BPFL_GetterFunctions.GetTowerDataArray`) (`self.TowerClassIndex`)))))) (`self.TowerLevel`) (/ (`self.OutputPerCycle`) (`self.RechargeTime`)) (`self.Range`) _returnvalue_2 _upgradedtowerlevel (/ _upgradedoutputpercycle _upgradedrechargetime) _upgradedrange (`self.CalculateTowerUpgradeCost`))
        (else
          (`/Game/FPSTowerDefenseToolkit/Blueprints/BP_PlayerController.UpdateHUD_DisplayTowerUpgradeStats` _asbp_player_controller (`KismetTextLibrary.Conv_StringToText` (`|GetEnumeratorNameAsString` _towertype)) _towerlevel _returnvalue _range _returnvalue_2 _towerlevel _returnvalue _range 0))))))

(event `/Game/FPSTowerDefenseToolkit/Blueprints/Interfaces/BPI_TowerFunctions.SellTower`
  ;[0 1 0.4 0.5] 'BPI_TowerFunctions' interface function to automatically handle return of tower resources & pre termination protocols
  (`self.ReturnTowerResources`)
  (`/Game/FPSTowerDefenseToolkit/Blueprints/BP_GameMode.ReportTowerPendingDestroy` (cast `/Game/FPSTowerDefenseToolkit/Blueprints/BP_GameMode` (`GameplayStatics.GetGameMode`) :!pure true) self) ; Let Game Mode handle the pre termination protocols
)

(event `/Game/FPSTowerDefenseToolkit/Blueprints/Interfaces/BPI_TowerFunctions.UpgradeTower`
  ;[0 1 0.4 0.5] 'BPI_TowerFunctions' interface function to handle tower upgrades
  (bind (_success_ _upgradecost) (`self.EvaluateTowerUpgradeRequirements`))
  (if _success_
    (`self.SetUpgradedTowerAttributes` _upgradecost)
    (`self.UseTowerResources` _upgradecost)))

(fn `AttackEnemyUnits`
  ;[1 0 0 0.5] Attack all enemy units in range
  (for _array_element (`self.EnemyUnitsInRangeArray`)
    (`/Engine/EditorBlueprintResources/StandardMacros.IsValid` _array_element
      (:`Is Valid`
        (`GameplayStatics.ApplyDamage` _array_element (`self.OutputPerCycle`) null self))))
  (return))

(fn `CalculateSellingPrice`
  (returns (Returns :type Integer))
  ;[0 1 1 0.5] Overrides parent function; When selling a tower, the player receives tower resources back base on the total cost invested in the tower as well as a the unique Sell Modifer Cost for the tower
  (return (`KismetMathLibrary.FTrunc` (* (`self.TotalSetupCost`) (`.SellModifier_Cost_37_B09C6F514D028EF1AC97DEA8283A8420` (break `/Game/FPSTowerDefenseToolkit/Blueprints/Structs/Struct_TowerData` (`KismetArrayLibrary.Array_Get` (`/Game/FPSTowerDefenseToolkit/Blueprints/FunctionLibraries/BPFL_GetterFunctions.GetTowerDataArray`) (`self.TowerClassIndex`))))))))

(fn `CalculateTowerUpgradeCost`
  (returns (UpgradeCost :type Integer))
  (bind ((`TowerCost_5_E1AD7BEA4BEF28BC32CC68A787CFE968` _towercost) (`UpgradeModifier_Cost_32_50551FE946FF406F676A2DBBA10A1BB5` _upgrademodifier_cost)) (break `/Game/FPSTowerDefenseToolkit/Blueprints/Structs/Struct_TowerData` (`KismetArrayLibrary.Array_Get` (`/Game/FPSTowerDefenseToolkit/Blueprints/FunctionLibraries/BPFL_GetterFunctions.GetTowerDataArray`) (`self.TowerClassIndex`))))
  ;[0 1 1 0.5] Calculates the amount of resources required to upgrade the tower based on it's level & the unique upgrade modifier cost
  (return (`KismetMathLibrary.FTrunc` (* _towercost (`KismetMathLibrary.MultiplyMultiply_FloatFloat` _upgrademodifier_cost (`KismetMathLibrary.Conv_IntToDouble` (`self.TowerLevel`)))))))

(fn `EvaluateTowerUpgradeRequirements`
  (returns (`Success?` :type Boolean) (UpgradeCost :type Integer))
  (locals (Local_TowerUpgradeCost :type Integer))
  ;[0 1 1 0.5] Checks if the tower can be upgraded based on it's tower level as well as the availability of tower resources
  (bind _asbp_player_state (cast `/Game/FPSTowerDefenseToolkit/Blueprints/BP_PlayerState` (`Controller.PlayerState` (`GameplayStatics.GetPlayerController` 0)))
    (:`then`
      (set `local.Local_TowerUpgradeCost` (`self.CalculateTowerUpgradeCost`))
      (return (and (>= (`/Game/FPSTowerDefenseToolkit/Blueprints/BP_PlayerState.RetrieveTowerPoints` _asbp_player_state) (`local.Local_TowerUpgradeCost`)) (< (`self.TowerLevel`) (`.MaxUpgradeLevel_45_9AD5995F47810E3D0838F498F7F7A66E` (break `/Game/FPSTowerDefenseToolkit/Blueprints/Structs/Struct_TowerData` (`KismetArrayLibrary.Array_Get` (`/Game/FPSTowerDefenseToolkit/Blueprints/FunctionLibraries/BPFL_GetterFunctions.GetTowerDataArray`) (`self.TowerClassIndex`)))))) (`local.Local_TowerUpgradeCost`)))
    (:`CastFailed`
      (return false 0))))

(fn `UserConstructionScript`
  (locals (Local_GridGenerator :type "/Game/FPSTowerDefenseToolkit/Blueprints/GameplayActors/BP_PlanarGridGenerator Object Reference"))
  ;[0 1 1 0.5] Check location in World space to determine if it should be decommissioned; Anchors Floor Traps to the Grid Floor
  (bind _returnvalue (`KismetMaterialLibrary.CreateDynamicMaterialInstance` "/Game/FPSTowerDefenseToolkit/Materials/M_Basic.M_Basic"))
  (bind _output_get (set `self.MID_Trap` _returnvalue))
  (`PrimitiveComponent.SetMaterial` (`self.Tower`) 0 _output_get)
  (cast `/Game/FPSTowerDefenseToolkit/Blueprints/BP_GameState` (`GameplayStatics.GetGameState`) ; Make sure that grid snapping is executed only when placing the trap in the editor
    (:`then`
      (`self.UseTowerResources` (`.TowerCost_5_E1AD7BEA4BEF28BC32CC68A787CFE968` (break `/Game/FPSTowerDefenseToolkit/Blueprints/Structs/Struct_TowerData` (`KismetArrayLibrary.Array_Get` (`/Game/FPSTowerDefenseToolkit/Blueprints/FunctionLibraries/BPFL_GetterFunctions.GetTowerDataArray`) (`self.TowerClassIndex`))))))
    (:`CastFailed`
      (bind (_gridlinkedplatformexists_ _platformactor _tracehitlocation) (`self.GetGridGeneratorPlatform`)) ; Checks for an underlying grid generator platform
      (if _gridlinkedplatformexists_
        (bind _asbp_planar_grid_generator (cast `/Game/FPSTowerDefenseToolkit/Blueprints/GameplayActors/BP_PlanarGridGenerator` _platformactor))
        (bind _output_get_2 (set `local.Local_GridGenerator` _asbp_planar_grid_generator))
        (bind (_gridcellindex _gridgeneratorindex _gridvector) (`/Game/FPSTowerDefenseToolkit/Blueprints/GameplayActors/BP_PlanarGridGenerator.RetrieveTraceHitGridData` _output_get_2 _tracehitlocation))
        (`self.K2_SetActorTransform` (`KismetMathLibrary.MakeTransform` _gridvector (`self.K2_GetActorRotation` (`local.Local_GridGenerator`))) false true) ; Snaps to Grid
      ))))