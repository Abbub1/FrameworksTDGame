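; BP_TrapHolo is the holographic preview for placing traps on the tower defense grid.
; On each display update it builds a transform from the focused cell, grid rotation and TowerManager's trap Z offset.
; Empty cells show the hologram as placeable only if the player's tower points cover the selected tower's cost.
; Trap cells show it as unplaceable, while tower or tower base cells deactivate it.
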(event `self.UpdateDisplayParameters`
  (params (GridCellIndex :type Integer) (GridGeneratorIndex :type Integer) (GridVector :type "Vector Structure") (GridGeneratorRotation :type "Rotator Structure") (GridCellStatus :type "/Game/FPSTowerDefenseToolkit/Blueprints/Enums/EGridCellStatus Enum" :default "NewEnumerator0") (HalfGridSize :type "Float (single-precision)"))
  ;[0 1 1 0.5] Updates display parameters based on input passed in from Tower Spawn Handler; Determines the state of the Holographic Tower
  (`parent.UpdateDisplayParameters` GridCellIndex GridGeneratorIndex GridVector GridGeneratorRotation GridCellStatus HalfGridSize)
  (bind _actortransform (`self.CreateNewActorTransform` (`self.FocusedGridVector`) (`self.FocusedGridGeneratorRotation`)))
  (set `self.NewActorTransform` _actortransform)
  (switch `/Game/FPSTowerDefenseToolkit/Blueprints/Enums/EGridCellStatus` (`self.FocusedGridCellStatus`)
    (:`NewEnumerator0`
      (bind _success_ (`self.EvaluateTowerResourceRequirements`))
      (`self.UpdateTowerPlacementStatus` _success_)
      (`self.K2_SetActorTransform` (`self.NewActorTransform`) :!label _label)
      (`self.SetHologramColor`)
      (`self.ActivateHoloTower`))
    (:`NewEnumerator1`
      (`self.DeactivateHoloTower` :!label _label_2))
    (:`NewEnumerator2`
      (goto _label_2))
    (:`NewEnumerator3`
      (`self.UpdateTowerPlacementStatus` false)
      (goto _label))))

(fn `CreateNewActorTransform`
  (params (GridVector :type "Vector Structure") (GridGeneratorRotation :type "Rotator Structure"))
  (returns (ActorTransform :type "Transform Structure"))
  ;[0 1 1 0.5] Creates new transform based on the focused grid cell & rotation of the focused grid generator
  (return (`KismetMathLibrary.MakeTransform` (`KismetMathLibrary.MakeVector` (.x GridVector) (.y GridVector) (+ (.z GridVector) (`/Game/FPSTowerDefenseToolkit/Blueprints/GameplayActors/BP_TowerManager.TrapZOffset` (`/Game/FPSTowerDefenseToolkit/Blueprints/FunctionLibraries/BPFL_GetterFunctions.GetTowerManager` self)))) GridGeneratorRotation (`self.HoloTowerScale`))))

(fn `EvaluateTowerResourceRequirements`
  (returns (`Success?` :type Boolean))
  (bind _asbp_player_character (cast `/Game/FPSTowerDefenseToolkit/Blueprints/BP_PlayerCharacter` (`GameplayStatics.GetPlayerCharacter` 0))
    (:`then`
      (bind _asbp_player_state (cast `/Game/FPSTowerDefenseToolkit/Blueprints/BP_PlayerState` (`Pawn.PlayerState` _asbp_player_character))
        (:`then`
          (return (>= (`/Game/FPSTowerDefenseToolkit/Blueprints/BP_PlayerState.RetrieveTowerPoints` _asbp_player_state) (`.TowerCost_5_E1AD7BEA4BEF28BC32CC68A787CFE968` (break `/Game/FPSTowerDefenseToolkit/Blueprints/Structs/Struct_TowerData` (`/Game/FPSTowerDefenseToolkit/Blueprints/GameplayActors/BP_TowerManager.RetrieveTowerDataAtSelectedIndex` (`/Game/FPSTowerDefenseToolkit/Blueprints/FunctionLibraries/BPFL_GetterFunctions.GetTowerManager` self) (`/Game/FPSTowerDefenseToolkit/Blueprints/BP_PlayerCharacter.RetrieveActiveTowerSpawnIndex` _asbp_player_character)))))))
        (:`CastFailed`
          (return false))))
    (:`CastFailed`
      (return false))))

(fn `UserConstructionScript`
  (`parent.UserConstructionScript`))