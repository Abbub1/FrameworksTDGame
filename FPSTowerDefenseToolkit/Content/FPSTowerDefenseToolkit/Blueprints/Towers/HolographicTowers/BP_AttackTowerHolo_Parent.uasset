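; Parent Blueprint for holographic attack towers that preview tower placement on the focused grid cell.
; Display updates from the Tower Spawn Handler snap the hologram to the cell, using the grid's yaw and the manager's Z offset.
; It shows only on Tower Base or Tower cells, and hides if the player is too close.
; Placement is valid only on a Tower Base with enough player tower points, and the hologram color is then refreshed.
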(event `self.UpdateDisplayParameters`
  (params (GridCellIndex :type Integer) (GridGeneratorIndex :type Integer) (GridVector :type "Vector Structure") (GridGeneratorRotation :type "Rotator Structure") (GridCellStatus :type "/Game/FPSTowerDefenseToolkit/Blueprints/Enums/EGridCellStatus Enum" :default "NewEnumerator0") (HalfGridSize :type "Float (single-precision)"))
  ;[0 1 1 0.5] Updates display parameters based on input passed in from Tower Spawn Handler; Determines the state of the Holographic Tower
  (`parent.UpdateDisplayParameters` GridCellIndex GridGeneratorIndex GridVector GridGeneratorRotation GridCellStatus HalfGridSize)
  (bind _actortransform (`self.CreateNewActorTransform` (`self.FocusedGridVector`) (`self.FocusedGridGeneratorRotation`)))
  (set `self.NewActorTransform` _actortransform)
  (bind _success_ (`self.ValidateDistanceToPlayerCharacter` (`self.FocusedGridVector`) (`self.HalfGridSize`)))
  (if _success_
    (switch `/Game/FPSTowerDefenseToolkit/Blueprints/Enums/EGridCellStatus` (`self.FocusedGridCellStatus`)
      (:`NewEnumerator0`
        (`self.DeactivateHoloTower` :!label _label))
      (:`NewEnumerator1`
        (bind _success__2 (`self.EvaluateTowerResourceRequirements`))
        (`self.UpdateTowerPlacementStatus` _success__2)
        (`self.K2_SetActorTransform` (`self.NewActorTransform`) :!label _label_2)
        (`self.SetHologramColor`)
        (`self.ActivateHoloTower`))
      (:`NewEnumerator2`
        (`self.UpdateTowerPlacementStatus` false)
        (goto _label_2))
      (:`NewEnumerator3`
        (goto _label)))
    (else
      (goto _label))))

(fn `CreateNewActorTransform`
  (params (GridVector :type "Vector Structure") (GridGeneratorRotation :type "Rotator Structure"))
  (returns (ActorTransform :type "Transform Structure"))
  ;[0 1 1 0.5] Creates new transform based on the focused grid cell & rotation of the focused grid generator
  (return (`KismetMathLibrary.MakeTransform` (`KismetMathLibrary.MakeVector` (.x GridVector) (.y GridVector) (+ (.z GridVector) (`/Game/FPSTowerDefenseToolkit/Blueprints/GameplayActors/BP_TowerManager.TowerZOffset` (`/Game/FPSTowerDefenseToolkit/Blueprints/FunctionLibraries/BPFL_GetterFunctions.GetTowerManager` self)))) (`KismetMathLibrary.MakeRotator` 0.0 0.0 (.yaw GridGeneratorRotation)) (`self.HoloTowerScale`))))

(fn `EvaluateTowerResourceRequirements`
  (returns (`Success?` :type Boolean))
  (bind _asbp_player_character (cast `/Game/FPSTowerDefenseToolkit/Blueprints/BP_PlayerCharacter` (`GameplayStatics.GetPlayerCharacter` 0))
    (:`then`
      (bind _asbp_player_state (cast `/Game/FPSTowerDefenseToolkit/Blueprints/BP_PlayerState` (`Pawn.PlayerState` _asbp_player_character))
        (:`then`
          (return (>= (`/Game/FPSTowerDefenseToolkit/Blueprints/BP_PlayerState.RetrieveTowerPoints` _asbp_player_state) (`.TowerCost_5_E1AD7BEA4BEF28BC32CC68A787CFE968` (break `/Game/FPSTowerDefenseToolkit/Blueprints/Structs/Struct_TowerData` (`/Game/FPSTowerDefenseToolkit/Blueprints/GameplayActors/BP_TowerManager.RetrieveTowerDataAtSelectedIndex` (`/Game/FPSTowerDefenseToolkit/Blueprints/FunctionLibraries/BPFL_GetterFunctions.GetTowerManager` self) (`/Game/FPSTowerDefenseToolkit/Blueprints/BP_PlayerCharacter.RetrieveActiveTowerSpawnIndex` _asbp_player_character)))))))
        (:`CastFailed`
          (return false))))
    (:`CastFailed`
      (return false))))

(fn `UserConstructionScript`
  (`parent.UserConstructionScript`))

(fn `ValidateDistanceToPlayerCharacter`
  (params (SpawnVector :type "Vector Structure") (MinRequiredDistance :type "Float (double-precision)"))
  (returns (`Success?` :type Boolean))
  ;[0 1 1 0.5] Makes sure that towers do not spawn if player is blocking the spawn position
  (return (> (`KismetMathLibrary.VSize` (- SpawnVector (`self.K2_GetActorLocation` (`GameplayStatics.GetPlayerCharacter` 0)))) MinRequiredDistance)))