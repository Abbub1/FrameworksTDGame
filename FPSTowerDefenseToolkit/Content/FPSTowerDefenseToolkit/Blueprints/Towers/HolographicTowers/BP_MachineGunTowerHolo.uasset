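; Holographic preview variant of the machine gun tower, built on a parent holo tower Blueprint.
; It extends the parent's activate and deactivate events to show or hide an added tower gun mesh along with the base hologram.
; The construction script applies the inherited holo material to that gun mesh so it matches the rest of the preview.
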(event `self.ActivateHoloTower`
  ;[0 1 1 0.5] Extend parent functions to display/hide tower gun
  (`parent.ActivateHoloTower`)
  (`SceneComponent.SetHiddenInGame` (`self.TowerGunHolo`) false false))

(event `self.DeactivateHoloTower`
  ;[0 1 1 0.5] Extend parent functions to display/hide tower gun
  (`parent.DeactivateHoloTower`)
  (`SceneComponent.SetHiddenInGame` (`self.TowerGunHolo`) true false))

(fn `UserConstructionScript`
  (`parent.UserConstructionScript`)
  (`PrimitiveComponent.SetMaterial` (`self.TowerGunHolo`) 0 (`self.HoloMaterial`)))