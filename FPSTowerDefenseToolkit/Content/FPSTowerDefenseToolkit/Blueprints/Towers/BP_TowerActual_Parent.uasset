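; Base tower class for the tower defense toolkit, holding per-instance grid placement, level, cost and combat stats.
; Static data comes from the Tower Data Array, whose modifiers scale upgrades, while Boost Tower bonuses are divided out and reapplied to output.
; It answers grid link queries and can trace down to find the platform beneath editor-placed towers.
; HUD display, upgrade, sell and resource functions are stubs for child classes.
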(event `/Game/FPSTowerDefenseToolkit/Blueprints/Interfaces/BPI_HUDStatsUpdates.DisplayHUDStats`
  ;[0 1 0.4 0.5] 'BPI_HUDStatsUpdates' interface function; Implemented through child classes
)

(event `/Game/FPSTowerDefenseToolkit/Blueprints/Interfaces/BPI_TowerFunctions.UpgradeTower`
  ;[0 1 0.4 0.5] 'BPI_TowerFunctions' interface function; Implemented through child classes
)

(event `/Game/FPSTowerDefenseToolkit/Blueprints/Interfaces/BPI_TowerFunctions.SellTower`
  ;[0 1 0.4 0.5] 'BPI_TowerFunctions' interface function; Implemented through child classes
)

(fn `ApplyDamageBoost`
  (params (Boost :type "Float (double-precision)"))
  (locals (Local_TempOutputPerCycle :type "Float (double-precision)"))
  ;[0 1 1 0.5] Calculates damage boost from Boost Towers & modifies Attack Damage
  (set `local.Local_TempOutputPerCycle` (/ (`self.OutputPerCycle`) (`self.DamageBoost`)))
  (set `self.DamageBoost` (+ Boost (`self.DamageBoost`))) ; Update Boost value
  (set `self.OutputPerCycle` (* (`local.Local_TempOutputPerCycle`) (`self.DamageBoost`))) ; Apply the new Boost
  (return))

(fn `CalculateSellingPrice`
  (returns (Returns :type Integer))
  ;[0 1 1 0.5] Calculates the selling price of the tower; Implemented through child classes
  (return 0))

(fn `CalculateTowerUpgradeCost`
  (returns (UpgradeCost :type Integer))
  ;[0 1 1 0.5] Calculates the amount of resources required to upgrade the tower; Implemented through child classes
  (return 0))

(fn `CalculateUpgradedTowerAttributes`
  (returns (UpgradedTowerLevel :type Integer) (UpgradedOutputPerCycle :type "Float (double-precision)") (UpgradedRechargeTime :type "Float (double-precision)") (UpgradedRange :type "Float (double-precision)"))
  (bind ((`UpgradeModifier_OutputPerCycle_34_89D0E9BD4420CCF55A2B89A312D76768` _upgrademodifier_outputpercycle) (`UpgradeModifier_RateOfFire_36_73EEBDDC4266AEF810C6CEAE522D21FB` _upgrademodifier_rateoffire) (`UpgradeModifier_Range_50_64FBB56A4BE6D4B93F9ED3B690AF16BC` _upgrademodifier_range)) (break `/Game/FPSTowerDefenseToolkit/Blueprints/Structs/Struct_TowerData` (`KismetArrayLibrary.Array_Get` (`/Game/FPSTowerDefenseToolkit/Blueprints/FunctionLibraries/BPFL_GetterFunctions.GetTowerDataArray`) (`self.TowerClassIndex`))))
  ;[0 1 1 0.5] Calculate upgraded attributes for the tower
  (return (+ (`self.TowerLevel`) 1) (* (* (/ (`self.OutputPerCycle`) (`self.DamageBoost`)) _upgrademodifier_outputpercycle) (`self.DamageBoost`)) (/ (`self.RechargeTime`) _upgrademodifier_rateoffire) (* (`self.Range`) _upgrademodifier_range)))

(fn `EvaluateTowerUpgradeRequirements`
  (returns (`Success?` :type Boolean) (UpgradeCost :type Integer))
  ;[0 1 1 0.5] Checks if the tower can be upgraded; Implemented through child classes
  (return false 0))

(fn `GetFloatAsTextWithScale`
  (params (FloatInput :type "Float (double-precision)") (Scale :type Integer))
  (returns (TextOutput :type Text))
  (bind _returnvalue (`KismetMathLibrary.FFloor` FloatInput))
  ;[0 1 1 0.5] Take a floating point value & set it's scale [number of digits succeeding the decimal point] based on the requirements & return the result as a text value
  (return (`KismetTextLibrary.Conv_StringToText` (`KismetStringLibrary.Concat_StrStr` (`KismetStringLibrary.Conv_IntToString` _returnvalue) "." (`KismetStringLibrary.GetSubstring` (`KismetStringLibrary.Conv_DoubleToString` (- FloatInput (`KismetMathLibrary.Conv_IntToDouble` _returnvalue))) 2 Scale)))))

(fn `GetGridGeneratorPlatform`
  (returns (`GridLinkedPlatformExists?` :type Boolean) (PlatformActor :type "Actor Object Reference") (TraceHitLocation :type "Vector Structure"))
  (bind _returnvalue (`self.K2_GetActorLocation`))
  ;[0 1 1 0.5] Get information about the underlying platform on which the tower is placed; Used only when the towers are placed into the level from the editor itself
  (bind _outhit (`KismetSystemLibrary.LineTraceSingle` (`KismetMathLibrary.MakeVector` (.x _returnvalue) (.y _returnvalue) (+ (.z _returnvalue) 200.0)) (`KismetMathLibrary.MakeVector` (.x _returnvalue) (.y _returnvalue) (- (.z _returnvalue) 1000.0)) "TraceTypeQuery3"))
  (bind (_bblockinghit _binitialoverlap _time _location _impactpoint _normal _impactnormal _physmat _hitactor) (`GameplayStatics.BreakHitResult` _outhit))
  (return (`KismetSystemLibrary.DoesImplementInterface` _hitactor "/Game/FPSTowerDefenseToolkit/Blueprints/Interfaces/BPI_GridLink.BPI_GridLink_C") _hitactor _location))

(fn `RetrieveTraceHitGridData`
  (params (TraceHitLocation :type "Vector Structure"))
  (returns (GridCellIndex :type Integer) (GridGeneratorIndex :type Integer) (GridVector :type "Vector Structure"))
  ;[0 1 0.4 0.5] 'BPI_GridLink' interface function used to retrieve grid data of the implementing actor
  (return (`self.GridCellIndex`) (`self.GridGeneratorIndex`) (`.GridVector_10_7F7B6B8542ECC301E9FFB082D723054A` (break `/Game/FPSTowerDefenseToolkit/Blueprints/Structs/Struct_GridCellData` (`KismetArrayLibrary.Array_Get` (`.GridGeneratorData_8_13E757544C1E18F1261E9C9C7CA2FC04` (break `/Game/FPSTowerDefenseToolkit/Blueprints/Structs/Struct_GridData` (`KismetArrayLibrary.Array_Get` (`/Game/FPSTowerDefenseToolkit/Blueprints/FunctionLibraries/BPFL_GetterFunctions.GetGridDataArray` self) (`self.GridGeneratorIndex`)))) (`self.GridCellIndex`))))))

(fn `ReturnTowerResources`
  ;[0 1 1 0.5] Used to automatically handle return of tower resources when a tower is sold back by the player; Implemented through child classes
  (return))

(fn `SetDefaultAttributes`
  (params (SelectedTowerDataArrayIndex :type Integer) (GridCellIndex :type Integer) (GridGeneratorIndex :type Integer) (TowerCost :type Integer) (OutputPerCycle :type "Float (double-precision)") (RechargeTime :type "Float (double-precision)") (Range :type "Float (double-precision)"))
  ;[0 1 1 0.5] [Only dynamic parameters are stored in the class; All static parameters are retrieved from the Tower Data Array] Setter function used to update grid data & default stats for towers placed in the level from the editor
  (set `self.TowerClassIndex` SelectedTowerDataArrayIndex)
  (set `self.GridCellIndex` GridCellIndex)
  (set `self.GridGeneratorIndex` GridGeneratorIndex)
  (set `self.TotalSetupCost` TowerCost)
  (set `self.OutputPerCycle` (* OutputPerCycle (`self.DamageBoost`)))
  (set `self.RechargeTime` RechargeTime)
  (set `self.Range` Range)
  (return))

(fn `SetUpgradedTowerAttributes`
  (params (UpgradeCost :type Integer))
  ;[0 1 1 0.5] Sets upgraded attributes when the tower is upgraded
  (set `self.TotalSetupCost` (+ (`self.TotalSetupCost`) UpgradeCost))
  (bind (_upgradedtowerlevel _upgradedoutputpercycle _upgradedrechargetime _upgradedrange) (`self.CalculateUpgradedTowerAttributes`))
  (set `self.TowerLevel` _upgradedtowerlevel)
  (set `self.OutputPerCycle` _upgradedoutputpercycle) ; Upgraded OutputPerCycle
  (set `self.RechargeTime` _upgradedrechargetime) ; Upgraded recharge time
  (set `self.Range` _upgradedrange) ; UpgradedRange
  (return))

(fn `UserConstructionScript`)

(fn `UseTowerResources`
  (params (ResourceAmount :type Integer))
  ;[0 1 1 0.5] Automatically handles the tower resource usage at spawn; implemented through child classes
  (return))