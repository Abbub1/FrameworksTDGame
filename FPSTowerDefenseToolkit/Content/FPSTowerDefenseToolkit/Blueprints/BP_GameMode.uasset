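; Game mode for a first-person tower defense level that acts as the central hub for its core actors.
; On BeginPlay it caches the grid, tower, wave, creep AI, power core and spawn point actors, then opens the tower loadout menu or initializes them all in a fixed order.
; It exposes getters, forwards tower and creep deaths to their managers, rebuilds enemy nav paths and respawns players while the power core exists.
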(event `self.ReceiveBeginPlay`
  ;[0 1 1 0.5] Start Mission
  (`self.StoreCoreGameplayActorReferences`)
  (if (`self.SelectTowersAtLevelStart?`)
    (bind _asbp_player_hud (cast `/Game/FPSTowerDefenseToolkit/Blueprints/BP_PlayerHUD` (`PlayerController.GetHUD` (`GameplayStatics.GetPlayerController` 0))))
    (`/Game/FPSTowerDefenseToolkit/Blueprints/BP_PlayerHUD.DisplayLoadoutMenu` _asbp_player_hud) ; Request the Player HUD class to Tower Loadout Menu
    (else
      (`self.InitializeCoreGameplayObjects`))))

(event `ReportPlayerCharacterPendingDestroy`
  (params (PlayerCharacter :type "Character Object Reference"))
  ;[0 1 1 0.5] Handle player death & respawn
  (`self.K2_DestroyActor` PlayerCharacter)
  (`KismetSystemLibrary.Delay` (`self.PlayerRespawnTime`))
  (`/Engine/EditorBlueprintResources/StandardMacros.IsValid` (`self.PowerCoreRef`)
    (:`Is Valid`
      (bind _returnvalue (`|SpawnActorFromClass` "/Game/FPSTowerDefenseToolkit/Blueprints/BP_PlayerCharacter.BP_PlayerCharacter_C" (`self.GetTransform` (`KismetArrayLibrary.Array_Get` (`self.PlayerSpawnPointsArray`))) "AdjustIfPossibleButAlwaysSpawn" "OverrideRootScale"))
      (bind _asbp_player_controller (cast `/Game/FPSTowerDefenseToolkit/Blueprints/BP_PlayerController` (`GameplayStatics.GetPlayerController` 0)))
      (`/Game/FPSTowerDefenseToolkit/Blueprints/BP_PlayerController.PossessCharacter` _asbp_player_controller _returnvalue) ; Requeast Player Controller to Possess the spawned character
    )))

(fn `InitializeCoreGameplayObjects`
  ;[0 1 1 0.5] Load In-Game HUD & Initialize the core gameplay actors manually
  (`/Game/FPSTowerDefenseToolkit/Blueprints/BP_GameInstance.UpdateHUDState` (cast `/Game/FPSTowerDefenseToolkit/Blueprints/BP_GameInstance` (`GameplayStatics.GetGameInstance`) :!pure true) "NewEnumerator2") ; Load In Game HUD
  (`/Game/FPSTowerDefenseToolkit/Blueprints/GameplayActors/BP_GridManager.InitializeGridManager` (`self.GridManagerRef`))
  (`/Game/FPSTowerDefenseToolkit/Blueprints/GameplayActors/BP_WaveManager.InitializeWaveManager` (`self.WaveManagerRef`))
  (`/Game/FPSTowerDefenseToolkit/Blueprints/GameplayActors/BP_TowerManager.InitializeTowerManager` (`self.TowerManagerRef`))
  (`/Game/FPSTowerDefenseToolkit/Blueprints/GameplayActors/BP_PowerCore.InitializePowerCore` (`self.PowerCoreRef`))
  (`/Game/FPSTowerDefenseToolkit/Blueprints/EnemyAI/BP_CreepAIManager.InitializeCreepAIManager` (`self.CreepAIManagerRef`))
  (for _array_element (`self.EnemySpawnPointActorsArray`)
    (`/Game/FPSTowerDefenseToolkit/Blueprints/GameplayActors/BP_EnemySpawnPoint.InitializeEnemySpawnPoint` _array_element))
  (bind _asbp_game_state (cast `/Game/FPSTowerDefenseToolkit/Blueprints/BP_GameState` (`GameplayStatics.GetGameState`))
    (:`then`
      (`/Game/FPSTowerDefenseToolkit/Blueprints/BP_GameState.InitializeGameState` _asbp_game_state)
      (bind _asbp_player_controller (cast `/Game/FPSTowerDefenseToolkit/Blueprints/BP_PlayerController` (`GameplayStatics.GetPlayerController` 0))
        (:`then`
          (`/Game/FPSTowerDefenseToolkit/Blueprints/BP_PlayerController.InitializePlayerController` _asbp_player_controller)
          (bind _asbp_player_character (cast `/Game/FPSTowerDefenseToolkit/Blueprints/BP_PlayerCharacter` (`GameplayStatics.GetPlayerCharacter` 0))
            (:`then`
              (`/Game/FPSTowerDefenseToolkit/Blueprints/BP_PlayerCharacter.InitializePlayerCharacter` _asbp_player_character))
            (:`CastFailed`
              (`KismetSystemLibrary.PrintString` "Failed Cast: InitializeCoreGameplayActors Func - GameMode" :!label _label))))
        (:`CastFailed`
          (goto _label))))
    (:`CastFailed`
      (goto _label)))
  (return))

(fn `RebuildNavPaths`
  ;[0 1 1 0.5] Rebuild Spline Paths from all Enemy Spawn Points to the Power Core
  (for _array_element (`self.EnemySpawnPointActorsArray`)
    (`/Game/FPSTowerDefenseToolkit/Blueprints/GameplayActors/BP_EnemySpawnPoint.CreateNavPath` _array_element))
  (return))

(fn `ReportCreepPendingDestroy`
  (params (Creep :type "/Game/FPSTowerDefenseToolkit/Blueprints/EnemyAI/BP_EnemyAI_Parent Object Reference"))
  ;[1 0 0 0.5] Execute pre termination protocols for creeps
  (`/Game/FPSTowerDefenseToolkit/Blueprints/GameplayActors/BP_WaveManager.EvaluateWaveTerminationStatus` (`self.WaveManagerRef`) Creep))

(fn `ReportTowerPendingDestroy`
  (params (Tower :type "/Game/FPSTowerDefenseToolkit/Blueprints/Towers/BP_TowerActual_Parent Object Reference"))
  ;[1 0 0 0.5] Execute pre termination protocols for towers
  (`/Game/FPSTowerDefenseToolkit/Blueprints/GameplayActors/BP_TowerManager.DestroyTower` (`self.TowerManagerRef`) Tower))

(fn `RetrieveCreepAIManager`
  (returns (CreepAIManagerRef :type "/Game/FPSTowerDefenseToolkit/Blueprints/EnemyAI/BP_CreepAIManager Object Reference"))
  ;[0 1 1 0.5] Returns a reference to the Creep AI Manager
  (return (`self.CreepAIManagerRef`)))

(fn `RetrieveEnemySpawnPointActors`
  (returns (EnemySpawnPointActors :type "Array of /Game/FPSTowerDefenseToolkit/Blueprints/GameplayActors/BP_EnemySpawnPoint Object Reference"))
  ;[0 1 1 0.5] Returns an array containing references to all enemy spawn points
  (return (`self.EnemySpawnPointActorsArray`)))

(fn `RetrieveGridManager`
  (returns (GridManagerRef :type "/Game/FPSTowerDefenseToolkit/Blueprints/GameplayActors/BP_GridManager Object Reference"))
  ;[0 1 1 0.5] Getter function used by other blueprints to retrieve a reference to the Grid Manager
  (return (`self.GridManagerRef`)))

(fn `RetrieveMaxNumberOfTowerTypes`
  (returns (MaxNumberOfTowerTypes :type Integer))
  ;[0 1 1 0.5] Getter function used by other blueprints to retrieve the max number of tower types that the player can select from the loadout menu
  (return (`self.MaxNumberOfTowerTypes`)))

(fn `RetrievePowerCore`
  (returns (PowerCoreRef :type "/Game/FPSTowerDefenseToolkit/Blueprints/GameplayActors/BP_PowerCore Object Reference"))
  ;[0 1 1 0.5] Getter function used by other blueprints to retrieve a reference to the Power Core
  (return (`self.PowerCoreRef`)))

(fn `RetrieveTowerManager`
  (returns (TowerManagerRef :type "/Game/FPSTowerDefenseToolkit/Blueprints/GameplayActors/BP_TowerManager Object Reference"))
  ;[0 1 1 0.5] Getter function used by other blueprints to retrieve a reference to the Tower Manager
  (return (`self.TowerManagerRef`)))

(fn `RetrieveWaveManager`
  (returns (WaveManagerRef :type "/Game/FPSTowerDefenseToolkit/Blueprints/GameplayActors/BP_WaveManager Object Reference"))
  ;[0 1 1 0.5] Getter function used by other blueprints to retrieve a reference to the Power Core
  (return (`self.WaveManagerRef`)))

(fn `StoreCoreGameplayActorReferences`
  ;[0 1 1 0.5] Store references to all core gameplay actors
  (bind _outactors (`GameplayStatics.GetAllActorsOfClass` "/Game/FPSTowerDefenseToolkit/Blueprints/GameplayActors/BP_GridManager.BP_GridManager_C"))
  (set `self.GridManagerRef` (`KismetArrayLibrary.Array_Get` _outactors))
  (bind _outactors_2 (`GameplayStatics.GetAllActorsOfClass` (`self.TowerSpawnManagerClassRef`)))
  (set `self.TowerManagerRef` (`KismetArrayLibrary.Array_Get` _outactors_2))
  (bind _outactors_3 (`GameplayStatics.GetAllActorsOfClass` (`self.WaveManagerClassRef`)))
  (set `self.WaveManagerRef` (`KismetArrayLibrary.Array_Get` _outactors_3))
  (bind _outactors_4 (`GameplayStatics.GetAllActorsOfClass` (`self.PowerCoreClassRef`)))
  (set `self.PowerCoreRef` (`KismetArrayLibrary.Array_Get` _outactors_4))
  (bind _outactors_5 (`GameplayStatics.GetAllActorsOfClass` (`self.EnemySpawnPointClassRef`)))
  (set `self.EnemySpawnPointActorsArray` _outactors_5)
  (bind _outactors_6 (`GameplayStatics.GetAllActorsOfClass` (`self.CreepAIManagerClassRef`)))
  (set `self.CreepAIManagerRef` (`KismetArrayLibrary.Array_Get` _outactors_6))
  (bind _outactors_7 (`GameplayStatics.GetAllActorsOfClass` "/Script/Engine.PlayerStart"))
  (set `self.PlayerSpawnPointsArray` _outactors_7)
  (return))

(fn `UserConstructionScript`)