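; Player state for the FPS tower defense game that tracks two build resources: tower bases left and Tower Points.
; Update functions add an increment to each value, then tell the first player controller (BP_PlayerController) to refresh the matching HUD display.
; Simple getters expose both counts to other Blueprints.
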(fn `RetrieveTowerBasesLeft`
  (returns (TowerBasesLeft :type Integer))
  ;[0 1 1 0.5] Getter function used by other blueprints to retrieve the number of tower bases left
  (return (`self.TowerBasesLeft`)))

(fn `RetrieveTowerPoints`
  (returns (TowerPoints :type Integer))
  ;[0 1 1 0.5] Getter function used by other blueprints to retrieve the amount of tower points left
  (return (`self.TowerPoints`)))

(fn `UpdateTowerBasesLeft`
  (params (Increment :type Integer))
  ;[0 1 1 0.5] Updates the number of available tower bases; Request the player controller to handle the corresponding HUD updates
  (set `self.TowerBasesLeft` (+ (`self.TowerBasesLeft`) Increment))
  (bind _asbp_player_controller (cast `/Game/FPSTowerDefenseToolkit/Blueprints/BP_PlayerController` (`GameplayStatics.GetPlayerController` 0)))
  (`/Game/FPSTowerDefenseToolkit/Blueprints/BP_PlayerController.UpdateHUD_NumberOfTowerBases` _asbp_player_controller (`self.TowerBasesLeft`)))

(fn `UpdateTowerPoints`
  (params (Increment :type Integer))
  ;[0 1 1 0.5] Updates the amount of Tower Points remaining; Request the player controller to handle the corresponding HUD updates
  (set `self.TowerPoints` (+ (`self.TowerPoints`) Increment))
  (bind _asbp_player_controller (cast `/Game/FPSTowerDefenseToolkit/Blueprints/BP_PlayerController` (`GameplayStatics.GetPlayerController` 0)))
  (`/Game/FPSTowerDefenseToolkit/Blueprints/BP_PlayerController.UpdateHUD_TowerPoints` _asbp_player_controller (`self.TowerPoints`)))

(fn `UserConstructionScript`)