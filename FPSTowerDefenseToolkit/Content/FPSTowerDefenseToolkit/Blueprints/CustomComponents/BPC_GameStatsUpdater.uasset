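; BPC_GameStatsUpdater is a component that reports damage and kill statistics to BP_GameState for the mission stats.
; EvaluateDamageReceived and EvaluateCreepDeletionData compare the instigator to player controller 0 to credit either the player or towers.
; Any instigator other than that controller counts as a tower, and each call casts the game state and invokes the matching update function.
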(fn `EvaluateCreepDeletionData`
  (params (DeletionInstigator :type "Controller Object Reference"))
  (bind _asbp_game_state (cast `/Game/FPSTowerDefenseToolkit/Blueprints/BP_GameState` (`GameplayStatics.GetGameState`) :!pure true))
  ;[0 1 1 0.5] Requests the game state to update the kill score mission stats based on the entity responsible for it
  (if (== DeletionInstigator (`GameplayStatics.GetPlayerController` 0))
    (`/Game/FPSTowerDefenseToolkit/Blueprints/BP_GameState.UpdateStats_PlayerKills` _asbp_game_state)
    (else
      (`/Game/FPSTowerDefenseToolkit/Blueprints/BP_GameState.UpdateStats_TowerKills` _asbp_game_state)))
  (return))

(fn `EvaluateDamageReceived`
  (params (DamageReceived :type "Float (double-precision)") (Instigator :type "Controller Object Reference"))
  (bind _asbp_game_state (cast `/Game/FPSTowerDefenseToolkit/Blueprints/BP_GameState` (`GameplayStatics.GetGameState`) :!pure true))
  ;[0 1 1 0.5] Requests the game state to update the damage score mission stats based on the damage causing agent
  (if (== Instigator (`GameplayStatics.GetPlayerController` 0))
    (`/Game/FPSTowerDefenseToolkit/Blueprints/BP_GameState.UpdateStats_PlayerInflictedDamage` _asbp_game_state DamageReceived)
    (else
      (`/Game/FPSTowerDefenseToolkit/Blueprints/BP_GameState.UpdateStats_TowerInflictedDamage` _asbp_game_state DamageReceived)))
  (return))