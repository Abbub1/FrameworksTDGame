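; Actor component that tracks damage-based threat for its owner, weighting potential targets by damage dealt so the owner can focus on immediate threats.
; EvaluateDamageReceived matches the damage causer to the owner's potential targets and reports damage as a fraction of max HP.
; A looping timer, started only for BPI_DamagePerception owners, applies a per-cycle decrement to every target.
; The owner holds the perception data, exchanged through interface messages.
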(event `self.ReceiveBeginPlay`
  ;[0 1 1 0.5] Initiates timed damage perception updates if the owning actor meets the compabitibility requirements
  (if (`KismetSystemLibrary.DoesImplementInterface` (`self.GetOwner`) "/Game/FPSTowerDefenseToolkit/Blueprints/Interfaces/BPI_DamagePerception.BPI_DamagePerception_C")
    (bind _returnvalue (`KismetSystemLibrary.K2_SetTimer` null "DecrementDamageWeightage" (`self.DamageWeightageDecrementTimer`) true))
    (set `self.DamageWeightageDecrementTimerHandle` _returnvalue)))

(event `self.ReceiveEndPlay`
  (params (EndPlayReason :type "EEndPlayReason Enum" :default "Destroyed"))
  (bind _damageweightagedecrementtimerhandle (`self.DamageWeightageDecrementTimerHandle`))
  ;[0 1 1 0.5] Clear timers before getting destroyed
  (if (`KismetSystemLibrary.K2_TimerExistsHandle` _damageweightagedecrementtimerhandle)
    (`KismetSystemLibrary.K2_ClearAndInvalidateTimerHandle` _damageweightagedecrementtimerhandle)))

(fn `DecrementDamageWeightage`
  ;[0 1 1 0.5] Requests the owning actor to reduce the impact of perceived damage over time [Helps ensure that the owning actor can concentrate on the immediate threat
  (bind (_maxhp _potentialtargets) (message `/Game/FPSTowerDefenseToolkit/Blueprints/Interfaces/BPI_DamagePerception.RetrieveDamagePerceptionRequisites` (`self.GetOwner`)))
  (for (_ _array_index) _potentialtargets
    (message `/Game/FPSTowerDefenseToolkit/Blueprints/Interfaces/BPI_DamagePerception.UpdateDamagePerceptionData` (`self.GetOwner`) _array_index (`self.DamagePercentDecrementPerCycle`))))

(fn `DisplayOwnerIncompatibilityWarning`
  ;[0 0 0 0.5] Prints a warning message if the owning actor does not implement the requisite interface
  (`KismetSystemLibrary.PrintString` (`KismetStringLibrary.Concat_StrStr` "Warning: [Class: BPC_VisualPerception] Owning actor '" (`KismetSystemLibrary.GetDisplayName` (`self.GetOwner`)) "' does not implement requisite interface")))

(fn `EvaluateDamageReceived`
  (params (DamageCausingAgent :type "Actor Object Reference") (DamageReceived :type "Float (double-precision)"))
  (locals (Local_OwnerMaxHP :type "Float (double-precision)" :default 0.0))
  ;[0 1 1 0.5] Evaluates damage received to the owning actor & returns the damage to health ratio if the damage causing agent meets the necessary perception requirements
  (`/Engine/EditorBlueprintResources/StandardMacros.IsValid` DamageCausingAgent
    (:`Is Valid`
      (bind (_maxhp _potentialtargets) (message `/Game/FPSTowerDefenseToolkit/Blueprints/Interfaces/BPI_DamagePerception.RetrieveDamagePerceptionRequisites` (`self.GetOwner`)))
      (set `local.Local_OwnerMaxHP` _maxhp)
      (for (_array_element _array_index) _potentialtargets
        (if (== _array_element DamageCausingAgent)
          (message `/Game/FPSTowerDefenseToolkit/Blueprints/Interfaces/BPI_DamagePerception.UpdateDamagePerceptionData` (`self.GetOwner`) _array_index (/ DamageReceived (`local.Local_OwnerMaxHP`)))
          (break))))))