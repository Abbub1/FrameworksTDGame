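; BPC_FocusFire is an actor component that lets its owner respond to manual focus fire orders in the tower defense toolkit.
; It registers owners implementing BPI_ManualTargetOverride with the Tower Manager on BeginPlay, warns otherwise, and unregisters on EndPlay.
; When evaluating an order, it sends an interface message to override the owner's active target if the focus target is in range and not already active.
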(event `self.ReceiveBeginPlay`
  ;[0 1 1 0.5] Alerts the Tower Manager about the presene of the owning actor if it meets the compabitibility requirements
  (if (`KismetSystemLibrary.DoesImplementInterface` (`self.GetOwner`) "/Game/FPSTowerDefenseToolkit/Blueprints/Interfaces/BPI_ManualTargetOverride.BPI_ManualTargetOverride_C")
    (`/Game/FPSTowerDefenseToolkit/Blueprints/GameplayActors/BP_TowerManager.AddNewFocusFireCallResponder` (`/Game/FPSTowerDefenseToolkit/Blueprints/FunctionLibraries/BPFL_GetterFunctions.GetTowerManager` self) (`self.GetOwner`))
    (else
      (`self.DisplayOwnerIncompatibilityWarning`))))

(event `self.ReceiveEndPlay`
  (params (EndPlayReason :type "EEndPlayReason Enum" :default "Destroyed"))
  ;[0 1 1 0.5] Request the Tower Manager to remove the owning actor from the list of potential targets
  (`/Game/FPSTowerDefenseToolkit/Blueprints/GameplayActors/BP_TowerManager.RemoveFocusFireCallResponder` (`/Game/FPSTowerDefenseToolkit/Blueprints/FunctionLibraries/BPFL_GetterFunctions.GetTowerManager` self) (`self.GetOwner`)))

(fn `DisplayOwnerIncompatibilityWarning`
  ;[0 0 0 0.5] Prints a warning message if the owning actor does not implement the requisite interface
  (`KismetSystemLibrary.PrintString` (`KismetStringLibrary.Concat_StrStr` "Warning: [Class: BPC_VisualPerception] Owning actor '" (`KismetSystemLibrary.GetDisplayName` (`self.GetOwner`)) "' does not implement requisite interface")))

(fn `EvaluateManualTargetOverrideOrder`
  (params (TargetsInRange :type "Array of Actor Object Reference") (FocusFireTarget :type "Actor Object Reference") (ExistingActiveTarget :type "/Game/FPSTowerDefenseToolkit/Blueprints/EnemyAI/BP_EnemyAI_Parent Object Reference"))
  ;[0 1 1 0.5] If the focus fire target is within range of the owning actor, request active target override
  (if (and (`KismetArrayLibrary.Array_Contains` TargetsInRange FocusFireTarget) (!= FocusFireTarget ExistingActiveTarget))
    (message `/Game/FPSTowerDefenseToolkit/Blueprints/Interfaces/BPI_ManualTargetOverride.OverrideActiveTarget` (`self.GetOwner`) FocusFireTarget)))