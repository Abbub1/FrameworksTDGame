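; Actor component that marks its owner as a potential target for creeps in the tower defense game.
; On BeginPlay it registers the owning actor with the Creep AI Manager, retrying after a short delay until the manager is valid to cover spawn order at level start.
; On EndPlay it asks the manager to remove the owner from the potential target list.
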(event `self.ReceiveBeginPlay`
  (bind _creepaimanager (`/Game/FPSTowerDefenseToolkit/Blueprints/FunctionLibraries/BPFL_GetterFunctions.GetCreepAIManager` self))
  ;[0 1 1 0.5] Alerts the Creep AI Manager about the presence of the owning actor
  (`/Engine/EditorBlueprintResources/StandardMacros.IsValid` _creepaimanager :!label _label
    (:`Is Valid`
      (`/Game/FPSTowerDefenseToolkit/Blueprints/EnemyAI/BP_CreepAIManager.AddNewPotentialTarget` _creepaimanager (`self.GetOwner`)))
    (:`Is Not Valid`
      (`KismetSystemLibrary.Delay` 0.1) ; Makes sure that an actor spawned before the Creep AI Manager at level start gets registered
      (goto _label))))

(event `self.ReceiveEndPlay`
  (params (EndPlayReason :type "EEndPlayReason Enum" :default "Destroyed"))
  ;[0 1 1 0.5] Request the Creep AI Manager to remove the owning actor from the list of potential targets
  (`/Game/FPSTowerDefenseToolkit/Blueprints/EnemyAI/BP_CreepAIManager.RemovePotentialTarget` (`/Game/FPSTowerDefenseToolkit/Blueprints/FunctionLibraries/BPFL_GetterFunctions.GetCreepAIManager` self) (`self.GetOwner`)))